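; Base world actor for an inventory and equipment item, with a static or skeletal mesh driven by its DataAsset.
; Construction and BeginPlay set the mesh, preferring static; BeginPlay also records mesh type and applies the asset's relative transform and any skeletal AnimBP.
; It can snap to an owning Character's mesh socket, switch to ragdoll-profile physics and track equipped state, unequipping when destroyed.
; Use and hide hooks are empty stubs.
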(event `self.ReceiveBeginPlay`
  (bind _returnvalue (select `/Game/Library/InventoryandEquipment/Blueprints/Enums/E_MeshType` (`self.MeshType`) :`NewEnumerator1` (`self.ItemStaticMesh`) :`NewEnumerator2` (`self.ItemSkeletalMesh`) :!type "SceneComponent Object Reference"))
  (`self.UpdateWorldItemMesh`)
  (add `self.OnDestroyed` (`|CreateDelegate` :!event `OnDestroyed_Event`))
  (`|ExecutionSequence`
    (:`then_0`
      (`/Engine/EditorBlueprintResources/StandardMacros.IsValid` (`SkinnedMeshComponent.SkeletalMesh` (`self.ItemSkeletalMesh`))
        (:`Is Valid`
          (bind _dataasset (`self.DataAsset`)
            (:`then`
              (set `self.MeshType` "NewEnumerator2")
              (bind _animationblueprint (`/Game/Library/InventoryandEquipment/Blueprints/Items/RPGItem.AnimationBlueprint` _dataasset)
                (:`then`
                  (`SkeletalMeshComponent.SetAnimInstanceClass` (`self.ItemSkeletalMesh`) _animationblueprint))
                (:`else`)))
            (:`else`)))
        (:`Is Not Valid`
          (`/Engine/EditorBlueprintResources/StandardMacros.IsValid` (`StaticMeshComponent.StaticMesh` (`self.ItemStaticMesh`))
            (:`Is Valid`
              (set `self.MeshType` "NewEnumerator1"))
            (:`Is Not Valid`
              (set `self.MeshType` "NewEnumerator0"))))))
    (:`then_1`
      (bind _dataasset_2 (`self.DataAsset`)
        (:`then`
          (`/Engine/EditorBlueprintResources/StandardMacros.IsValid` _returnvalue
            (:`Is Valid`
              (`SceneComponent.K2_SetRelativeTransform` _returnvalue (`/Game/Library/InventoryandEquipment/Blueprints/Items/RPGItem.RelativeTransform` _dataasset_2) false false))))
        (:`else`)))))

(event `OnDestroyed_Event` :!signature `self.OnDestroyed`
  (params (DestroyedActor :type "Actor Object Reference"))
  (`self.OnItemUnequipped`))

(fn `Attach Actor`
  (params (SocketName :type Name) (`UseExtraMesh?` :type Boolean))
  (returns (`Success?` :type Boolean))
  (`self.K2_AttachToComponent` (`Character.Mesh` (cast `Character` (`self.GetOwner`) :!pure true)) (`local.SocketName`) "SnapToTarget" "SnapToTarget" "SnapToTarget")
  (return true))

(fn `GetItemAnimInstance`
  (returns (ReturnValue :type "AnimInstance Object Reference"))
  (bind _returnvalue (`SkeletalMeshComponent.GetAnimInstance` (`self.ItemSkeletalMesh`)))
  (`/Engine/EditorBlueprintResources/StandardMacros.IsValid` _returnvalue
    (:`Is Valid`
      (return _returnvalue))))

(fn `GetItemMeshComponent`
  (returns (ReturnValue :type "PrimitiveComponent Object Reference"))
  (return (select `/Game/Library/InventoryandEquipment/Blueprints/Enums/E_MeshType` (`self.MeshType`) :`NewEnumerator1` (`self.ItemStaticMesh`) :`NewEnumerator2` (`self.ItemSkeletalMesh`) :!type "PrimitiveComponent Object Reference")))

(fn `GetOwnerCharacter`
  (returns (AsCharacter :type "Character Object Reference"))
  (return (cast `Character` (`self.GetOwner`) :!pure true)))

(fn `GetProjectileState`
  (returns (ProjectileState :type "/Game/Library/CombatSystem/Blueprints/Enums/Archery/E_WeaponProjectileState Enum"))
  (return "NewEnumerator0"))

(fn `IsItemEquipped?`
  (returns (`bIsItemEquipped?` :type Boolean))
  (return (`self.bIsItemEquipped?`)))

(fn `OnItemEquipped`
  (`self.SetItemEquipped` true))

(fn `OnItemUnequipped`
  (`self.SetItemEquipped` false))

(fn `OnUse`)

(fn `OnWorldItemHidden`
  (params (`HIdden?` :type Boolean)))

(fn `SetItemEquipped`
  (params (Condition :type Boolean))
  (set `self.bIsItemEquipped?` Condition))

(fn `SetItemMeshSimulatePhysics`
  (bind _itemstaticmesh (`self.ItemStaticMesh`))
  (bind _itemskeletalmesh (`self.ItemSkeletalMesh`))
  (`/Engine/EditorBlueprintResources/StandardMacros.IsValid` (`StaticMeshComponent.StaticMesh` _itemstaticmesh)
    (:`Is Valid`
      (`PrimitiveComponent.SetCollisionProfileName` _itemstaticmesh "ragdoll" true)
      (`PrimitiveComponent.SetSimulatePhysics` _itemstaticmesh true))
    (:`Is Not Valid`
      (`/Engine/EditorBlueprintResources/StandardMacros.IsValid` (`SkinnedMeshComponent.SkeletalMesh` _itemskeletalmesh)
        (:`Is Valid`
          (`PrimitiveComponent.SetCollisionProfileName` _itemskeletalmesh "ragdoll" true)
          (`PrimitiveComponent.SetSimulatePhysics` _itemskeletalmesh true))))))

(fn `UpdateWorldItemMesh`
  (bind _dataasset (`self.DataAsset`)
    (:`then`
      (bind _itemmesh (`/Game/Library/InventoryandEquipment/Blueprints/Items/RPGItem.ItemMesh` _dataasset)
        (:`then`
          (`StaticMeshComponent.SetStaticMesh` (`self.ItemStaticMesh`) _itemmesh))
        (:`else`
          (bind _itemskeletalmesh (`/Game/Library/InventoryandEquipment/Blueprints/Items/RPGItem.ItemSkeletalMesh` _dataasset)
            (:`then`
              (`SkinnedMeshComponent.SetSkinnedAssetAndUpdate` (`self.ItemSkeletalMesh`) _itemskeletalmesh true))
            (:`else`)))))
    (:`else`)))

(fn `UserConstructionScript`
  (`self.UpdateWorldItemMesh`))