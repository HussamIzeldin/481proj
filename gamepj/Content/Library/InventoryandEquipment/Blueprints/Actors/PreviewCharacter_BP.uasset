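; Preview character actor that renders a copy of its owner's equipped gear and idle pose through a show-only SceneCaptureComponent2D, toggled by StartCapture/EndCapture.
; It listens to the owner's EquipmentComponent, adding, removing or re-socketing meshes on CharacterMesh, with optional master pose for skeletal items.
; Quivers spawn as actors initialized with arrow count and mesh, and dual-wield weapons get a second mesh.
; Combat state selects sockets and idle animation.
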(event `self.ReceiveBeginPlay`
  (bind _equipmentcomponent (`self.EquipmentComponent`))
  (set `self.EquipmentComponent` (`self.GetComponentByClass` (`self.GetOwner`) "/Game/Library/InventoryandEquipment/Blueprints/Components/EquipmentComponent.EquipmentComponent_C"))
  (add `/Game/Library/InventoryandEquipment/Blueprints/Components/EquipmentComponent.OnEquipSlotActorAttached` (`self.EquipmentComponent`) (`|CreateDelegate` :!event `OnEquipSlotActorAttached`))
  (add `/Game/Library/InventoryandEquipment/Blueprints/Components/EquipmentComponent.OnActiveSlotEquipped` (`self.EquipmentComponent`) (`|CreateDelegate` :!event `OnActiveSlotEquipped`))
  (add `/Game/Library/InventoryandEquipment/Blueprints/Components/EquipmentComponent.OnActiveSlotUnequipped` (`self.EquipmentComponent`) (`|CreateDelegate` :!event `OnActiveSlotUnequipped`))
  (add `/Game/Library/InventoryandEquipment/Blueprints/Components/EquipmentComponent.OnCombatTypeChanged` _equipmentcomponent (`|CreateDelegate` :!event `OnCombatTypeChanged`))
  (add `/Game/Library/InventoryandEquipment/Blueprints/Components/EquipmentComponent.OnCombatChanged` _equipmentcomponent (`|CreateDelegate` :!event `OnCombatChanged`)))

(event `Start Capture`
  (set `SceneCaptureComponent.bCaptureEveryFrame` true (`self.SceneCaptureComponent2D`)))

(event `OnEquipSlotActorAttached`
  (params (EquipSlot :type "/Game/Library/InventoryandEquipment/Blueprints/Enums/Equipment/E_EquipSlots Enum" :default "NewEnumerator2") (SocketName :type Name) (AttachedActor :type "/Game/Library/InventoryandEquipment/Blueprints/Actors/WorldItem_BP Object Reference") (ItemAttached :type "/Game/Library/InventoryandEquipment/Blueprints/Structs/ItemSlot_Struct Structure"))
  (`self.AttachEquipSlotMesh` EquipSlot SocketName))

(event `UpdatePreview`
  (`self.UpdateAmmo`))

(event `EndCapture`
  (set `SceneCaptureComponent.bCaptureEveryFrame` false (`self.SceneCaptureComponent2D`)))

(event `OnActiveSlotEquipped`
  (params (NewSlotItem :type "/Game/Library/InventoryandEquipment/Blueprints/Structs/ItemSlot_Struct Structure") (SlotEquipped :type "/Game/Library/InventoryandEquipment/Blueprints/Enums/Equipment/E_EquipSlots Enum" :default "NewEnumerator2") (ActiveIndex :type Integer))
  (bind ((`Item_10_935CAA5D46A0F03B37160AA639594528` _item)) (break `/Game/Library/InventoryandEquipment/Blueprints/Structs/ItemSlot_Struct` NewSlotItem))
  (bind _itemtype (`/Game/Library/InventoryandEquipment/Blueprints/Items/RPGItem.ItemType` _item))
  ;[1 0 0 1 32] Update character preview when active slot item has been equipped
  (`BlueprintMapLibrary.Map_Add` (`self.EquippedItems`) SlotEquipped NewSlotItem)
  (if (`|EnumEquality` _itemtype "NewEnumerator10")
    (`self.AddEquipmentActor` _item)
    (elif (and (`|EnumEquality` (`/Game/Library/InventoryandEquipment/Blueprints/Items/RPGItem.ItemEquipSpawnSetting` _item) "NewEnumerator0") (`|EnumInequality` _itemtype "NewEnumerator10"))
      (`self.AddEquipmentMesh` _item)
      (`self.Add Dual WieldMesh` _item))))

(event `OnActiveSlotUnequipped`
  (params (RemovedItem :type "/Game/Library/InventoryandEquipment/Blueprints/Structs/ItemSlot_Struct Structure") (SlotRemoved :type "/Game/Library/InventoryandEquipment/Blueprints/Enums/Equipment/E_EquipSlots Enum" :default "NewEnumerator2") (ActiveIndex :type Integer))
  (bind _equippedactors (`self.EquippedActors`))
  (bind _equippedmeshes (`self.EquippedMeshes`))
  (bind _equipslot (`/Game/Library/InventoryandEquipment/Blueprints/Items/RPGItem.EquipSlot` RemovedItem_Item_10_935CAA5D46A0F03B37160AA639594528))
  (bind _value (`BlueprintMapLibrary.Map_Find` _equippedmeshes _equipslot))
  (bind _value_2 (`BlueprintMapLibrary.Map_Find` _equippedactors _equipslot))
  ;[1 0 0 1 32] Update character preview when active slot item has been Unequipped
  (`/Engine/EditorBlueprintResources/StandardMacros.IsValid` RemovedItem_Item_10_935CAA5D46A0F03B37160AA639594528
    (:`Is Valid`
      (`|ExecutionSequence`
        (:`then_0`
          (`/Engine/EditorBlueprintResources/StandardMacros.IsValid` _value
            (:`Is Valid`
              (`ActorComponent.K2_DestroyComponent` _value)
              (`BlueprintMapLibrary.Map_Remove` _equippedmeshes _equipslot))))
        (:`then_1`
          (`/Engine/EditorBlueprintResources/StandardMacros.IsValid` _value_2
            (:`Is Valid`
              (`self.K2_DestroyActor` _value_2)
              (`BlueprintMapLibrary.Map_Remove` _equippedactors _equipslot))))
        (:`then_2`
          (`self.DestroyDualWieldMesh` RemovedItem_Item_10_935CAA5D46A0F03B37160AA639594528))))))

(event `OnCombatChanged`
  (params (`CombatEnabled?` :type Boolean))
  ;[1 0 0 1 32] On Combat Type changed
  (set `self.CombatEnabled?` `CombatEnabled?`)
  (`self.OnCombatTypeChanged` (`/Game/Library/InventoryandEquipment/Blueprints/Components/EquipmentComponent.GetCurrentCombatType` (`self.EquipmentComponent`))))

(event `UpdateAmmo`
  (bind _value (`BlueprintMapLibrary.Map_Find` (`self.EquippedActors`) "NewEnumerator13"))
  (bind _value_2 (`BlueprintMapLibrary.Map_Find` (`self.EquippedItems`) "NewEnumerator20"))
  ;[1 0 0 1 32] Update character preview when ammo is updated
  (if (and (`KismetSystemLibrary.IsValid` (break `/Game/Library/InventoryandEquipment/Blueprints/Structs/ItemSlot_Struct` _value_2)) (`KismetSystemLibrary.IsValid` _value))
    (message `/Game/Library/InventoryandEquipment/Blueprints/Interfaces/WorldItemBPI.InitializeQuiver` _value (`/Game/Library/InventoryandEquipment/Blueprints/Components/EquipmentComponent.GetHeldAmountForActiveSlot` (`self.EquipmentComponent`) "NewEnumerator20") (`/Game/Library/InventoryandEquipment/Blueprints/Items/RPGItem.ItemMesh` (break `/Game/Library/InventoryandEquipment/Blueprints/Structs/ItemSlot_Struct` _value_2)))))

(event `OnCombatTypeChanged`
  (params (CombatType :type "/Game/Library/CombatSystem/Blueprints/Enums/CombatEnums/E_CombatType Enum" :default "NewEnumerator16"))
  ;[1 0 0 1 32] Update character preview idle animation when combat type changes
  (`SkeletalMeshComponent.PlayAnimation` (`self.CharacterMesh`) (select `bool` (`self.CombatEnabled?`) :`false` "/Game/Library/CombatSystem/Characters/Mannequin/Animations/Kwang/Locomotion/Idle_TravelMode_Anim.Idle_TravelMode_Anim" :`true` (`BlueprintMapLibrary.Map_Find` (`self.IdleAnimations`) CombatType) :!type "AnimationAsset Object Reference") true))

(event `InitializeActor`
  (params (ItemActorTarget :type "Actor Object Reference") (Item :type "/Game/Library/InventoryandEquipment/Blueprints/Items/RPGItem Object Reference"))
  (bind _value (`BlueprintMapLibrary.Map_Find` (`self.EquippedItems`) "NewEnumerator20"))
  ;[1 0 0 1 32] Initialize character preview quiver
  (switch `/Game/Library/InventoryandEquipment/Blueprints/Enums/E_ItemType` (`/Game/Library/InventoryandEquipment/Blueprints/Items/RPGItem.ItemType` Item)
    (:`NewEnumerator10`
      (`KismetSystemLibrary.Delay` 0.1)
      (message `/Game/Library/InventoryandEquipment/Blueprints/Interfaces/WorldItemBPI.InitializeQuiver` ItemActorTarget (`.Amount_5_DD6A685B4B673304A94C98B9ACD032DF` (break `/Game/Library/InventoryandEquipment/Blueprints/Structs/ItemSlot_Struct` _value)) (`/Game/Library/InventoryandEquipment/Blueprints/Items/RPGItem.ItemMesh` (break `/Game/Library/InventoryandEquipment/Blueprints/Structs/ItemSlot_Struct` _value))))))

(fn `Add Dual WieldMesh`
  (params (InputItem :type "/Game/Library/InventoryandEquipment/Blueprints/Items/RPGItem Object Reference"))
  (locals (L_Item :type "/Game/Library/InventoryandEquipment/Blueprints/Items/RPGItem Object Reference"))
  (bind _l_item (`local.L_Item`))
  (bind _l_item_2 (`local.L_Item`))
  (bind _l_item_3 (`local.L_Item`))
  (bind _l_item_4 (`local.L_Item`))
  (bind _itemskeletalmesh (`/Game/Library/InventoryandEquipment/Blueprints/Items/RPGItem.ItemSkeletalMesh` _l_item_2))
  (bind _itemmesh (`/Game/Library/InventoryandEquipment/Blueprints/Items/RPGItem.ItemMesh` (`local.L_Item`)))
  (bind _item (break `/Game/Library/InventoryandEquipment/Blueprints/Structs/ItemSlot_Struct` (`BlueprintMapLibrary.Map_Find` (`self.EquippedItems`) "NewEnumerator11")))
  (set `local.L_Item` _item)
  (`/Engine/EditorBlueprintResources/StandardMacros.IsValid` _l_item
    (:`Is Valid`
      (if (== (`local.InputItem`) _item)
        (if (`|EnumEquality` (`/Game/Library/InventoryandEquipment/Blueprints/Items/RPGItem.WeaponHandType` _l_item) "NewEnumerator5")
          (`/Engine/EditorBlueprintResources/StandardMacros.IsValid` _itemmesh
            (:`Is Valid`
              (`self.AddItemStaticMesh` _itemmesh "NewEnumerator9" (select `bool` (and (`self.CombatEnabled?`) (not (`/Game/Library/InventoryandEquipment/Blueprints/Components/EquipmentComponent.Is Equip Slot Disabled?` (`self.EquipmentComponent`) (`/Game/Library/InventoryandEquipment/Blueprints/Items/RPGItem.EquipSlot` (`local.L_Item`))))) :`false` (`BlueprintMapLibrary.Map_Find` (`/Game/Library/InventoryandEquipment/Blueprints/Items/RPGItem.UnEquipSocket` _l_item_4) "NewEnumerator18") :`true` (`BlueprintMapLibrary.Map_Find` (`/Game/Library/InventoryandEquipment/Blueprints/Items/RPGItem.EquipSocket` _l_item_4) "NewEnumerator9"))))
            (:`Is Not Valid`
              (`/Engine/EditorBlueprintResources/StandardMacros.IsValid` _itemskeletalmesh
                (:`Is Valid`
                  (`self.AddItemSkeletalMesh` _itemskeletalmesh "NewEnumerator9" (select `bool` (and (`self.CombatEnabled?`) (not (`/Game/Library/InventoryandEquipment/Blueprints/Components/EquipmentComponent.Is Equip Slot Disabled?` (`self.EquipmentComponent`) (`/Game/Library/InventoryandEquipment/Blueprints/Items/RPGItem.EquipSlot` _l_item_2)))) :`false` (`BlueprintMapLibrary.Map_Find` (`/Game/Library/InventoryandEquipment/Blueprints/Items/RPGItem.UnEquipSocket` _l_item_3) "NewEnumerator18") :`true` (`BlueprintMapLibrary.Map_Find` (`/Game/Library/InventoryandEquipment/Blueprints/Items/RPGItem.EquipSocket` _l_item_3) "NewEnumerator9"))))))))))))

(fn `AddEquipmentActor`
  (params (Item :type "/Game/Library/InventoryandEquipment/Blueprints/Items/RPGItem Object Reference"))
  (bind _equippedactors (`self.EquippedActors`))
  (bind _item (`local.Item`))
  (bind _equippedactors_2 (`self.EquippedActors`))
  (bind _value (`/Game/Library/InventoryandEquipment/Blueprints/Items/RPGItem.GetEquipSocket` _item))
  (bind _value_2 (`BlueprintMapLibrary.Map_Find` _equippedactors_2 (`/Game/Library/InventoryandEquipment/Blueprints/Items/RPGItem.EquipSlot` Item)))
  (bind _equipslot (`/Game/Library/InventoryandEquipment/Blueprints/Items/RPGItem.EquipSlot` (`local.Item`)))
  (`/Engine/EditorBlueprintResources/StandardMacros.IsValid` _value_2
    (:`Is Valid`
      (`KismetArrayLibrary.Array_RemoveItem` (`SceneCaptureComponent.ShowOnlyActors` (`self.SceneCaptureComponent2D`)) _value_2)
      (`self.K2_DestroyActor` _value_2)
      (`BlueprintMapLibrary.Map_Remove` _equippedactors_2 (`/Game/Library/InventoryandEquipment/Blueprints/Items/RPGItem.EquipSlot` (`local.Item`))))
    (:`Is Not Valid`
      _))
  (bind _world_item_actor_class (`/Game/Library/InventoryandEquipment/Blueprints/Items/RPGItem.World Item Actor Class` (`local.Item`))
    (:`then`
      (bind _returnvalue (`|SpawnActorFromClass` _world_item_actor_class (`self.GetTransform`) "Undefined" "OverrideRootScale" null (`local.Item`) null null))
      (`self.InitializeActor` _returnvalue (`local.Item`))
      (`KismetArrayLibrary.Array_Add` (`SceneCaptureComponent.ShowOnlyActors` (`self.SceneCaptureComponent2D`)) _returnvalue)
      (`BlueprintMapLibrary.Map_Add` _equippedactors _equipslot _returnvalue)
      (`self.K2_AttachToComponent` (`BlueprintMapLibrary.Map_Find` _equippedactors _equipslot) (`self.CharacterMesh`) (select `bool` (`/Game/Library/InventoryandEquipment/Blueprints/Items/RPGItem.IsWeapon?` (`local.Item`)) :`false` _value :`true` (select `bool` (and (`self.CombatEnabled?`) (not (`/Game/Library/InventoryandEquipment/Blueprints/Components/EquipmentComponent.Is Equip Slot Disabled?` (`self.EquipmentComponent`) (`/Game/Library/InventoryandEquipment/Blueprints/Items/RPGItem.EquipSlot` _item)))) :`false` (`/Game/Library/InventoryandEquipment/Blueprints/Items/RPGItem.GetUnEquipSocket` _item) :`true` _value)) "SnapToTarget" "SnapToTarget" "SnapToTarget" true))
    (:`else`)))

(fn `AddEquipmentMesh`
  (params (Item :type "/Game/Library/InventoryandEquipment/Blueprints/Items/RPGItem Object Reference"))
  (bind _item (`local.Item`))
  (bind _item_2 (`local.Item`))
  (bind _item_3 (`local.Item`))
  (bind _item_4 (`local.Item`))
  (bind _value (`BlueprintMapLibrary.Map_Find` (`self.EquippedMeshes`) (`/Game/Library/InventoryandEquipment/Blueprints/Items/RPGItem.EquipSlot` Item)))
  (bind _itemskeletalmesh (`/Game/Library/InventoryandEquipment/Blueprints/Items/RPGItem.ItemSkeletalMesh` _item_4))
  (bind _equipslot (`/Game/Library/InventoryandEquipment/Blueprints/Items/RPGItem.EquipSlot` (`local.Item`)))
  (bind _itemmesh (`/Game/Library/InventoryandEquipment/Blueprints/Items/RPGItem.ItemMesh` (`local.Item`)))
  (bind _itemskeletalmesh_2 (`/Game/Library/InventoryandEquipment/Blueprints/Items/RPGItem.ItemSkeletalMesh` _item_2))
  (bind _itemmesh_2 (`/Game/Library/InventoryandEquipment/Blueprints/Items/RPGItem.ItemMesh` (`local.Item`)))
  (bind _equipslot_2 (`/Game/Library/InventoryandEquipment/Blueprints/Items/RPGItem.EquipSlot` _item_2))
  (`/Engine/EditorBlueprintResources/StandardMacros.IsValid` _value
    (:`Is Valid`
      (`ActorComponent.K2_DestroyComponent` _value))
    (:`Is Not Valid`
      _))
  (if (`/Game/Library/InventoryandEquipment/Blueprints/Items/RPGItem.IsWeapon?` (`local.Item`))
    (`/Engine/EditorBlueprintResources/StandardMacros.IsValid` _itemmesh
      (:`Is Valid`
        (`self.AddItemStaticMesh` _itemmesh _equipslot (select `bool` (and (`self.CombatEnabled?`) (not (`/Game/Library/InventoryandEquipment/Blueprints/Components/EquipmentComponent.Is Equip Slot Disabled?` (`self.EquipmentComponent`) _equipslot))) :`false` (`/Game/Library/InventoryandEquipment/Blueprints/Items/RPGItem.GetUnEquipSocket` _item) :`true` (`/Game/Library/InventoryandEquipment/Blueprints/Items/RPGItem.GetEquipSocket` _item))))
      (:`Is Not Valid`
        (`/Engine/EditorBlueprintResources/StandardMacros.IsValid` _itemskeletalmesh_2
          (:`Is Valid`
            (`self.AddItemSkeletalMesh` _itemskeletalmesh_2 _equipslot_2 (select `bool` (and (`self.CombatEnabled?`) (not (`/Game/Library/InventoryandEquipment/Blueprints/Components/EquipmentComponent.Is Equip Slot Disabled?` (`self.EquipmentComponent`) _equipslot_2))) :`false` (`/Game/Library/InventoryandEquipment/Blueprints/Items/RPGItem.GetUnEquipSocket` _item_2) :`true` (`/Game/Library/InventoryandEquipment/Blueprints/Items/RPGItem.GetEquipSocket` _item_2)))))))
    (else
      (`/Engine/EditorBlueprintResources/StandardMacros.IsValid` _itemmesh_2
        (:`Is Valid`
          (`self.AddItemStaticMesh` _itemmesh_2 (`/Game/Library/InventoryandEquipment/Blueprints/Items/RPGItem.EquipSlot` _item_3) (`/Game/Library/InventoryandEquipment/Blueprints/Items/RPGItem.GetEquipSocket` _item_3)))
        (:`Is Not Valid`
          (`/Engine/EditorBlueprintResources/StandardMacros.IsValid` _itemskeletalmesh
            (:`Is Valid`
              (`self.AddItemSkeletalMesh` _itemskeletalmesh (`/Game/Library/InventoryandEquipment/Blueprints/Items/RPGItem.EquipSlot` _item_4) (`/Game/Library/InventoryandEquipment/Blueprints/Items/RPGItem.GetEquipSocket` _item_4)))))))))

(fn `AddItemSkeletalMesh`
  (params (SkeletalMesh :type "SkeletalMesh Object Reference") (EquipSlot :type "/Game/Library/InventoryandEquipment/Blueprints/Enums/Equipment/E_EquipSlots Enum" :default "NewEnumerator2") (EquipSocket :type Name))
  (bind (_value _returnvalue) (`BlueprintMapLibrary.Map_Find` (`self.AllowMasterPoseComponent`) (`local.EquipSlot`)))
  (if (`|EnumInequality` EquipSlot "NewEnumerator2")
    (bind _returnvalue_2 (`AddComponent|NODE_AddSkeletalMeshComponent-0` :`RelativeTransform` (`self.GetTransform`)))
    (`BlueprintMapLibrary.Map_Add` (`self.EquippedMeshes`) (`local.EquipSlot`) _returnvalue_2)
    (`SceneCaptureComponent.ShowOnlyComponent` (`self.SceneCaptureComponent2D`) _returnvalue_2)
    (`SkinnedMeshComponent.SetSkinnedAssetAndUpdate` _returnvalue_2 (`local.SkeletalMesh`) false)
    (`SceneComponent.K2_AttachToComponent` _returnvalue_2 (`self.CharacterMesh`) (`local.EquipSocket`) "SnapToTarget" "SnapToTarget" "SnapToTarget" true)
    (if (and _value _returnvalue)
      (`SkinnedMeshComponent.SetLeaderPoseComponent` _returnvalue_2 (`self.CharacterMesh`) false))))

(fn `AddItemStaticMesh`
  (params (Mesh :type "StaticMesh Object Reference") (EquipSlot :type "/Game/Library/InventoryandEquipment/Blueprints/Enums/Equipment/E_EquipSlots Enum" :default "NewEnumerator2") (EquipSocket :type Name))
  (if (`|EnumInequality` EquipSlot "NewEnumerator2")
    (bind _returnvalue (`AddComponent|NODE_AddStaticMeshComponent-1` :`RelativeTransform` (`self.GetTransform`)))
    (`SceneCaptureComponent.ShowOnlyComponent` (`self.SceneCaptureComponent2D`) _returnvalue)
    (`BlueprintMapLibrary.Map_Add` (`self.EquippedMeshes`) (`local.EquipSlot`) _returnvalue)
    (`StaticMeshComponent.SetStaticMesh` _returnvalue (`local.Mesh`))
    (`SceneComponent.K2_AttachToComponent` _returnvalue (`self.CharacterMesh`) (`local.EquipSocket`) "SnapToTarget" "SnapToTarget" "SnapToTarget" true)))

(fn `AttachDualWeapon`
  (params (InputItem :type "/Game/Library/InventoryandEquipment/Blueprints/Items/RPGItem Object Reference") (`Disabled?` :type Boolean))
  (locals (L_Item :type "/Game/Library/InventoryandEquipment/Blueprints/Items/RPGItem Object Reference"))
  (bind _l_item (`local.L_Item`))
  (bind _item (break `/Game/Library/InventoryandEquipment/Blueprints/Structs/ItemSlot_Struct` (`BlueprintMapLibrary.Map_Find` (`self.EquippedItems`) "NewEnumerator11")))
  (set `local.L_Item` _item)
  (`/Engine/EditorBlueprintResources/StandardMacros.IsValid` (`local.L_Item`)
    (:`Is Valid`
      (if (== (`local.InputItem`) _item)
        (`self.AttachEquipSlotMesh` "NewEnumerator9" (select `bool` `Disabled?` :`false` (`BlueprintMapLibrary.Map_Find` (`/Game/Library/InventoryandEquipment/Blueprints/Items/RPGItem.EquipSocket` _l_item) "NewEnumerator9") :`true` (`BlueprintMapLibrary.Map_Find` (`/Game/Library/InventoryandEquipment/Blueprints/Items/RPGItem.UnEquipSocket` _l_item) "NewEnumerator18")))))))

(fn `AttachEquipSlotMesh`
  (params (EquipSlot :type "/Game/Library/InventoryandEquipment/Blueprints/Enums/Equipment/E_EquipSlots Enum" :default "NewEnumerator2") (SocketName :type Name))
  (bind _value (`BlueprintMapLibrary.Map_Find` (`self.EquippedMeshes`) EquipSlot))
  (`/Engine/EditorBlueprintResources/StandardMacros.IsValid` _value
    (:`Is Valid`
      (`SceneComponent.K2_AttachToComponent` _value (`self.CharacterMesh`) SocketName "SnapToTarget" "SnapToTarget" "SnapToTarget" true))))

(fn `DestroyDualWieldMesh`
  (params (InputItem :type "/Game/Library/InventoryandEquipment/Blueprints/Items/RPGItem Object Reference"))
  (locals (L_Item :type "/Game/Library/InventoryandEquipment/Blueprints/Items/RPGItem Object Reference"))
  (bind _l_item (`local.L_Item`))
  (bind _equippedactors (`self.EquippedActors`))
  (bind _equippedmeshes (`self.EquippedMeshes`))
  (bind _value (`BlueprintMapLibrary.Map_Find` _equippedmeshes "NewEnumerator9"))
  (bind _value_2 (`BlueprintMapLibrary.Map_Find` _equippedactors "NewEnumerator9"))
  (bind _item (break `/Game/Library/InventoryandEquipment/Blueprints/Structs/ItemSlot_Struct` (`BlueprintMapLibrary.Map_Find` (`self.EquippedItems`) "NewEnumerator11")))
  (set `local.L_Item` _item)
  (`/Engine/EditorBlueprintResources/StandardMacros.IsValid` _l_item
    (:`Is Valid`
      (if (== (`local.InputItem`) _item)
        (if (`|EnumEquality` (`/Game/Library/InventoryandEquipment/Blueprints/Items/RPGItem.WeaponHandType` _l_item) "NewEnumerator5")
          (`|ExecutionSequence`
            (:`then_0`
              (`/Engine/EditorBlueprintResources/StandardMacros.IsValid` _value
                (:`Is Valid`
                  (`ActorComponent.K2_DestroyComponent` _value)
                  (`BlueprintMapLibrary.Map_Remove` _equippedmeshes "NewEnumerator9"))))
            (:`then_1`
              (`/Engine/EditorBlueprintResources/StandardMacros.IsValid` _value_2
                (:`Is Valid`
                  (`self.K2_DestroyActor` _value_2)
                  (`BlueprintMapLibrary.Map_Remove` _equippedactors "NewEnumerator9"))))))))))

(fn `UserConstructionScript`
  (bind _scenecapturecomponent2d (`self.SceneCaptureComponent2D`))
  (`SceneCaptureComponent.ShowOnlyActorComponents` (`self.SceneCaptureComponent2D`) self false)
  (set `SceneCaptureComponent2D.FOVAngle` (`self.FOV Angle`) (`self.SceneCaptureComponent2D`))
  (`SceneCaptureComponent.ShowOnlyComponent` _scenecapturecomponent2d null)
  (`SceneCaptureComponent.ShowOnlyComponent` _scenecapturecomponent2d null))