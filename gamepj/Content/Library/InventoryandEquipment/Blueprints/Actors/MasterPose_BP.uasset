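; MasterPose_BP is an equipment item actor for skeletal mesh items that follow the animation of the owning Character.
; AttachActor snaps ItemSkeletalMesh to the given socket on the owner's mesh, then sets that mesh as its master pose component.
; It returns whether the item mesh was valid and ignores the UseExtraMesh input; the event graph only calls the parent's BeginPlay.
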(event `self.ReceiveBeginPlay`
  (`parent.ReceiveBeginPlay`))

(fn `Attach Actor`
  (params (SocketName :type Name) (`UseExtraMesh?` :type Boolean))
  (returns (`Success?` :type Boolean))
  (bind _mesh (`Character.Mesh` (cast `Character` (`self.GetOwner`) :!pure true)))
  (`/Engine/EditorBlueprintResources/StandardMacros.IsValid` (`self.ItemSkeletalMesh`)
    (:`Is Valid`
      (`SceneComponent.K2_AttachToComponent` (`self.ItemSkeletalMesh`) _mesh (`local.SocketName`) "SnapToTarget" "SnapToTarget" "SnapToTarget" true)
      (`SkinnedMeshComponent.SetLeaderPoseComponent` (`self.ItemSkeletalMesh`) _mesh false)
      (return true))
    (:`Is Not Valid`
      (return false))))

(fn `UserConstructionScript`
  (`parent.UserConstructionScript`))