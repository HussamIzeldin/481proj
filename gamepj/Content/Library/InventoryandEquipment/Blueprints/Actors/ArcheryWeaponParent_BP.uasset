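; Parent Blueprint for archery weapons in the inventory and equipment system, managing the arrow display and string-draw state.
; On attach, the owner's combat state sets arrow mesh visibility, with the mesh snapped to data-asset sockets on weapon or character.
; Equipping passes draw speed and string socket to anim instances and registers with EquipmentComponent.
; A reversible timeline drives DrawStringAlpha; AttachAmmo attaches projectiles, while Reload and OnAmmoAttached are empty here.
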(event `StartDrawStringTimeline`
  (params (`Reverse?` :type Boolean) (TL_PlayRate :type "Float (double-precision)" :default 6.0))
  (`TimelineComponent.SetPlayRate` (`self.DrawStringTL`) TL_PlayRate)
  (if (not `Reverse?`)
    (bind (_direction _drawstringalpha) (`Timeline|DrawStringTL` :!label _label)
      (:`Update`
        (set `self.DrawStringAlpha` _drawstringalpha)))
    (else
      (goto _label :!via `Reverse`))))

(event `StopDrawStringTL`
  (goto _label :!via `Stop`))

(event `Reload`
  (if (not (`KismetSystemLibrary.IsValid` (`self.ArcheryProjectile`)))
    _))

(fn `Attach Actor`
  (params (SocketName :type Name) (`UseExtraMesh?` :type Boolean))
  (returns (`Success?` :type Boolean))
  (bind _combatmode (message `/Game/Library/CombatSystem/Blueprints/Interfaces/CombatBPI.CombatEnabled?` (`self.GetOwner`)))
  (if _combatmode
    (`self.UpdateArrowMesh`)
    (`self.UpdateArrowVisibility` true)
    (`self.AttachArrow` false)
    (else
      (`self.UpdateArrowVisibility` false)))
  (bind _success_ (`parent.Attach Actor` (`local.SocketName`) false))
  (return _success_))

(fn `Attach Ammo`
  (params (SocketName :type Name) (New_ArrowState :type "/Game/Library/CombatSystem/Blueprints/Enums/Archery/E_WeaponProjectileState Enum" :default "NewEnumerator0") (AttachParent :type "PrimitiveComponent Object Reference"))
  (returns (`Success?` :type Boolean))
  (bind _new_arrowstate (`local.New_ArrowState`))
  (bind _archeryprojectile (`self.ArcheryProjectile`))
  (`/Engine/EditorBlueprintResources/StandardMacros.IsValid` _archeryprojectile
    (:`Is Valid`
      (`self.K2_AttachToComponent` _archeryprojectile AttachParent (`local.SocketName`) "SnapToTarget" "SnapToTarget" "SnapToTarget" true)
      (`/Game/Library/InventoryandEquipment/Blueprints/Actors/Projectiles/ProjectileParent_BP.Set Weapon Projectile State` (`self.ArcheryProjectile`) _new_arrowstate)
      (`self.OnAmmoAttached` (`|EnumEquality` _new_arrowstate "NewEnumerator2"))
      (return true))
    (:`Is Not Valid`
      (return false))))

(fn `AttachArrow`
  (params (`AttachToCharacter?` :type Boolean))
  (bind _dataasset (`self.DataAsset`)
    (:`then`
      (if `AttachToCharacter?`
        (`SceneComponent.K2_AttachToComponent` (`self.ArrowMesh`) (`Character.Mesh` (cast `Character` (`self.GetOwner`) :!pure true)) (`/Game/Library/InventoryandEquipment/Blueprints/Items/RPGItem.PlayerHandStringSocketName` _dataasset) "SnapToTarget" "SnapToTarget" "SnapToTarget" true)
        (else
          (`SceneComponent.K2_AttachToComponent` (`self.ArrowMesh`) (`self.GetItemMeshComponent`) (`/Game/Library/InventoryandEquipment/Blueprints/Items/RPGItem.Archery Projectile Equip socket` _dataasset) "SnapToTarget" "SnapToTarget" "SnapToTarget" true))))
    (:`else`)))

(fn `IsArrowMeshVisible?`
  (returns (ReturnValue :type Boolean))
  (return (`SceneComponent.IsVisible` (`self.ArrowMesh`))))

(fn `OnAmmoAttached`
  (params (`AttachedToWeapon?` :type Boolean)))

(fn `OnItemEquipped`
  (`parent.OnItemEquipped`)
  (bind _dataasset (`self.DataAsset`)
    (:`then`
      (message `/Game/Library/CombatSystem/Blueprints/Interfaces/AnimInstanceBPI.SetBowDrawSpeed` (`SkeletalMeshComponent.GetAnimInstance` (`Character.Mesh` (cast `Character` (`self.GetOwner`) :!pure true))) (`/Game/Library/InventoryandEquipment/Blueprints/Items/RPGItem.BowDrawSpeedRate` _dataasset))
      (message `/Game/Library/CombatSystem/Blueprints/Interfaces/AnimInstanceBPI.SetPlayerHandStringSocketName` (`SkeletalMeshComponent.GetAnimInstance` (`self.ItemSkeletalMesh`)) (`/Game/Library/InventoryandEquipment/Blueprints/Items/RPGItem.PlayerHandStringSocketName` _dataasset))
      (bind _equipmentcomponent (`self.EquipmentComponent`)
        (:`then`
          (`/Game/Library/InventoryandEquipment/Blueprints/Components/EquipmentComponent.Set Archery Weapon` _equipmentcomponent self))
        (:`else`)))
    (:`else`)))

(fn `UpdateArrowMesh`
  (`self.DataAsset`
    (:`then`
      (bind _mesh (message `/Game/Library/CombatSystem/Blueprints/Interfaces/CombatBPI.GetArrowMesh` (`self.GetOwner`)))
      (`StaticMeshComponent.SetStaticMesh` (`self.ArrowMesh`) _mesh))
    (:`else`)))

(fn `UpdateArrowVisibility`
  (params (`Visible?` :type Boolean))
  (`SceneComponent.SetVisibility` (`self.ArrowMesh`) `Visible?` false))

(fn `UserConstructionScript`
  (`parent.UserConstructionScript`))