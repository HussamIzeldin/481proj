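; PickUpActor_BP is an interactable pickup actor that holds loot items for the inventory and equipment library.
; AddItem appends to the Items array until MaxSlots is reached and returns whether it succeeded, while GetLootItems exposes the array.
; Interact destroys the actor when DestroyInteractableOnUse is set, without transferring any items itself.
; GetPlayerSpawnTransform is an empty stub.
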(event `self.ReceiveBeginPlay`
  (`parent.ReceiveBeginPlay`))

(event `/Game/Library/CombatSystem/Blueprints/Interfaces/InteractableBPI.Interact`
  (params (Caller :type "Actor Object Reference"))
  ;[0.5469 1 0] If true, destroy this actor
  (if (`self.bDestroyInteractableOnUse?`)
    (`self.K2_DestroyActor`)))

(fn `Add Item`
  (params (NewItem :type "/Game/Library/InventoryandEquipment/Blueprints/Structs/ItemSlot_Struct Structure (by ref)"))
  (returns (`Success?` :type Boolean))
  (if (not (>= (`KismetArrayLibrary.Array_Length` (`self.Items`)) (`self.MaxSlots`)))
    (`KismetArrayLibrary.Array_Add` (`self.Items`) NewItem)
    (return true)
    (else
      (return false))))

(fn `GetLootItems`
  (returns (ItemToEquip :type "Array of /Game/Library/InventoryandEquipment/Blueprints/Structs/ItemSlot_Struct Structure"))
  (return (`self.Items`)))

(fn `GetPlayerSpawnTransform`
  (returns (SpawnTransform :type "Transform Structure"))
  (return))

(fn `UserConstructionScript`)