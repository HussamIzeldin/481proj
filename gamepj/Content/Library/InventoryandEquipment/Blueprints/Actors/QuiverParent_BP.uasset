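; Base equippable quiver actor that displays the remaining archery ammo as arrows inside the quiver.
; On equip it reads the active ammo slot for mesh and count, showing one fewer than the amount, capped at a maximum.
; An InstancedStaticMesh on the item mesh's socket draws arrows at the transforms of 25 placeholder components.
; Slot updates rebuild instances only when archery ammo increases; UpdateQuiver and InitializeQuiver events allow direct refreshes.
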(event `EquipSlotUpdated_Event`
  (params (EquipSlot :type "/Game/Library/InventoryandEquipment/Blueprints/Enums/Equipment/E_EquipSlots Enum" :default "NewEnumerator2") (EquipSlotUpdated :type "/Game/Library/InventoryandEquipment/Blueprints/Structs/EquipmentSlot_Struct Structure") (UpdateType :type "/Game/Library/InventoryandEquipment/Blueprints/Enums/Equipment/E_UpdateQuickSlotType Enum" :default "NewEnumerator0") (`Item Index` :type Integer))
  (bind ((`ActiveItemIndex_20_CBBA13604B2E78D5C0285EB1B0728468` _activeitemindex) (`Items_17_DD6A685B4B673304A94C98B9ACD032DF` _items)) (break `/Game/Library/InventoryandEquipment/Blueprints/Structs/EquipmentSlot_Struct` EquipSlotUpdated))
  (bind _output (`|GetArrayItem` _items _activeitemindex))
  (bind ((`Amount_5_DD6A685B4B673304A94C98B9ACD032DF` _amount)) (break `/Game/Library/InventoryandEquipment/Blueprints/Structs/ItemSlot_Struct` _output))
  (if (and (`|EnumEquality` EquipSlot "NewEnumerator20") (> _amount (`.Amount_5_DD6A685B4B673304A94C98B9ACD032DF` (break `/Game/Library/InventoryandEquipment/Blueprints/Structs/ItemSlot_Struct` (`self.LastUpdatedAmmoItem`)))) (`/Game/Library/InventoryandEquipment/Blueprints/Libraries/InventoryEquipmentLibrary.IsAmmoArchery?` _output))
    (`self.UpdateArrowsInQuiver` _amount)))

(event `/Game/Library/InventoryandEquipment/Blueprints/Interfaces/WorldItemBPI.UpdateQuiver`
  (params (Amount :type Integer))
  (`self.UpdateArrowsInQuiver` Amount))

(event `self.ReceiveBeginPlay`
  (`parent.ReceiveBeginPlay`)
  (bind _dataasset (`self.DataAsset`)
    (:`then`
      (`SceneComponent.K2_AttachToComponent` (`self.InstancedStaticMesh`) (`self.GetItemMeshComponent`) (`/Game/Library/InventoryandEquipment/Blueprints/Items/RPGItem.FindEquipSocket` _dataasset "NewEnumerator20") "SnapToTarget" "SnapToTarget" "SnapToTarget" true))
    (:`else`)))

(event `/Game/Library/InventoryandEquipment/Blueprints/Interfaces/WorldItemBPI.InitializeQuiver`
  (params (Arrows :type Integer) (ArrowMesh :type "StaticMesh Object Reference"))
  (set `self.EquippedArrowMesh` ArrowMesh)
  (`self.UpdateArrowsInQuiver` Arrows))

(fn `AddArrowsToQuiver`
  (params (AmountToAdd :type Integer))
  (locals (L_ArrowsInQuiver :type Integer :default 0))
  (for _index (range AmountToAdd)
    (bind _output (`|GetArrayItem` (`self.Arrows`) _index))
    (`/Engine/EditorBlueprintResources/StandardMacros.IsValid` _output
      (:`Is Valid`
        (`InstancedStaticMeshComponent.AddInstance` (`self.InstancedStaticMesh`) (`SceneComponent.GetRelativeTransform` _output))
        (`self.SetArrowsInQuiver` (+ (`self.ArrowsInQuiver`) 1)))))
  (`KismetArrayLibrary.Array_Resize` (`self.Arrows`) (`self.ArrowsInQuiver`))
  (return))

(fn `InitializeArrowsInQuiver`
  (params (AmountToAdd :type Integer) (InArrowMesh :type "StaticMesh Object Reference"))
  (bind _instancedstaticmesh (`self.InstancedStaticMesh`))
  (bind _returnvalue (+ (`self.ArrowsInQuiver`) (`local.AmountToAdd`)))
  (`/Engine/EditorBlueprintResources/StandardMacros.IsValid` InArrowMesh
    (:`Is Valid`
      (set `self.EquippedArrowMesh` InArrowMesh)
      (`self.SetArrowsInQuiver` (`KismetMathLibrary.Clamp` (select `bool` (> _returnvalue (`self.MaxArrowsInQuiver`)) :`false` _returnvalue :`true` (`self.MaxArrowsInQuiver`)) 0 (`self.MaxArrowsInQuiver`)))
      (`KismetArrayLibrary.Array_Clear` (`self.Arrows`))
      (bind _output_get (set `self.Arrows` (`|MakeArray` (`self.Arrow`) (`self.Arrow1`) (`self.Arrow2`) (`self.Arrow3`) (`self.Arrow4`) (`self.Arrow5`) (`self.Arrow6`) (`self.Arrow7`) (`self.Arrow8`) (`self.Arrow9`) (`self.Arrow10`) (`self.Arrow11`) (`self.Arrow12`) (`self.Arrow13`) (`self.Arrow14`) (`self.Arrow15`) (`self.Arrow16`) (`self.Arrow17`) (`self.Arrow18`) (`self.Arrow19`) (`self.Arrow20`) (`self.Arrow21`) (`self.Arrow22`) (`self.Arrow23`) (`self.Arrow24`))))
      (`KismetArrayLibrary.Array_Resize` _output_get (`self.ArrowsInQuiver`))
      (`InstancedStaticMeshComponent.ClearInstances` _instancedstaticmesh)
      (`StaticMeshComponent.SetStaticMesh` _instancedstaticmesh (`local.InArrowMesh`))
      (for _array_element (`self.Arrows`)
        (`InstancedStaticMeshComponent.AddInstance` (`self.InstancedStaticMesh`) (`SceneComponent.GetRelativeTransform` _array_element))))))

(fn `OnItemEquipped`
  (bind _item (`/Game/Library/InventoryandEquipment/Blueprints/Components/EquipmentComponent.GetActiveEquippedSlotItem` (`self.EquipmentComponent`) "NewEnumerator20"))
  (bind ((`Item_10_935CAA5D46A0F03B37160AA639594528` _item_2) (`Amount_5_DD6A685B4B673304A94C98B9ACD032DF` _amount)) (break `/Game/Library/InventoryandEquipment/Blueprints/Structs/ItemSlot_Struct` _item))
  (`parent.OnItemEquipped`)
  (add `/Game/Library/InventoryandEquipment/Blueprints/Components/EquipmentComponent.EquipSlotUpdated` (`self.EquipmentComponent`) (`|CreateDelegate` :!event `EquipSlotUpdated_Event`))
  (`/Game/Library/InventoryandEquipment/Blueprints/Libraries/CombatSystemMacroLibrary.OnItemValid` _item
    (:`true`
      (`self.DataAsset`
        (:`then`
          (`self.InitializeArrowsInQuiver` (- _amount 1) (`/Game/Library/InventoryandEquipment/Blueprints/Items/RPGItem.ItemMesh` _item_2)))
        (:`else`)))))

(fn `OnItemUnequipped`
  (`parent.OnItemUnequipped`)
  (bind _equipmentcomponent (`self.EquipmentComponent`)
    (:`then`
      (remove `/Game/Library/InventoryandEquipment/Blueprints/Components/EquipmentComponent.EquipSlotUpdated` _equipmentcomponent (`|CreateDelegate` :!event `EquipSlotUpdated_Event`)))
    (:`else`)))

(fn `RemoveArrowsFromQuiver`
  (params (`Amount To Remove` :type Integer))
  (locals (L_ArrowsInQuiver :type Integer :default 0))
  (for _index (range `Amount To Remove`)
    (`InstancedStaticMeshComponent.RemoveInstance` (`self.InstancedStaticMesh`) _index)
    (`self.SetArrowsInQuiver` (- (`self.ArrowsInQuiver`) (`local.Amount To Remove`))))
  (`KismetArrayLibrary.Array_Resize` (`self.Arrows`) (`self.ArrowsInQuiver`))
  (return))

(fn `SetArrowsInQuiver`
  (params (ArrowsInQuiver :type Integer))
  (bind _output_get (set `self.ArrowsInQuiver` ArrowsInQuiver))
  (setmembers `/Game/Library/InventoryandEquipment/Blueprints/Structs/ItemSlot_Struct` :`StructRef` (`self.LastUpdatedAmmoItem`) :`Amount` _output_get))

(fn `UpdateArrowsInQuiver`
  (params (InAmount :type Integer))
  (bind _instancedstaticmesh (`self.InstancedStaticMesh`))
  (`self.SetArrowsInQuiver` (`KismetMathLibrary.Clamp` (- InAmount 1) 0 (`self.MaxArrowsInQuiver`)))
  (bind _equipmentcomponent (`self.EquipmentComponent`)
    (:`then`
      (set `self.LastUpdatedAmmoItem` (`/Game/Library/InventoryandEquipment/Blueprints/Components/EquipmentComponent.GetActiveEquippedSlotItem` _equipmentcomponent "NewEnumerator20")))
    (:`else`
      _))
  (`KismetArrayLibrary.Array_Clear` (`self.Arrows`))
  (bind _output_get (set `self.Arrows` (`|MakeArray` (`self.Arrow`) (`self.Arrow1`) (`self.Arrow2`) (`self.Arrow3`) (`self.Arrow4`) (`self.Arrow5`) (`self.Arrow6`) (`self.Arrow7`) (`self.Arrow8`) (`self.Arrow9`) (`self.Arrow10`) (`self.Arrow11`) (`self.Arrow12`) (`self.Arrow13`) (`self.Arrow14`) (`self.Arrow15`) (`self.Arrow16`) (`self.Arrow17`) (`self.Arrow18`) (`self.Arrow19`) (`self.Arrow20`) (`self.Arrow21`) (`self.Arrow22`) (`self.Arrow23`) (`self.Arrow24`))))
  (`KismetArrayLibrary.Array_Resize` _output_get (`self.ArrowsInQuiver`))
  (`InstancedStaticMeshComponent.ClearInstances` _instancedstaticmesh)
  (`StaticMeshComponent.SetStaticMesh` _instancedstaticmesh (`self.EquippedArrowMesh`))
  (for _array_element (`self.Arrows`)
    (`InstancedStaticMeshComponent.AddInstance` (`self.InstancedStaticMesh`) (`SceneComponent.GetRelativeTransform` _array_element))))

(fn `UserConstructionScript`)