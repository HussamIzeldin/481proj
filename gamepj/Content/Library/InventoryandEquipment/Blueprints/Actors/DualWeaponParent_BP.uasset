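; Base weapon actor for dual-wielded weapons, adding a second weapon mesh and collision component.
; For one hand type, BeginPlay duplicates a static item mesh, while a skeletal one is reused as the second mesh reference.
; Second-weapon hits feed the shared OnHit handler.
; Equipping registers it as active and offhand actor, attaching by combat state; AttachActor snaps either mesh to a character socket.
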(event `self.ReceiveBeginPlay`
  (bind _returnvalue (`self.GetItemMeshComponent`))
  (`parent.ReceiveBeginPlay`)
  (`/Game/Library/CombatSystem/Blueprints/Components/CollisionComponent.InitializeComponent` (`self.SecondWeaponCollisionComponent`) (`self.GetOwner`))
  (bind _dataasset (`self.DataAsset`)
    (:`then`
      (if (`|EnumEquality` (`/Game/Library/InventoryandEquipment/Blueprints/Items/RPGItem.WeaponHandType` _dataasset) "NewEnumerator5")
        (bind _asstatic_mesh_component (cast `StaticMeshComponent` _returnvalue)
          (:`then`
            (bind _returnvalue_2 (`AddComponent|NODE_AddStaticMeshComponent-3` :`RelativeTransform` (`SceneComponent.GetRelativeTransform` _returnvalue)))
            (bind _output_get (set `self.SecondWeaponStaticMesh` _returnvalue_2))
            (`PrimitiveComponent.SetCollisionEnabled` _output_get "NoCollision")
            (`StaticMeshComponent.SetStaticMesh` _returnvalue_2 (`StaticMeshComponent.StaticMesh` _asstatic_mesh_component)))
          (:`CastFailed`
            (bind _asskeletal_mesh_component (cast `SkeletalMeshComponent` _returnvalue))
            (bind _output_get_2 (set `self.SecondWeaponSkeletalMeshComponent` _asskeletal_mesh_component))
            (`PrimitiveComponent.SetCollisionEnabled` _output_get_2 "NoCollision")
            (`SkinnedMeshComponent.SetSkinnedAssetAndUpdate` _asskeletal_mesh_component (`SkinnedMeshComponent.SkeletalMesh` _asskeletal_mesh_component) true)))))
    (:`else`)))

(event `self.SecondWeaponCollisionComponent.OnCollisionEnabled`
  (params (TraceTarget :type "/Game/Library/CombatSystem/Blueprints/Enums/CombatEnums/E_CollisionTraceTarget Enum" :default "NewEnumerator0"))
  (bind _mesh (`self.GetSecondWeaponMesh`))
  ;[1 0 0 1 42] On Hit
  (`/Game/Library/CombatSystem/Blueprints/Components/CollisionComponent.SetCollisionMesh` (`self.SecondWeaponCollisionComponent`) _mesh (`SceneComponent.GetAllSocketNames` _mesh)))

(event `self.SecondWeaponCollisionComponent.OnHit`
  (params (HitResult :type "HitResult Structure") (HitCollisionChannel :type "ECollisionChannel Enum" :default "ECC_WorldStatic"))
  (bind _lasthit (`self.LastHit`))
  ;[1 0 0 1 42] On Hit
  (set `self.LastHit` HitResult)
  (if (`|EnumEquality` HitCollisionChannel "ECC_Pawn")
    (`self.On Hit` _lasthit "ECC_Pawn")
    (else
      (`self.On Hit` _lasthit HitCollisionChannel))))

(fn `Attach Actor`
  (params (SocketName :type Name) (`UseExtraMesh?` :type Boolean))
  (returns (`Success?` :type Boolean))
  (bind _returnvalue (`SceneComponent.K2_AttachToComponent` (select `bool` `UseExtraMesh?` :`false` (`self.GetItemMeshComponent`) :`true` (`self.GetSecondWeaponMesh`) :!type "SceneComponent Object Reference") (`Character.Mesh` (cast `Character` (`self.GetOwner`) :!pure true)) SocketName "SnapToTarget" "SnapToTarget" "SnapToTarget" true))
  (return _returnvalue))

(fn `OnItemEquipped`
  (bind _dataasset (`self.DataAsset`))
  (`parent.OnItemEquipped`)
  (bind _equipmentcomponent (`self.EquipmentComponent`)
    (:`then`
      (`/Game/Library/InventoryandEquipment/Blueprints/Components/EquipmentComponent.Set Active Equipped Item Actor` _equipmentcomponent "NewEnumerator9" self)
      (`/Game/Library/InventoryandEquipment/Blueprints/Components/EquipmentComponent.SetOffhandWeaponActor` (`self.EquipmentComponent`) self)
      (`/Engine/EditorBlueprintResources/StandardMacros.IsValid` _dataasset
        (:`Is Valid`
          (`/Game/Library/InventoryandEquipment/Blueprints/Components/EquipmentComponent.Attach Equip Slot Actor` (`self.EquipmentComponent`) "NewEnumerator9" true (select `bool` (`/Game/Library/InventoryandEquipment/Blueprints/Components/EquipmentComponent.Is Combat Enabled?` (`self.EquipmentComponent`)) :`false` (`BlueprintMapLibrary.Map_Find` (`/Game/Library/InventoryandEquipment/Blueprints/Items/RPGItem.UnEquipSocket` _dataasset) "NewEnumerator18") :`true` (`BlueprintMapLibrary.Map_Find` (`/Game/Library/InventoryandEquipment/Blueprints/Items/RPGItem.EquipSocket` _dataasset) "NewEnumerator9")) "NewEnumerator18"))))
    (:`else`)))

(fn `OnItemUnequipped`
  (`parent.OnItemUnequipped`)
  (`self.SetItemEquipped` false))

(fn `UserConstructionScript`
  (`parent.UserConstructionScript`))