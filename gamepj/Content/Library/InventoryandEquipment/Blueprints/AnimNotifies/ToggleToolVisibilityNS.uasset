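; Anim notify state that shows an equipped tool actor only for the span of the notify within an animation.
; On begin and end it gets the owner's EquipmentComponent and looks up the active equipped actor in one fixed slot, presumably the tool slot.
; If that actor is valid, it unhides it in game on begin and hides it again on end.
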(fn `Received_NotifyBegin`
  (params (MeshComp :type "SkeletalMeshComponent Object Reference") (Animation :type "AnimSequenceBase Object Reference") (TotalDuration :type "Float (double-precision)"))
  (returns (ReturnValue :type Boolean))
  (bind _value (`/Game/Library/InventoryandEquipment/Blueprints/Components/EquipmentComponent.GetActiveEquippedSlotActor` (`Actor.GetComponentByClass` (`ActorComponent.GetOwner` MeshComp) "/Game/Library/InventoryandEquipment/Blueprints/Components/EquipmentComponent.EquipmentComponent_C") "NewEnumerator21"))
  (`/Engine/EditorBlueprintResources/StandardMacros.IsValid` _value
    (:`Is Valid`
      (`Actor.SetActorHiddenInGame` _value false)
      (return true))
    (:`Is Not Valid`
      (return false))))

(fn `Received_NotifyEnd`
  (params (MeshComp :type "SkeletalMeshComponent Object Reference") (Animation :type "AnimSequenceBase Object Reference"))
  (returns (ReturnValue :type Boolean))
  (bind _value (`/Game/Library/InventoryandEquipment/Blueprints/Components/EquipmentComponent.GetActiveEquippedSlotActor` (`Actor.GetComponentByClass` (`ActorComponent.GetOwner` MeshComp) "/Game/Library/InventoryandEquipment/Blueprints/Components/EquipmentComponent.EquipmentComponent_C") "NewEnumerator21"))
  (`/Engine/EditorBlueprintResources/StandardMacros.IsValid` _value
    (:`Is Valid`
      (`Actor.SetActorHiddenInGame` _value true)
      (return true))
    (:`Is Not Valid`
      (return true))))