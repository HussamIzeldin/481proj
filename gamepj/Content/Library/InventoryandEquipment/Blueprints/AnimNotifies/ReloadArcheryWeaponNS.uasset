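; Anim notify state that handles the arrow and quiver during an archery weapon reload animation.
; On begin, it finds the active archery weapon through the owner's EquipmentComponent, shows and attaches the arrow, then sends the active slot's held amount to the equipped quiver actor, if valid.
; On end, it calls AttachArrow with false on the weapon to switch the attachment state back.
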(fn `Received_NotifyBegin`
  (params (MeshComp :type "SkeletalMeshComponent Object Reference") (Animation :type "AnimSequenceBase Object Reference") (TotalDuration :type "Float (double-precision)"))
  (returns (ReturnValue :type Boolean))
  (bind _returnvalue (`Actor.GetComponentByClass` (`ActorComponent.GetOwner` MeshComp) "/Game/Library/InventoryandEquipment/Blueprints/Components/EquipmentComponent.EquipmentComponent_C"))
  (bind _value (`/Game/Library/InventoryandEquipment/Blueprints/Components/EquipmentComponent.GetActiveEquippedSlotActor` _returnvalue "NewEnumerator13"))
  (`/Engine/EditorBlueprintResources/StandardMacros.IsValid` _returnvalue
    (:`Is Valid`
      (bind _asarchery_weapon_parent_bp (cast `/Game/Library/InventoryandEquipment/Blueprints/Actors/ArcheryWeaponParent_BP` (`/Game/Library/InventoryandEquipment/Blueprints/Components/EquipmentComponent.GetActiveEquippedSlotActor` _returnvalue "NewEnumerator11"))
        (:`then`
          (`/Game/Library/InventoryandEquipment/Blueprints/Actors/ArcheryWeaponParent_BP.UpdateArrowVisibility` _asarchery_weapon_parent_bp true)
          (`/Game/Library/InventoryandEquipment/Blueprints/Actors/ArcheryWeaponParent_BP.AttachArrow` _asarchery_weapon_parent_bp true)
          (`/Engine/EditorBlueprintResources/StandardMacros.IsValid` _value
            (:`Is Valid`
              (message `/Game/Library/InventoryandEquipment/Blueprints/Interfaces/WorldItemBPI.UpdateQuiver` _value (`/Game/Library/InventoryandEquipment/Blueprints/Components/EquipmentComponent.GetHeldAmountForActiveSlot` _returnvalue "NewEnumerator20"))
              (return true))))
        (:`CastFailed`
          _)))
    (:`Is Not Valid`
      _))
  (return false))

(fn `Received_NotifyEnd`
  (params (MeshComp :type "SkeletalMeshComponent Object Reference") (Animation :type "AnimSequenceBase Object Reference"))
  (returns (ReturnValue :type Boolean))
  (bind _returnvalue (`Actor.GetComponentByClass` (`ActorComponent.GetOwner` MeshComp) "/Game/Library/InventoryandEquipment/Blueprints/Components/EquipmentComponent.EquipmentComponent_C"))
  (`/Engine/EditorBlueprintResources/StandardMacros.IsValid` _returnvalue
    (:`Is Valid`
      (bind _asarchery_weapon_parent_bp (cast `/Game/Library/InventoryandEquipment/Blueprints/Actors/ArcheryWeaponParent_BP` (`/Game/Library/InventoryandEquipment/Blueprints/Components/EquipmentComponent.GetActiveEquippedSlotActor` _returnvalue "NewEnumerator11"))
        (:`then`
          (`/Game/Library/InventoryandEquipment/Blueprints/Actors/ArcheryWeaponParent_BP.AttachArrow` _asarchery_weapon_parent_bp false)
          (return true))
        (:`CastFailed`
          _)))
    (:`Is Not Valid`
      _))
  (return false))