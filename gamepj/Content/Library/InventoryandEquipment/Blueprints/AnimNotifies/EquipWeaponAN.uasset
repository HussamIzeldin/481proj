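; Animation notify that completes equipping a weapon at a chosen frame of an animation.
; It looks up the EquipmentComponent on the mesh's owner and, if present, enables the configured equip slot and turns combat on.
; It then attaches that slot's actor, optionally to the socket named on the notify instead of the default, and returns the attach result.
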(fn `Received_Notify`
  (params (MeshComp :type "SkeletalMeshComponent Object Reference") (Animation :type "AnimSequenceBase Object Reference"))
  (returns (ReturnValue :type Boolean))
  (bind _returnvalue (`Actor.GetComponentByClass` (`ActorComponent.GetOwner` MeshComp) "/Game/Library/InventoryandEquipment/Blueprints/Components/EquipmentComponent.EquipmentComponent_C"))
  (`/Engine/EditorBlueprintResources/StandardMacros.IsValid` _returnvalue
    (:`Is Valid`
      (`/Game/Library/InventoryandEquipment/Blueprints/Components/EquipmentComponent.SetSlotDisabled` _returnvalue (`self.EquipSlot`) false)
      (`/Game/Library/InventoryandEquipment/Blueprints/Components/EquipmentComponent.SetCombatEnabled` _returnvalue true)
      (bind _success_ (`/Game/Library/InventoryandEquipment/Blueprints/Components/EquipmentComponent.Attach Equip Slot Actor` _returnvalue (`self.EquipSlot`) (`self.UseNotifySocketName?`) (`self.EquipSocket`) "NewEnumerator18"))
      (return _success_))))