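; Anim notify state that temporarily hides the actor equipped in a chosen slot while part of an animation plays.
; On begin, it hides that actor only if combat is enabled, the slot is not disabled and its item derives from the class mapped to that slot.
; On end, it unhides the chosen slot's actor and also a second, hardcoded slot's actor, without repeating those checks.
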(fn `Received_NotifyBegin`
  (params (MeshComp :type "SkeletalMeshComponent Object Reference") (Animation :type "AnimSequenceBase Object Reference") (TotalDuration :type "Float (double-precision)"))
  (returns (ReturnValue :type Boolean))
  (bind _returnvalue (`ActorComponent.GetOwner` MeshComp))
  (bind _equipslottohide (`self.EquipSlotToHide`))
  (bind _returnvalue_2 (`Actor.GetComponentByClass` _returnvalue "/Game/Library/InventoryandEquipment/Blueprints/Components/EquipmentComponent.EquipmentComponent_C"))
  (bind _value (`/Game/Library/InventoryandEquipment/Blueprints/Components/EquipmentComponent.GetActiveEquippedSlotActor` _returnvalue_2 (`self.EquipSlotToHide`)))
  (bind _item_item (break `/Game/Library/InventoryandEquipment/Blueprints/Structs/ItemSlot_Struct` (`/Game/Library/InventoryandEquipment/Blueprints/Components/EquipmentComponent.GetActiveEquippedSlotItem` _returnvalue_2 _equipslottohide)))
  (bind _combatmode (message `/Game/Library/CombatSystem/Blueprints/Interfaces/CombatBPI.CombatEnabled?` _returnvalue))
  (if _combatmode
    (if (not (`/Game/Library/InventoryandEquipment/Blueprints/Components/EquipmentComponent.Is Equip Slot Disabled?` _returnvalue_2 (`self.EquipSlotToHide`)))
      (`/Engine/EditorBlueprintResources/StandardMacros.IsValid` _value
        (:`Is Valid`
          (`/Engine/EditorBlueprintResources/StandardMacros.IsValid` _item_item
            (:`Is Valid`
              (if (`KismetMathLibrary.ClassIsChildOf` (`GameplayStatics.GetObjectClass` _item_item) (`BlueprintMapLibrary.Map_Find` (`self.ParentClassToHide`) _equipslottohide))
                (`Actor.SetActorHiddenInGame` _value true)
                (return true)
                (else
                  (return false))))
            (:`Is Not Valid`
              _)))
        (:`Is Not Valid`
          _))))
  (return false))

(fn `Received_NotifyEnd`
  (params (MeshComp :type "SkeletalMeshComponent Object Reference") (Animation :type "AnimSequenceBase Object Reference"))
  (returns (ReturnValue :type Boolean))
  (bind _returnvalue (`Actor.GetComponentByClass` (`ActorComponent.GetOwner` MeshComp) "/Game/Library/InventoryandEquipment/Blueprints/Components/EquipmentComponent.EquipmentComponent_C"))
  (bind _value (`/Game/Library/InventoryandEquipment/Blueprints/Components/EquipmentComponent.GetActiveEquippedSlotActor` _returnvalue (`self.EquipSlotToHide`)))
  (bind _value_2 (`/Game/Library/InventoryandEquipment/Blueprints/Components/EquipmentComponent.GetActiveEquippedSlotActor` _returnvalue "NewEnumerator11"))
  (if (`KismetSystemLibrary.IsValid` _value)
    (`Actor.SetActorHiddenInGame` _value false))
  (`/Engine/EditorBlueprintResources/StandardMacros.IsValid` _value_2
    (:`Is Valid`
      (`Actor.SetActorHiddenInGame` _value_2 false)
      (return true))
    (:`Is Not Valid`
      (return false))))