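; Anim notify that triggers item use on the animated mesh's owner at a set point in an animation.
; With UseEquippedTool set, it calls UseActiveSlotItem on the owner's EquipmentComponent for a fixed enum value.
; Otherwise it has the InventoryComponent immediately use its last used item, falling back to the equipment path if no valid inventory exists.
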(fn `Received_Notify`
  (params (MeshComp :type "SkeletalMeshComponent Object Reference") (Animation :type "AnimSequenceBase Object Reference"))
  (returns (ReturnValue :type Boolean))
  (bind _returnvalue (`Actor.GetComponentByClass` (`ActorComponent.GetOwner` MeshComp) "/Game/Library/InventoryandEquipment/Blueprints/Components/InventoryComponent.InventoryComponent_C"))
  (if (`self.UseEquippedTool`)
    (`/Game/Library/InventoryandEquipment/Blueprints/Components/EquipmentComponent.UseActiveSlotItem` (`Actor.GetComponentByClass` (`ActorComponent.GetOwner` MeshComp) "/Game/Library/InventoryandEquipment/Blueprints/Components/EquipmentComponent.EquipmentComponent_C") "NewEnumerator21" :!label _label)
    (else
      (`/Engine/EditorBlueprintResources/StandardMacros.IsValid` _returnvalue
        (:`Is Valid`
          (`/Game/Library/InventoryandEquipment/Blueprints/Components/InventoryComponent.Use Item` _returnvalue (`/Game/Library/InventoryandEquipment/Blueprints/Components/InventoryComponent.GetLastUsedItem` _returnvalue) true))
        (:`Is Not Valid`
          (goto _label)))))
  (return true))