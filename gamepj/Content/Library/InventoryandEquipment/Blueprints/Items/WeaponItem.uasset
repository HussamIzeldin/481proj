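; WeaponItem is a weapon item Blueprint in the inventory and equipment library that supplies impact effects and physical damage.
; GetImpactEffect maps an impact decision to a general, blocked, perfect block, parry or defense break effect, with none assigned for the None case.
; GetPhysicalDamage returns the value of the item's modifier for a single stat enum entry.
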(fn `GetImpactEffect`
  (params (ImpactDecision :type "/Game/Library/CombatSystem/Blueprints/Enums/E_ImpactDecision Enum" :default "NewEnumerator5"))
  (returns (ImpactEffect :type "/Game/Library/CombatSystem/Blueprints/ImpactEffects/ImpactEffect_Base Class Reference"))
  (return (select `/Game/Library/CombatSystem/Blueprints/Enums/E_ImpactDecision` ImpactDecision :`NewEnumerator0` (`self.GeneralImpactEffect`) :`NewEnumerator1` (`self.BlockedImpactEffect`) :`NewEnumerator3` (`self.PerfectBlockImpactEffect`) :`NewEnumerator4` (`self.ParryImpactEffect`) :`NewEnumerator6` (`self.DefenseBreakImpactEffect`))))

(fn `GetPhysicalDamage`
  (returns (ReturnValue :type "Float (double-precision)"))
  (return (`.Value_15_37105C9C4BDE6B2DECE3298F933045F1` (break `/Game/Library/CombatSystem/Blueprints/Structs/Stats/ItemStatModifier_Struct` (`self.GetModifierForStat` "NewEnumerator21")))))