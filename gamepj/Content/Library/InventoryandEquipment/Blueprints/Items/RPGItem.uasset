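; RPGItem is an item definition for the inventory and equipment system, exposing queries on stacking, resale value, stats and type.
; Equip sockets are looked up by slot; unequip sockets first remap the slot through an inline three-entry map.
; Weapon detection combines item type and hand type checks.
; UseItem is empty, physical damage returns zero and impact effect ignores its input, apparently as defaults for subclasses.
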(fn `CanStack?`
  (returns (Condition :type Boolean))
  (return (> (`self.MaxCount`) 1)))

(fn `FindEquipSocket`
  (params (EquipSlot :type "/Game/Library/InventoryandEquipment/Blueprints/Enums/Equipment/E_EquipSlots Enum" :default "NewEnumerator2"))
  (returns (Value :type Name))
  (return (`BlueprintMapLibrary.Map_Find` (`self.EquipSocket`) EquipSlot)))

(fn `FindUnEquipSocket`
  (params (EquipSlot :type "/Game/Library/InventoryandEquipment/Blueprints/Enums/Equipment/E_EquipSlots Enum" :default "NewEnumerator2"))
  (returns (Value :type Name))
  (return (`BlueprintMapLibrary.Map_Find` (`self.UnEquipSocket`) (`BlueprintMapLibrary.Map_Find` (`|MakeMap` "NewEnumerator11" "NewEnumerator19" "NewEnumerator9" "NewEnumerator18" "NewEnumerator25" "NewEnumerator24" :!type "/Game/Library/InventoryandEquipment/Blueprints/Enums/Equipment/E_EquipSlots Enum" :!valuetype "/Game/Library/InventoryandEquipment/Blueprints/Enums/Equipment/E_UnequipSlots Enum") EquipSlot))))

(fn `Get Un Equip Socket for Equip Slot`
  (params (InEquipSlot :type "/Game/Library/InventoryandEquipment/Blueprints/Enums/Equipment/E_EquipSlots Enum" :default "NewEnumerator2"))
  (returns (Value :type Name))
  (return (`BlueprintMapLibrary.Map_Find` (`self.UnEquipSocket`) (`BlueprintMapLibrary.Map_Find` (`|MakeMap` "NewEnumerator11" "NewEnumerator19" "NewEnumerator9" "NewEnumerator18" "NewEnumerator25" "NewEnumerator24" :!type "/Game/Library/InventoryandEquipment/Blueprints/Enums/Equipment/E_EquipSlots Enum" :!valuetype "/Game/Library/InventoryandEquipment/Blueprints/Enums/Equipment/E_UnequipSlots Enum") InEquipSlot))))

(fn `GetEquipSocket`
  (returns (Value :type Name))
  (return (`BlueprintMapLibrary.Map_Find` (`self.EquipSocket`) (`self.EquipSlot`))))

(fn `GetImpactEffect`
  (params (ImpactDecision :type "/Game/Library/CombatSystem/Blueprints/Enums/E_ImpactDecision Enum" :default "NewEnumerator5"))
  (returns (ImpactEffect :type "/Game/Library/CombatSystem/Blueprints/ImpactEffects/ImpactEffect_Base Class Reference"))
  (return (`self.GeneralImpactEffect`)))

(fn `GetItemStatValue`
  (params (Stat :type "/Game/Library/CombatSystem/Blueprints/Enums/Stats/E_Stats Enum" :default "NewEnumerator0"))
  (returns (Value :type "Float (double-precision)"))
  (return (`.Value_15_37105C9C4BDE6B2DECE3298F933045F1` (break `/Game/Library/CombatSystem/Blueprints/Structs/Stats/ItemStatModifier_Struct` (`BlueprintMapLibrary.Map_Find` (`self.ItemStats`) Stat)))))

(fn `GetModifierForStat`
  (params (Stat :type "/Game/Library/CombatSystem/Blueprints/Enums/Stats/E_Stats Enum" :default "NewEnumerator0"))
  (returns (Value :type "/Game/Library/CombatSystem/Blueprints/Structs/Stats/ItemStatModifier_Struct Structure"))
  (return (`BlueprintMapLibrary.Map_Find` (`self.ItemStats`) Stat)))

(fn `GetPhysicalDamage`
  (returns (ReturnValue :type "Float (double-precision)"))
  (return 0.0))

(fn `GetResellValue`
  (returns (Value :type Integer))
  (return (`KismetMathLibrary.FTrunc` (* (`self.Price`) (`self.Resell Value Multiplier`)))))

(fn `GetRoomOnStack`
  (params (`Amount ` :type Integer))
  (returns (ReturnValue :type Integer))
  (return (- (`self.MaxCount`) `Amount `)))

(fn `GetUnEquipSocket`
  (returns (Value :type Name))
  (return (`self.Get Un Equip Socket for Equip Slot` (`self.EquipSlot`))))

(fn `IsWeapon?`
  (returns (ReturnValue :type Boolean))
  (bind _itemtype (`self.ItemType`))
  (return (or (`|EnumEquality` _itemtype "NewEnumerator1") (`|EnumEquality` _itemtype "NewEnumerator4") (`|EnumEquality` _itemtype "NewEnumerator8") (`|EnumInequality` (`self.WeaponHandType`) "NewEnumerator2"))))

(fn `UseItem`
  (params (Caller :type "Actor Object Reference")))