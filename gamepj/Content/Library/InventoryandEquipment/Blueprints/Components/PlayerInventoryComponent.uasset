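; Player-side inventory component that extends a base inventory with item dropping, equipping and UI hookups.
; Dropping uses traces to pick a spot, tries merging into a PickUpActor_BP below or spawns one, then removes the amount from inventory.
; Equipping passes slot items to the owner's EquipmentComponent and flags them equipped; unequip is an empty stub.
; Initialization binds the pause-menu inventory widget, and obtained items optionally queue messages on the main HUD.
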(event `self.ReceiveBeginPlay`
  (`parent.ReceiveBeginPlay`)
  (bind _ascharacter (cast `Character` (`self.GetOwner`)))
  (set `self.OwnerCharacter` _ascharacter)
  (set `self.EquipmentComponent` (`Actor.GetComponentByClass` (`self.OwnerCharacter`) "/Game/Library/InventoryandEquipment/Blueprints/Components/EquipmentComponent.EquipmentComponent_C")))

(fn `DropItemAtIndex`
  (params (Item :type "/Game/Library/InventoryandEquipment/Blueprints/Structs/ItemSlot_Struct Structure") (Amount :type Integer))
  (returns (`Success?` :type Boolean))
  (locals (L_SpawnLocation :type "Vector Structure" :default (0.0 0.0 0.0)) (L_HitSomething :type Boolean :default false))
  (bind _returnvalue (`self.GetOwner`))
  (bind _returnvalue_2 (`self.GetOwner`))
  (bind (_item _amount _index _isequipped_ _guid) (break `/Game/Library/InventoryandEquipment/Blueprints/Structs/ItemSlot_Struct` (`local.Item`)))
  (bind (_item_2 _amount_2 _index_2 _isequipped__2 _guid_2) (break `/Game/Library/InventoryandEquipment/Blueprints/Structs/ItemSlot_Struct` (`local.Item`)))
  (bind ((`Amount_5_DD6A685B4B673304A94C98B9ACD032DF` _amount_3)) (break `/Game/Library/InventoryandEquipment/Blueprints/Structs/ItemSlot_Struct` (`local.Item`)))
  (bind (_condition _pick_up_actor) (`self.IsCollidingWithPickUpActor?` (`local.L_SpawnLocation`)))
  (bind _returnvalue_3 (`Actor.K2_GetActorLocation` _returnvalue_2))
  (bind _returnvalue_4 (+ (+ (`Actor.K2_GetActorLocation` _returnvalue) (* (`Actor.GetActorForwardVector` _returnvalue) 50.0)) (0.0 0.0 -50.0)))
  (if (and (`/Game/Library/InventoryandEquipment/Blueprints/Libraries/InventoryEquipmentLibrary.IsSlotItemValid?` (`local.Item`)) (> (`local.Amount`) 0))
    (bind (_outhit _returnvalue_5) (`KismetSystemLibrary.LineTraceSingle` _returnvalue_3 (+ _returnvalue_3 (* (`Actor.GetActorForwardVector` _returnvalue_2) 150.0)) "TraceTypeQuery1"))
    (set `local.L_HitSomething` _returnvalue_5)
    (set `local.L_SpawnLocation` (select `bool` (`local.L_HitSomething`) :`false` _returnvalue_4 :`true` (`Actor.K2_GetActorLocation` (`self.GetOwner`))))
    (if _condition
      (bind _output_get (set `self.ItemPickupActor` _pick_up_actor))
      (bind _success_ (`/Game/Library/InventoryandEquipment/Blueprints/Actors/PickUpActor_BP.Add Item` _output_get (make `/Game/Library/InventoryandEquipment/Blueprints/Structs/ItemSlot_Struct` _item_2 (`local.Amount`) 0 false _guid_2)))
      (if (not _success_)
        (set `local.L_SpawnLocation` (select `bool` (`local.L_HitSomething`) :`false` (`self.FindUniquePickUpSpawnLocation`) :`true` (`Actor.K2_GetActorLocation` (`self.GetOwner`))))
        (bind _returnvalue_6 (`|SpawnActorFromClass` "/Game/Library/InventoryandEquipment/Blueprints/Actors/PickUpActor_BP.PickUpActor_BP_C" (`KismetMathLibrary.MakeTransform` (`local.L_SpawnLocation`)) "AdjustIfPossibleButAlwaysSpawn" "OverrideRootScale" null (`|MakeArray` (make `/Game/Library/InventoryandEquipment/Blueprints/Structs/ItemSlot_Struct` _item (`local.Amount`) 0 false _guid) :!type "/Game/Library/InventoryandEquipment/Blueprints/Structs/ItemSlot_Struct Structure") true null :!label _label))
        (set `self.ItemPickupActor` _returnvalue_6))
      (else
        (set `local.L_SpawnLocation` (select `bool` (`local.L_HitSomething`) :`false` _returnvalue_4 :`true` (`Actor.K2_GetActorLocation` (`self.GetOwner`))))
        (goto _label)))
    (if (>= (`local.Amount`) _amount_3)
      (`self.Remove Item` (`local.Item`) _amount_3)
      (return true)
      (else
        (`self.Remove Item` (`local.Item`) (`local.Amount`))
        (return true)))
    (else
      (return false))))

(fn `EquipItemAtIndex`
  (params (InventoryPanel :type "/Game/Library/InventoryandEquipment/Blueprints/Enums/E_InventoryPanels Enum" :default "NewEnumerator0") (InventoryIndex :type Integer :default 0) (EquipmentIndex :type Integer :default 0))
  (locals (L_ItemToEquip :type "/Game/Library/InventoryandEquipment/Blueprints/Structs/ItemSlot_Struct Structure"))
  (bind _intentoryitem (`self.GetInventoryItem` InventoryPanel InventoryIndex))
  (if (`/Game/Library/InventoryandEquipment/Blueprints/Libraries/InventoryEquipmentLibrary.IsSlotItemValid?` _intentoryitem)
    (set `local.L_ItemToEquip` _intentoryitem)
    (`/Game/Library/InventoryandEquipment/Blueprints/Components/EquipmentComponent.Equip Item` (`self.EquipmentComponent`) (`local.L_ItemToEquip`) EquipmentIndex "NewEnumerator1")
    (`self.SetItemEquipped` (`local.InventoryPanel`) (`local.InventoryIndex`) true)))

(fn `InitializeInventory`
  (`parent.InitializeInventory`)
  (bind _menu (message `/Game/Library/CombatSystem/Blueprints/Interfaces/PlayerControllerBPI.GetPauseMenuWidget` (`GameplayStatics.GetPlayerController` 0)))
  (bind _aswb_player_inventory_menu (cast `/Game/Library/UI/InventoryEquipmentUI/Blueprints/WB_PlayerInventoryMenu` _menu))
  (`/Game/Library/UI/InventoryEquipmentUI/Blueprints/WB_PlayerInventoryMenu.Initialize` _aswb_player_inventory_menu self)
  (bind _wb_coreinventory (`/Game/Library/UI/InventoryEquipmentUI/Blueprints/WB_PlayerInventoryMenu.WB_CoreInventory` _aswb_player_inventory_menu))
  (`/Game/Library/UI/InventoryEquipmentUI/Blueprints/WB_CoreInventory.Initialize` _wb_coreinventory (`self.SlotsPerRow`) self)
  (set `self.WB_MainInventory` _wb_coreinventory)
  (if (not (`self.bCanShowObtainedMessage?`))
    (bind _mainhud (message `/Game/Library/CombatSystem/Blueprints/Interfaces/PlayerControllerBPI.GetMainHUD` (`GameplayStatics.GetPlayerController` 0)))
    (bind _asmain_hud (cast `/Game/Library/UI/CombatUI/Widgets/MainHUD` _mainhud))
    (`Widget.RemoveFromParent` (`/Game/Library/UI/CombatUI/Widgets/MainHUD.ObtainedItemOverlay` _asmain_hud))))

(fn `IsCollidingWithPickUpActor?`
  (params (Start :type "Vector Structure"))
  (returns (Condition :type Boolean) (`Pick Up Actor` :type "/Game/Library/InventoryandEquipment/Blueprints/Actors/PickUpActor_BP Object Reference"))
  (bind _start (`local.Start`))
  (`self.ItemPickupActor`
    (:`then`
      (bind _outhit (`KismetSystemLibrary.LineTraceSingleForObjects` _start (+ _start (0.0 0.0 -100.0)) (`|MakeArray` "ObjectTypeQuery7" :!type "EObjectTypeQuery Enum") false (`|MakeArray` (`self.GetOwner`))))
      (bind (_bblockinghit _binitialoverlap _time _distance _location _impactpoint _normal _impactnormal _physmat _hitactor) (`GameplayStatics.BreakHitResult` _outhit))
      (bind _aspick_up_actor_bp (cast `/Game/Library/InventoryandEquipment/Blueprints/Actors/PickUpActor_BP` _hitactor)
        (:`then`
          (return _bblockinghit _aspick_up_actor_bp))
        (:`CastFailed`
          (return false null))))
    (:`else`
      (return false null))))

(fn `ShowObtainedItem`
  (params (Item :type "/Game/Library/InventoryandEquipment/Blueprints/Items/RPGItem Object Reference") (Amount :type Integer))
  (returns (`Success?` :type Boolean))
  (if (`self.bCanShowObtainedMessage?`)
    (`self.WB_MainInventory`
      (:`then`
        (bind _mainhud (message `/Game/Library/CombatSystem/Blueprints/Interfaces/PlayerControllerBPI.GetMainHUD` (`GameplayStatics.GetPlayerController` 0)))
        (bind _asmain_hud (cast `/Game/Library/UI/CombatUI/Widgets/MainHUD` _mainhud))
        (`/Engine/EditorBlueprintResources/StandardMacros.IsValid` _asmain_hud
          (:`Is Valid`
            (`/Game/Library/UI/CombatUI/Widgets/MainHUD.Add Item to Obtained Que` _asmain_hud (`local.Item`) (`local.Amount`))
            (return true))))
      (:`else`
        (return false)))
    (else
      (return false))))

(fn `UnEquipItemAtIndex`
  (params (InventoryPanel :type "/Game/Library/InventoryandEquipment/Blueprints/Enums/E_InventoryPanels Enum" :default "NewEnumerator0") (InventoryIndex :type Integer) (EquipmentIndex :type Integer)))