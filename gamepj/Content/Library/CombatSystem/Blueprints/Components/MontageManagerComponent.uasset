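; Character component that picks the animation montage, play rate and timing for combat actions, attacks, dodges and counterattacks.
; It loads defaults from the data table's "Default" row and combat-type sets from a named row, while weapon montages are passed in.
; Lookups layer default, combat type, weapon, then Punisher mode for actions and attacks, with conditions on weapon attacks.
; Most indices are clamped, optionally randomized; some are cached for queries.
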(event `self.ReceiveBeginPlay`
  (bind _ascharacter (cast `Character` (`self.GetOwner`)))
  (set `self.OwnerCharacter` _ascharacter)
  (set `self.CombatComponent` (`Actor.GetComponentByClass` (`self.OwnerCharacter`) "/Game/Library/CombatSystem/Blueprints/Components/CombatComponent.CombatComponent_C"))
  (`self.SetDefaultMontages`))

(fn `Get All Default General Action Montges`
  (returns (DefaultActionMontages :type "Map of /Game/Library/CombatSystem/Blueprints/Enums/CombatEnums/E_CharacterAction Enum to /Game/Library/CombatSystem/Blueprints/Structs/ActionMontage_Struct Structure"))
  (return (`self.DefaultGeneralActionMontages`)))

(fn `GetActionMontageFromItem`
  (params (CombatAction :type "/Game/Library/CombatSystem/Blueprints/Enums/CombatEnums/E_CharacterAction Enum" :default "NewEnumerator0") (MontageIndex :type Integer) (`RandomIndex?` :type Boolean) (SlotItem :type "/Game/Library/InventoryandEquipment/Blueprints/Structs/ItemSlot_Struct Structure (by ref)"))
  (returns (AnimMontage :type "AnimMontage Object Reference") (PlayRate :type "Float (double-precision)") (InTimeToStartMontageAt :type "Float (double-precision)") (ResetTimeMultiplier :type "Float (double-precision)"))
  (locals (L_ActionMontageStruct :type "/Game/Library/CombatSystem/Blueprints/Structs/ActionMontage_Struct Structure") (L_RandomIndex :type Integer) (L_LastIndex :type Integer :default 0))
  (bind _l_lastindex (`local.L_LastIndex`))
  (bind _actionmontages (break `/Game/Library/CombatSystem/Blueprints/Structs/ActionMontage_Struct` (`local.L_ActionMontageStruct`)))
  (bind _returnvalue (select `bool` (`local.RandomIndex?`) :`false` (`local.MontageIndex`) :`true` (`local.L_RandomIndex`)))
  (bind _returnvalue_2 (`KismetArrayLibrary.Array_LastIndex` _actionmontages))
  (bind (_value _returnvalue_3) (`BlueprintMapLibrary.Map_Find` (`.ActionMontages_15_715B4510444C15844C29FF847D7B0AF0` (break `/Game/Library/InventoryandEquipment/Blueprints/Structs/ItemMontages_Struct` (`/Game/Library/InventoryandEquipment/Blueprints/Libraries/InventoryEquipmentLibrary.Get Item Montages` SlotItem))) (`local.CombatAction`)))
  (bind (_animmontage _playrate _intimetostartmontageat _resettimemultiplier) (break `/Game/Library/CombatSystem/Blueprints/Structs/AnimMontage_Struct` (`|GetArrayItem` _actionmontages (select `bool` (> _returnvalue _l_lastindex) :`false` _returnvalue :`true` _l_lastindex))))
  (set `local.L_ActionMontageStruct` _value)
  (if _returnvalue_3
    (set `local.L_LastIndex` _returnvalue_2)
    (set `local.L_RandomIndex` (`KismetMathLibrary.RandomIntegerInRange` 0 _returnvalue_2))
    (`/Engine/EditorBlueprintResources/StandardMacros.IsValid` _animmontage
      (:`Is Valid`
        (return _animmontage _playrate _intimetostartmontageat _resettimemultiplier))
      (:`Is Not Valid`
        (return null 0.0 0.0 0.0)))
    (else
      (return null 0.0 0.0 0.0))))

(fn `GetAllAttackMontges`
  (returns (AttackMontages :type "Map of /Game/Library/CombatSystem/Blueprints/Enums/CombatEnums/E_AttackTypes Enum to /Game/Library/CombatSystem/Blueprints/Structs/ActionMontage_Struct Structure"))
  (return (`self.AttackMontages`)))

(fn `GetAllCombatTypeRollDodgeMontges`
  (returns (CombatTypeRollDodgeMontages :type "Map of /Game/Library/CombatSystem/Blueprints/Enums/E_DodgeDirection Enum to /Game/Library/CombatSystem/Blueprints/Structs/ActionMontage_Struct Structure"))
  (return (`self.CombatTypeRollDodgeMontages`)))

(fn `GetAllCombatTypeStepDodgeMontges`
  (returns (CombatTypeStepDodgeMontages :type "Map of /Game/Library/CombatSystem/Blueprints/Enums/E_DodgeDirection Enum to /Game/Library/CombatSystem/Blueprints/Structs/ActionMontage_Struct Structure"))
  (return (`self.CombatTypeStepDodgeMontages`)))

(fn `GetAllDefaultAttackMontges`
  (returns (DefaultAttackMontages :type "Map of /Game/Library/CombatSystem/Blueprints/Enums/CombatEnums/E_AttackTypes Enum to /Game/Library/CombatSystem/Blueprints/Structs/ActionMontage_Struct Structure"))
  (return (`self.DefaultAttackMontages`)))

(fn `GetAllDefaultRollDodgeMontges`
  (returns (DefaultRollDodgeMontages :type "Map of /Game/Library/CombatSystem/Blueprints/Enums/E_DodgeDirection Enum to /Game/Library/CombatSystem/Blueprints/Structs/ActionMontage_Struct Structure"))
  (return (`self.DefaultRollDodgeMontages`)))

(fn `GetAllDefaultStepDodgeMontges`
  (returns (DefaultStepDodgeMontages :type "Map of /Game/Library/CombatSystem/Blueprints/Enums/E_DodgeDirection Enum to /Game/Library/CombatSystem/Blueprints/Structs/ActionMontage_Struct Structure"))
  (return (`self.DefaultStepDodgeMontages`)))

(fn `GetAllGeneralActionMontges`
  (returns (GeneralActionMontages :type "Map of /Game/Library/CombatSystem/Blueprints/Enums/CombatEnums/E_CharacterAction Enum to /Game/Library/CombatSystem/Blueprints/Structs/ActionMontage_Struct Structure"))
  (return (`self.GeneralActionMontages`)))

(fn `GetAllPunisherModeActionMontges`
  (returns (PunisherModeActionMontages :type "Map of /Game/Library/CombatSystem/Blueprints/Enums/CombatEnums/E_CharacterAction Enum to /Game/Library/CombatSystem/Blueprints/Structs/ActionMontage_Struct Structure"))
  (return (`self.PunisherModeActionMontages`)))

(fn `GetAllPunisherModeAttackMontges`
  (returns (PunisherModeAttackMontages :type "Map of /Game/Library/CombatSystem/Blueprints/Enums/CombatEnums/E_AttackTypes Enum to /Game/Library/CombatSystem/Blueprints/Structs/ActionMontage_Struct Structure"))
  (return (`self.PunisherModeAttackMontages`)))

(fn `GetAttackMontage`
  (params (AttackType :type "/Game/Library/CombatSystem/Blueprints/Enums/CombatEnums/E_AttackTypes Enum" :default "NewEnumerator15") (AttackIndex :type Integer) (`RandomIndex?` :type Boolean))
  (returns (AnimMontage :type "AnimMontage Object Reference") (PlayRate :type "Float (double-precision)") (InTimeToStartMontageAt :type "Float (double-precision)") (ResetTimeMultiplier :type "Float (double-precision)"))
  (locals (L_CommonMontage :type Boolean) (L_Struct :type "/Game/Library/CombatSystem/Blueprints/Structs/ActionMontage_Struct Structure") (L_CombatTypeMontageFound :type Boolean) (L_WeaponSpecific :type Boolean) (L_PunisherModeAction :type Boolean) (L_RandomIndex :type Integer))
  (bind _attacktype (`local.AttackType`))
  (bind _attackmontagelastindex (`self.AttackMontageLastIndex`))
  (bind _actionmontages (break `/Game/Library/CombatSystem/Blueprints/Structs/ActionMontage_Struct` (`local.L_Struct`)))
  (bind (_value _returnvalue) (`BlueprintMapLibrary.Map_Find` (`self.WeaponAttackMontages`) _attacktype))
  (bind (_value_2 _returnvalue_2) (`BlueprintMapLibrary.Map_Find` (`self.GetAllPunisherModeAttackMontges`) (`local.AttackType`)))
  (bind (_value_3 _returnvalue_3) (`BlueprintMapLibrary.Map_Find` (`self.GetAllAttackMontges`) (`local.AttackType`)))
  (bind (_value_4 _returnvalue_4) (`BlueprintMapLibrary.Map_Find` (`self.GetAllDefaultAttackMontges`) (`local.AttackType`)))
  (bind _returnvalue_5 (select `bool` (`local.RandomIndex?`) :`false` (`local.AttackIndex`) :`true` (`local.L_RandomIndex`)))
  (bind _output_get (set `local.L_CommonMontage` _returnvalue_4))
  (if _output_get
    (set `local.L_Struct` _value_4) ; Common Row Attack Montages
  )
  (bind _output_get_2 (set `local.L_CombatTypeMontageFound` _returnvalue_3))
  (if _output_get_2
    (set `local.L_Struct` _value_3) ; Combat Type Attack Montages
  )
  (bind _output_get_3 (set `local.L_WeaponSpecific` (and _returnvalue (or (`|EnumEquality` _attacktype "NewEnumerator10") (and (not (`/Game/Library/CombatSystem/Blueprints/Components/CombatComponent.isPunisherMode?` (`self.CombatComponent`))) (not (`local.L_CommonMontage`)))))))
  (if _output_get_3
    (set `local.L_Struct` _value) ; Weapon Attack Montages
  )
  (bind _output_get_4 (set `local.L_PunisherModeAction` (and (`/Game/Library/CombatSystem/Blueprints/Components/CombatComponent.isPunisherMode?` (`self.CombatComponent`)) _returnvalue_2)))
  (if _output_get_4
    (set `local.L_Struct` _value_2) ; Punisher Mode Attack Montages
  )
  (if (or (`local.L_CombatTypeMontageFound`) (`local.L_WeaponSpecific`) (`local.L_CommonMontage`) (`local.L_PunisherModeAction`))
    (bind _output_get_5 (set `self.AttackMontageLastIndex` (`KismetArrayLibrary.Array_LastIndex` _actionmontages)))
    (set `local.L_RandomIndex` (`KismetMathLibrary.RandomIntegerInRange` 0 _output_get_5))
    (bind _output_get_6 (set `self.CurrentAttackMontageIndex` (select `bool` (> _returnvalue_5 _attackmontagelastindex) :`false` _returnvalue_5 :`true` _attackmontagelastindex)))
    (bind _output_get_7 (set `self.LastAttackMontage` (`|GetArrayItem` _actionmontages _output_get_6)))
    (bind (_animmontage _playrate _intimetostartmontageat _resettimemultiplier) (break `/Game/Library/CombatSystem/Blueprints/Structs/AnimMontage_Struct` _output_get_7))
    (`/Engine/EditorBlueprintResources/StandardMacros.IsValid` _animmontage
      (:`Is Valid`
        (return _animmontage _playrate _intimetostartmontageat _resettimemultiplier))
      (:`Is Not Valid`
        (return null 0.0 0.0 0.0)))
    (else
      (return null 0.0 0.0 0.0))))

(fn `GetAttackMontageIndex`
  (returns (MontageIndex :type Integer))
  (return (`self.CurrentAttackMontageIndex`)))

(fn `GetAttackMontageLastIndex`
  (returns (LastIndex :type Integer))
  (return (`self.AttackMontageLastIndex`)))

(fn `GetCounterAttackMontage`
  (params (Direction :type "/Game/Library/CombatSystem/Blueprints/Enums/CombatEnums/E_HitFacingDirection Enum" :default "NewEnumerator5"))
  (returns (AnimMontage :type "AnimMontage Object Reference") (PlayRate :type "Float (double-precision)") (InTimeToStartMontageAt :type "Float (double-precision)") (ResetTimeMultiplier :type "Float (double-precision)"))
  (bind (_value _returnvalue) (`BlueprintMapLibrary.Map_Find` (`self.CounterAttacks`) Direction))
  (bind (_animmontage _playrate _intimetostartmontageat _resettimemultiplier) (break `/Game/Library/CombatSystem/Blueprints/Structs/AnimMontage_Struct` _value))
  (if (and _returnvalue (`KismetSystemLibrary.IsValid` (`.AnimMontage_5_2620D50C4D110CA156B1A28F49A30836` (break `/Game/Library/CombatSystem/Blueprints/Structs/AnimMontage_Struct` _value))))
    (return _animmontage _playrate _intimetostartmontageat _resettimemultiplier)
    (else
      (return null 0.0 0.0 0.0))))

(fn `GetGeneralActionMontage`
  (params (CombatAction :type "/Game/Library/CombatSystem/Blueprints/Enums/CombatEnums/E_CharacterAction Enum" :default "NewEnumerator0") (MontageIndex :type Integer) (`RandomIndex?` :type Boolean))
  (returns (AnimMontage :type "AnimMontage Object Reference") (PlayRate :type "Float (double-precision)") (InTimeToStartMontageAt :type "Float (double-precision)") (ResetTimeMultiplier :type "Float (double-precision)"))
  (locals (L_SharedMontage :type Boolean) (L_ActionMontageStruct :type "/Game/Library/CombatSystem/Blueprints/Structs/ActionMontage_Struct Structure") (L_CombatTypeMontage :type Boolean) (L_WeaponSpecific :type Boolean) (L_PunisherModeAction :type Boolean) (L_RandomIndex :type Integer))
  (bind _generalcombatactionlastindex (`self.GeneralCombatActionLastIndex`))
  (bind _actionmontages (break `/Game/Library/CombatSystem/Blueprints/Structs/ActionMontage_Struct` (`local.L_ActionMontageStruct`)))
  (bind (_value _returnvalue) (`BlueprintMapLibrary.Map_Find` (`self.Get All Default General Action Montges`) (`local.CombatAction`)))
  (bind (_value_2 _returnvalue_2) (`BlueprintMapLibrary.Map_Find` (`self.GetAllPunisherModeActionMontges`) (`local.CombatAction`)))
  (bind (_value_3 _returnvalue_3) (`BlueprintMapLibrary.Map_Find` (`self.WeaponActionMontages`) (`local.CombatAction`)))
  (bind (_value_4 _returnvalue_4) (`BlueprintMapLibrary.Map_Find` (`self.GetAllGeneralActionMontges`) (`local.CombatAction`)))
  (bind _returnvalue_5 (select `bool` (`local.RandomIndex?`) :`false` (`local.MontageIndex`) :`true` (`local.L_RandomIndex`)))
  (bind _returnvalue_6 (`KismetArrayLibrary.Array_LastIndex` _actionmontages))
  (bind (_animmontage _playrate _intimetostartmontageat _resettimemultiplier) (break `/Game/Library/CombatSystem/Blueprints/Structs/AnimMontage_Struct` (`|GetArrayItem` _actionmontages (`self.GeneralCombatActionMontageIndex`))))
  (bind _output_get (set `local.L_SharedMontage` _returnvalue))
  (if _output_get
    (set `local.L_ActionMontageStruct` _value) ; Default Montage
  )
  (bind _output_get_2 (set `local.L_CombatTypeMontage` _returnvalue_4))
  (if _output_get_2
    (set `local.L_ActionMontageStruct` _value_4) ; Combat Type Montage
  )
  (bind _output_get_3 (set `local.L_WeaponSpecific` _returnvalue_3))
  (if _output_get_3
    (set `local.L_ActionMontageStruct` _value_3) ; Weapon Montage
  )
  (bind _output_get_4 (set `local.L_PunisherModeAction` (and (`/Game/Library/CombatSystem/Blueprints/Components/CombatComponent.isPunisherMode?` (`self.CombatComponent`)) _returnvalue_2)))
  (if _output_get_4
    (set `local.L_ActionMontageStruct` _value_2) ; Punisher Mode Montage
  )
  (if (or (`local.L_CombatTypeMontage`) (`local.L_WeaponSpecific`) (`local.L_SharedMontage`) (`local.L_PunisherModeAction`))
    (set `self.GeneralCombatActionLastIndex` _returnvalue_6)
    (set `local.L_RandomIndex` (`KismetMathLibrary.RandomIntegerInRange` 0 _returnvalue_6))
    (set `self.GeneralCombatActionMontageIndex` (select `bool` (> _returnvalue_5 _generalcombatactionlastindex) :`false` _returnvalue_5 :`true` _generalcombatactionlastindex))
    (`/Engine/EditorBlueprintResources/StandardMacros.IsValid` _animmontage
      (:`Is Valid`
        (return _animmontage _playrate _intimetostartmontageat _resettimemultiplier))
      (:`Is Not Valid`
        (return null 0.0 0.0 0.0)))
    (else
      (return null 0.0 0.0 0.0))))

(fn `GetGeneralCombatActionLastIndex`
  (returns (LastIndex :type Integer))
  (return (`self.GeneralCombatActionLastIndex`)))

(fn `GetGeneralCombatActionMontageIndex`
  (returns (MontageIndex :type Integer))
  (return (`self.GeneralCombatActionMontageIndex`)))

(fn `GetLastAttackMontage`
  (returns (LastAttackMontage :type "/Game/Library/CombatSystem/Blueprints/Structs/AnimMontage_Struct Structure"))
  (return (`self.LastAttackMontage`)))

(fn `GetRollDodgeMontage`
  (params (DodgeDirection :type "/Game/Library/CombatSystem/Blueprints/Enums/E_DodgeDirection Enum" :default "NewEnumerator8") (MontageIndex :type Integer))
  (returns (AnimMontage :type "AnimMontage Object Reference") (PlayRate :type "Float (double-precision)") (InTimeToStartMontageAt :type "Float (double-precision)") (ResetTimeMultiplier :type "Float (double-precision)"))
  (locals (L_CommonDodgeMontages :type Boolean) (L_MontageStruct :type "/Game/Library/CombatSystem/Blueprints/Structs/ActionMontage_Struct Structure") (L_CombatTypeSpecific :type Boolean) (L_WeaponSpecific :type Boolean))
  (bind _montageindex (`local.MontageIndex`))
  (bind _actionmontages (break `/Game/Library/CombatSystem/Blueprints/Structs/ActionMontage_Struct` (`local.L_MontageStruct`)))
  (bind (_value _returnvalue) (`BlueprintMapLibrary.Map_Find` (`self.WeaponRollDodgeMontages`) (`local.DodgeDirection`)))
  (bind (_value_2 _returnvalue_2) (`BlueprintMapLibrary.Map_Find` (`self.GetAllCombatTypeRollDodgeMontges`) (`local.DodgeDirection`)))
  (bind (_value_3 _returnvalue_3) (`BlueprintMapLibrary.Map_Find` (`self.GetAllDefaultRollDodgeMontges`) (`local.DodgeDirection`)))
  (bind _returnvalue_4 (`KismetArrayLibrary.Array_LastIndex` _actionmontages))
  (bind (_animmontage _playrate _intimetostartmontageat _resettimemultiplier) (break `/Game/Library/CombatSystem/Blueprints/Structs/AnimMontage_Struct` (`|GetArrayItem` _actionmontages (select `bool` (> _montageindex _returnvalue_4) :`false` _montageindex :`true` _returnvalue_4))))
  (bind _output_get (set `local.L_CommonDodgeMontages` _returnvalue_3))
  (if _output_get
    (set `local.L_MontageStruct` _value_3) ; Default montages
  )
  (bind _output_get_2 (set `local.L_CombatTypeSpecific` _returnvalue_2))
  (if _output_get_2
    (set `local.L_MontageStruct` _value_2) ; Combat Type Montages
  )
  (bind _output_get_3 (set `local.L_WeaponSpecific` _returnvalue))
  (if _output_get_3
    (set `local.L_MontageStruct` _value) ; Weapon Specific Montages
  )
  (if (or (`local.L_CommonDodgeMontages`) (`local.L_WeaponSpecific`) (`local.L_CombatTypeSpecific`))
    (`/Engine/EditorBlueprintResources/StandardMacros.IsValid` _animmontage
      (:`Is Valid`
        (return _animmontage _playrate _intimetostartmontageat _resettimemultiplier))
      (:`Is Not Valid`
        (return null 0.0 0.0 0.0)))
    (else
      (return null 0.0 0.0 0.0))))

(fn `GetStepDodgeMontage`
  (params (DodgeDirection :type "/Game/Library/CombatSystem/Blueprints/Enums/E_DodgeDirection Enum" :default "NewEnumerator8") (MontageIndex :type Integer))
  (returns (AnimMontage :type "AnimMontage Object Reference") (PlayRate :type "Float (double-precision)") (InTimeToStartMontageAt :type "Float (double-precision)") (ResetTimeMultiplier :type "Float (double-precision)"))
  (locals (L_CommonDodgeMontages :type Boolean) (L_MontageStruct :type "/Game/Library/CombatSystem/Blueprints/Structs/ActionMontage_Struct Structure") (L_CombatTypeSpecific :type Boolean) (L_WeaponSpecific :type Boolean))
  (bind _montageindex (`local.MontageIndex`))
  (bind _actionmontages (break `/Game/Library/CombatSystem/Blueprints/Structs/ActionMontage_Struct` (`local.L_MontageStruct`)))
  (bind (_value _returnvalue) (`BlueprintMapLibrary.Map_Find` (`self.WeaponStepDodgeMontages`) (`local.DodgeDirection`)))
  (bind (_value_2 _returnvalue_2) (`BlueprintMapLibrary.Map_Find` (`self.GetAllCombatTypeStepDodgeMontges`) (`local.DodgeDirection`)))
  (bind (_value_3 _returnvalue_3) (`BlueprintMapLibrary.Map_Find` (`self.GetAllDefaultStepDodgeMontges`) (`local.DodgeDirection`)))
  (bind _returnvalue_4 (`KismetArrayLibrary.Array_LastIndex` _actionmontages))
  (bind (_animmontage _playrate _intimetostartmontageat _resettimemultiplier) (break `/Game/Library/CombatSystem/Blueprints/Structs/AnimMontage_Struct` (`|GetArrayItem` _actionmontages (`self.StepDodgeIndex`))))
  (bind _output_get (set `local.L_CommonDodgeMontages` _returnvalue_3))
  (if _output_get
    (set `local.L_MontageStruct` _value_3) ; Common Montages
  )
  (bind _output_get_2 (set `local.L_CombatTypeSpecific` _returnvalue_2))
  (if _output_get_2
    (set `local.L_MontageStruct` _value_2) ; Combat Type Montages
  )
  (bind _output_get_3 (set `local.L_WeaponSpecific` _returnvalue))
  (if _output_get_3
    (set `local.L_MontageStruct` _value) ; Weapon Montages
  )
  (if (or (`local.L_CommonDodgeMontages`) (`local.L_WeaponSpecific`) (`local.L_CombatTypeSpecific`))
    (set `self.StepDodgeIndex` (select `bool` (> _montageindex _returnvalue_4) :`false` _montageindex :`true` _returnvalue_4))
    (`/Engine/EditorBlueprintResources/StandardMacros.IsValid` _animmontage
      (:`Is Valid`
        (return _animmontage _playrate _intimetostartmontageat _resettimemultiplier))
      (:`Is Not Valid`
        (return null 0.0 0.0 0.0)))
    (else
      (return null 0.0 0.0 0.0))))

(fn `GetStepDodgeMontageIndex`
  (returns (MontageIndex :type Integer))
  (return (`self.StepDodgeIndex`)))

(fn `ResetAttackMontageIndex`
  (set `self.AttackMontageLastIndex` 0)
  (set `self.CurrentAttackMontageIndex` 0))

(fn `SetDefaultMontages`
  (bind _returnvalue (`|GetDataTableRow` (`self.DataTable`) "Default")
    (:`then`
      (bind ((`OptionalCombatAbilities_230_49BC65744A6334773340BD870579443A` _optionalcombatabilities) (`GeneralActions_226_B43AD8FF45DFB3DE3D2E089C6315F96B` _generalactions) (`Attacks_229_126AF23643ABF3DFC0810BBF1B6F1330` _attacks) (`CounterAttacks_238_D68C402249C31428BD863F9F2436DE40` _counterattacks) (`DodgeDirection_94_8C0E0D504C241CF92E0F1ABC6DBE41F7` _dodgedirection)) (break `/Game/Library/CombatSystem/Blueprints/Structs/CombatMontages_Struct` _returnvalue))
      (set `self.DefaultGeneralActionMontages` _generalactions)
      (set `self.DefaultAttackMontages` _attacks)
      (bind (_dodgetype _rolldodgemontages _stepdodgemontages) (break `/Game/Library/CombatSystem/Blueprints/Structs/DodgeDirectionMap_Struct` _dodgedirection))
      (set `self.DefaultRollDodgeMontages` _rolldodgemontages)
      (set `self.DefaultStepDodgeMontages` _stepdodgemontages))))

(fn `UpdateMontages`
  (params (CombatType :type "/Game/Library/CombatSystem/Blueprints/Enums/CombatEnums/E_CombatType Enum" :default "NewEnumerator16") (CustomRowName :type Name) (`UseCustomRowName?` :type Boolean))
  (locals (L_RowName :type Name))
  (bind _returnvalue (`KismetStringLibrary.Conv_StringToName` (`|GetEnumeratorNameAsString` CombatType)))
  (if (`|EnumEquality` CombatType "NewEnumerator16")
    (`BlueprintMapLibrary.Map_Clear` (`self.GeneralActionMontages`))
    (`BlueprintMapLibrary.Map_Clear` (`self.CombatTypeRollDodgeMontages`))
    (`BlueprintMapLibrary.Map_Clear` (`self.PunisherModeActionMontages`))
    (`BlueprintMapLibrary.Map_Clear` (`self.CombatTypeStepDodgeMontages`))
    (`BlueprintMapLibrary.Map_Clear` (`self.AttackMontages`))
    (`BlueprintMapLibrary.Map_Clear` (`self.CounterAttacks`))
    (else
      (set `local.L_RowName` (select `bool` `UseCustomRowName?` :`false` _returnvalue :`true` CustomRowName))
      (bind _returnvalue_2 (`|GetDataTableRow` (`self.DataTable`) (`local.L_RowName`))
        (:`then`
          (bind ((`OptionalCombatAbilities_230_49BC65744A6334773340BD870579443A` _optionalcombatabilities) (`GeneralActions_226_B43AD8FF45DFB3DE3D2E089C6315F96B` _generalactions) (`Attacks_229_126AF23643ABF3DFC0810BBF1B6F1330` _attacks) (`CounterAttacks_238_D68C402249C31428BD863F9F2436DE40` _counterattacks) (`DodgeDirection_94_8C0E0D504C241CF92E0F1ABC6DBE41F7` _dodgedirection) (`PunisherModeMontages_169_ED7091B34B10DE4659A1CF903D91CDD8` _punishermodemontages)) (break `/Game/Library/CombatSystem/Blueprints/Structs/CombatMontages_Struct` _returnvalue_2))
          (set `self.GeneralActionMontages` _generalactions)
          (set `self.AttackMontages` _attacks)
          (bind ((`RollDodgeMontages_98_FD73ED40460FC9B9F22315810F90186C` _rolldodgemontages) (`StepDodgeMontages_99_E9A9B3F04D29592880F25591B286AA41` _stepdodgemontages)) (break `/Game/Library/CombatSystem/Blueprints/Structs/DodgeDirectionMap_Struct` _dodgedirection))
          (set `self.CombatTypeRollDodgeMontages` _rolldodgemontages)
          (set `self.CombatTypeStepDodgeMontages` _stepdodgemontages)
          (bind (_generalactions_2 _attacks_2) (break `/Game/Library/CombatSystem/Blueprints/Structs/PunisherModeMontage_Struct` _punishermodemontages))
          (set `self.PunisherModeActionMontages` _generalactions_2)
          (set `self.PunisherModeAttackMontages` _attacks_2)
          (set `self.CounterAttacks` _counterattacks)
          (`self.OnMontagesUpdated` (make `DataTableRowHandle` (`self.DataTable`) (`local.L_RowName`)))
          (return))
        (:`RowNotFound`
          (`KismetSystemLibrary.PrintString` (`KismetStringLibrary.Concat_StrStr` "Combat Type Row:" (`KismetStringLibrary.Conv_NameToString` _returnvalue) " NOT found") true true (struct :`R` 1.0 :`G` 0.05627 :`A` 1.0))
          (return))))))

(fn `UpdateWeaponMontages`
  (params (WeaponMontages :type "/Game/Library/InventoryandEquipment/Blueprints/Structs/ItemMontages_Struct Structure"))
  (bind (_actionmontages _attackmontages _rolldodgemontages _stepdodgemontages) (break `/Game/Library/InventoryandEquipment/Blueprints/Structs/ItemMontages_Struct` WeaponMontages))
  (set `self.WeaponActionMontages` _actionmontages)
  (set `self.WeaponAttackMontages` _attackmontages)
  (set `self.WeaponRollDodgeMontages` _rolldodgemontages)
  (set `self.WeaponStepDodgeMontages` _stepdodgemontages))