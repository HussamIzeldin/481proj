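; Character combat component that buffers combat input and tracks attack, dodge and punisher-mode state.
; Action, attack, quick-slot and held keys fire consume events immediately or wait while the buffer is open; closing can consume them and reset state through CharacterStateManagerComponent.
; It stores attack details in a reusable AttackInfo object, derives dodge direction from movement input, and loads optional abilities and dodge type from a data table.
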(event `self.ReceiveBeginPlay`
  (set `self.CombatStateManager` (`Actor.GetComponentByClass` (`self.GetOwner`) "/Game/Library/CombatSystem/Blueprints/Components/CharacterStateManagerComponent.CharacterStateManagerComponent_C"))
  (`|ExecutionSequence`
    (:`then_0`
      (bind _ascharacter (cast `Character` (`self.GetOwner`)))
      (set `self.GenericOwnerCharacter` _ascharacter))
    (:`then_1`
      (bind _asplayer_controller (cast `PlayerController` (`Pawn.GetController` (`self.GenericOwnerCharacter`))))
      (set `self.GenericPlayerController` _asplayer_controller))))

(fn `CalculateDirectionalDodge`
  (returns (Direction :type "/Game/Library/CombatSystem/Blueprints/Enums/E_DodgeDirection Enum"))
  (locals (DirectionalRollRotation :type "Float (double-precision)"))
  (set `local.DirectionalRollRotation` (.yaw (`KismetMathLibrary.NormalizedDeltaRotator` (`KismetMathLibrary.Conv_VectorToRotator` (`Pawn.GetLastMovementInputVector` (`self.GenericOwnerCharacter`))) (`Actor.K2_GetActorRotation` (`self.GetOwner`)))))
  (if (`KismetMathLibrary.InRange_FloatFloat` (`local.DirectionalRollRotation`) -30.0 30.0)
    ;[0 0.0625 1 0.5] Front
    (return "NewEnumerator0")
    (elif (`KismetMathLibrary.InRange_FloatFloat` (`local.DirectionalRollRotation`) 30.0 60.0)
      ;[1 0 0.4453 0.5] Front Right
      (return "NewEnumerator7")
      (elif (`KismetMathLibrary.InRange_FloatFloat` (`local.DirectionalRollRotation`) 60.0 120.0)
        ;[0.3359 1 0 0.5] Right
        (return "NewEnumerator1")
        (elif (`KismetMathLibrary.InRange_FloatFloat` (`local.DirectionalRollRotation`) 120.0 150.0)
          ;[0.3359 1 0 0.5] Back Right
          (return "NewEnumerator5")
          (elif (or (`KismetMathLibrary.InRange_FloatFloat` (`local.DirectionalRollRotation`) -180.0 -150.0) (`KismetMathLibrary.InRange_FloatFloat` (`local.DirectionalRollRotation`) 150.0 180.0))
            ;[1 0 0.4453 0.5] Back
            (return "NewEnumerator3")
            (elif (`KismetMathLibrary.InRange_FloatFloat` (`local.DirectionalRollRotation`) -60.0 -30.0)
              ;[1 0 0.9375 0.5] Front Left
              (return "NewEnumerator6")
              (elif (`KismetMathLibrary.InRange_FloatFloat` (`local.DirectionalRollRotation`) -120.0 -60.0)
                ;[1 0 0.9375 0.5] Left
                (return "NewEnumerator2")
                (elif (`KismetMathLibrary.InRange_FloatFloat` (`local.DirectionalRollRotation`) -150.0 -120.0)
                  ;[1 0 0.9375 0.5] Back left
                  (return "NewEnumerator4")
                  (else
                    (return "NewEnumerator0")))))))))))

(fn `CalculateFacingDirection`
  (returns (FacingDirection :type "/Game/Library/CombatSystem/Blueprints/Enums/E_GetupType Enum"))
  (if (>= (`KismetMathLibrary.Dot_VectorVector` (`KismetMathLibrary.GetRightVector` (`SceneComponent.GetSocketRotation` (`self.GetMesh`) "pelvis")) (0.0 0.0 1.0)) 0.0)
    (return "NewEnumerator1")
    (else
      (return "NewEnumerator2"))))

(fn `CanPerformOptionalAbility?`
  (params (OptionalAbility :type "/Game/Library/CombatSystem/Blueprints/Enums/E_OptionalCombatAbilities Enum" :default "NewEnumerator6"))
  (returns (Value :type Boolean))
  (return (`BlueprintMapLibrary.Map_Find` (`self.OptionalCombatAbilities`) OptionalAbility)))

(fn `ClearInputBuffer`
  (set `self.bIsBufferOpen` false)
  (set `self.CanConsumeInputBuffer?` false)
  (set `self.bSaveInput` false)
  (return))

(fn `ClearStoredBufferKeys`
  (set `self.StoredBufferKey` "NewEnumerator0")
  (set `self.AttackBufferKey` "NewEnumerator15")
  (set `self.QuickSlotBufferKey` "NewEnumerator0"))

(fn `CloseInputBuffer`
  ;[0 1 0.8828] If input saved is true, perform buffered action & close input buffer. If no input is saved close the input buffer
  (set `self.bIsBufferOpen` false)
  (set `self.bSaveInput` false)
  (if (`self.CanConsumeInputBuffer?`)
    (`self.ResetCombatState`)
    (`self.OnInputBufferConsumed` (`self.StoredBufferKey`))
    (`self.OnInputBufferClose`)
    (`self.ClearStoredBufferKeys`)
    (return)
    (else
      (`self.ClearStoredBufferKeys`)
      (return))))

(fn `GetAttackInfo`
  (returns (AttackInfo :type "/Game/Library/CombatSystem/Blueprints/Objects/AttackInfo Object Reference"))
  (return (`self.AttackInfo`)))

(fn `GetCurrentAttackType`
  (returns (CurrentAttackType :type "/Game/Library/CombatSystem/Blueprints/Enums/CombatEnums/E_AttackTypes Enum"))
  (return (`self.CurrentAttackType`)))

(fn `GetDodgeType`
  (returns (CurrentDodgeType :type "/Game/Library/CombatSystem/Blueprints/Enums/E_DodgeType Enum"))
  (return (`self.CurrentDodgeType`)))

(fn `GetHeldBufferKeys`
  (returns (HeldBufferKeys :type "Map of /Game/Library/CombatSystem/Blueprints/Enums/E_BufferKey Enum to Boolean"))
  (return (`self.HeldBufferKeys`)))

(fn `GetHeldBufferKeyValue`
  (params (Key :type "/Game/Library/CombatSystem/Blueprints/Enums/E_BufferKey Enum" :default "NewEnumerator0"))
  (returns (ReturnValue :type Boolean))
  (bind (_value _returnvalue) (`BlueprintMapLibrary.Map_Find` (`self.HeldBufferKeys`) Key))
  (return (and _value _returnvalue)))

(fn `GetInputHeldTime`
  (params (Key :type "Key Structure" :default "None"))
  (returns (ReturnValue :type "Float (double-precision)"))
  (bind _genericplayercontroller (`self.GenericPlayerController`)
    (:`then`
      (return (`PlayerController.GetInputKeyTimeDown` _genericplayercontroller Key)))
    (:`else`
      (return 0.0))))

(fn `GetLastStoredHeldBufferKey`
  (returns (BufferKey :type "/Game/Library/CombatSystem/Blueprints/Enums/E_BufferKey Enum"))
  (return (`self.LastStoredHeldBufferKey`)))

(fn `GetStoredAttackBufferKey`
  (returns (AttackBufferKey :type "/Game/Library/CombatSystem/Blueprints/Enums/CombatEnums/E_AttackTypes Enum"))
  (return (`self.AttackBufferKey`)))

(fn `GetStoredBufferKey`
  (returns (StoredBufferKey :type "/Game/Library/CombatSystem/Blueprints/Enums/E_BufferKey Enum"))
  (return (`self.StoredBufferKey`)))

(fn `GetStoredQuickSlotBufferKey`
  (returns (QuickSlotBufferKey :type "/Game/Library/InventoryandEquipment/Blueprints/Enums/Equipment/E_QuickSlots Enum"))
  (return (`self.QuickSlotBufferKey`)))

(fn `InputSaved?`
  (returns (Condition :type Boolean))
  (return (`self.bSaveInput`)))

(fn `IsBufferOpen?`
  (returns (Condition :type Boolean))
  (return (`self.bIsBufferOpen`)))

(fn `isPunisherMode?`
  (returns (PunisherMode :type Boolean))
  (return (`self.bPunisherMode`)))

(fn `OnlyBufferCertainKeys`
  (params (BufferKey :type "Map of /Game/Library/CombatSystem/Blueprints/Enums/E_BufferKey Enum to Boolean") (`ResetState?` :type Boolean))
  (bind (_value _returnvalue) (`BlueprintMapLibrary.Map_Find` BufferKey (`self.StoredBufferKey`)))
  ;[0 1 0.8828] If input saved is true, perform buffered action & close input buffer. If no input is saved close the input buffer
  (set `self.bIsBufferOpen` false)
  (set `self.bSaveInput` false)
  (if (and _value _returnvalue)
    (if (`self.CanConsumeInputBuffer?`)
      (if (`local.ResetState?`)
        (`/Game/Library/CombatSystem/Blueprints/Components/CharacterStateManagerComponent.SetState` (`self.CombatStateManager`) "NewEnumerator7"))
      (`self.OnInputBufferConsumed` (`self.StoredBufferKey`))
      (`self.OnInputBufferClose`)
      (set `self.bSaveInput` false)
      (`self.ClearStoredBufferKeys`)
      (return)
      (else
        _)))
  (`self.OnInputBufferClose`)
  (`self.ClearStoredBufferKeys`)
  (return))

(fn `OnMontagesUpdated`
  (params (DataTableInfo :type "DataTableRowHandle Structure"))
  (bind (_datatable _rowname) (break `DataTableRowHandle` DataTableInfo))
  (bind _returnvalue (`|GetDataTableRow` _datatable _rowname)
    (:`then`
      (bind ((`OptionalCombatAbilities_230_49BC65744A6334773340BD870579443A` _optionalcombatabilities) (`GeneralActions_226_B43AD8FF45DFB3DE3D2E089C6315F96B` _generalactions) (`Attacks_229_126AF23643ABF3DFC0810BBF1B6F1330` _attacks) (`CounterAttacks_238_D68C402249C31428BD863F9F2436DE40` _counterattacks) (`DodgeDirection_94_8C0E0D504C241CF92E0F1ABC6DBE41F7` _dodgedirection)) (break `/Game/Library/CombatSystem/Blueprints/Structs/CombatMontages_Struct` _returnvalue))
      (set `self.OptionalCombatAbilities` _optionalcombatabilities)
      (`self.SetDodgeType` (`.DodgeType_102_967D5DA240F1E12C505D57858736A3DE` (break `/Game/Library/CombatSystem/Blueprints/Structs/DodgeDirectionMap_Struct` _dodgedirection))))))

(fn `OpenInputBuffer`
  (set `self.CanConsumeInputBuffer?` true)
  (set `self.bIsBufferOpen` true)
  (`self.OnInputBufferOpen`))

(fn `ResetCombatState`
  (if (not (`/Game/Library/CombatSystem/Blueprints/Components/CharacterStateManagerComponent.isCombatDisabled?` (`self.CombatStateManager`)))
    (`/Game/Library/CombatSystem/Blueprints/Components/CharacterStateManagerComponent.SetState` (`self.CombatStateManager`) "NewEnumerator7")
    (return)
    (else
      (return))))

(fn `Set Character Attack Type`
  (params (AttackType :type "/Game/Library/CombatSystem/Blueprints/Enums/CombatEnums/E_AttackTypes Enum" :default "NewEnumerator0"))
  (locals (PrevAttackType :type "/Game/Library/CombatSystem/Blueprints/Enums/CombatEnums/E_AttackTypes Enum"))
  (set `local.PrevAttackType` (`self.CurrentAttackType`))
  (set `self.CurrentAttackType` AttackType)
  (return))

(fn `SetDodgeDirection`
  (params (OrientRotationToMovement :type Boolean))
  (returns (DodgeDirection :type "/Game/Library/CombatSystem/Blueprints/Enums/E_DodgeDirection Enum"))
  (if OrientRotationToMovement
    ;[0.6875 0 1] if orient rotation to movement is true set directional dodge with set actor rotation
    (return "NewEnumerator0")
    (else
      ;[1 0.04688 0] if orient rotation to movement is false calculate dodge direction for 8 way directional dodge animations
      (bind _direction (`self.CalculateDirectionalDodge`))
      (switch `/Game/Library/CombatSystem/Blueprints/Enums/E_DodgeDirection` _direction
        (:`NewEnumerator0`
          _)
        (:`NewEnumerator1`
          (return "NewEnumerator1"))
        (:`NewEnumerator2`
          (return "NewEnumerator2"))
        (:`NewEnumerator3`
          (return "NewEnumerator3"))
        (:`NewEnumerator4`
          _)
        (:`NewEnumerator5`
          _)
        (:`NewEnumerator6`
          _)
        (:`NewEnumerator7`
          _)
        (:`NewEnumerator9`
          (return "NewEnumerator9")))
      (return "NewEnumerator0"))))

(fn `SetDodgeType`
  (params (NewDodgeType :type "/Game/Library/CombatSystem/Blueprints/Enums/E_DodgeType Enum" :default "NewEnumerator0"))
  (if (`|EnumInequality` NewDodgeType (`self.CurrentDodgeType`))
    (set `self.CurrentDodgeType` (`local.NewDodgeType`))))

(fn `SetPunisherMode`
  (params (InPunisherMode :type Boolean))
  (if (!= InPunisherMode (`self.bPunisherMode`))
    (bind _output_get (set `self.bPunisherMode` (`local.InPunisherMode`)))
    (`self.OnPunisherModeChanged` _output_get)))

(fn `Store Attack Info`
  (params (MeleeSwingDirection :type "/Game/Library/CombatSystem/Blueprints/Enums/CombatEnums/E_MeleeSwingDirection Enum" :default "NewEnumerator21") (AttackPower :type "/Game/Library/CombatSystem/Blueprints/Enums/CombatEnums/E_AttackPower Enum" :default "NewEnumerator0") (CustomAttackType :type "/Game/Library/CombatSystem/Blueprints/Enums/CombatEnums/E_CustomAttackTypes Enum" :default "NewEnumerator0") (`CauseKnockback?` :type Boolean) (KnockbackTime :type "Float (double-precision)") (KnockbackSpeed :type "Float (double-precision)") (`IsUnblockableAttack?` :type Boolean) (AttackCategory :type "/Game/Library/CombatSystem/Blueprints/Enums/E_AttackCategory Enum" :default "NewEnumerator0") (CombatType :type "/Game/Library/CombatSystem/Blueprints/Enums/CombatEnums/E_CombatType Enum" :default "NewEnumerator16") (AttackIndex :type Integer))
  (bind _attackinfo (`self.AttackInfo`))
  (`/Engine/EditorBlueprintResources/StandardMacros.IsValid` _attackinfo
    (:`Is Valid`
      (`/Game/Library/CombatSystem/Blueprints/Objects/AttackInfo.StoreAttackInfo` _attackinfo MeleeSwingDirection AttackPower CustomAttackType `CauseKnockback?` KnockbackTime KnockbackSpeed `IsUnblockableAttack?` AttackCategory CombatType AttackIndex))
    (:`Is Not Valid`
      (bind _returnvalue (`|GenericCreateObject` "/Game/Library/CombatSystem/Blueprints/Objects/AttackInfo.AttackInfo_C" (`self.GetOwner`) MeleeSwingDirection AttackPower CustomAttackType `CauseKnockback?` KnockbackTime KnockbackSpeed `IsUnblockableAttack?` AttackCategory CombatType AttackIndex))
      (set `self.AttackInfo` _returnvalue))))

(fn `Store Basic Attack Info`
  (params (AttackCategory :type "/Game/Library/CombatSystem/Blueprints/Enums/CombatEnums/E_GeneralCombatType Enum" :default "NewEnumerator16") (CombatType :type "/Game/Library/CombatSystem/Blueprints/Enums/CombatEnums/E_CombatType Enum" :default "NewEnumerator16") (AttackIndex :type Integer))
  (bind _returnvalue (select `/Game/Library/CombatSystem/Blueprints/Enums/CombatEnums/E_GeneralCombatType` AttackCategory :`NewEnumerator16` "NewEnumerator0" :`NewEnumerator8` "NewEnumerator0" :`NewEnumerator11` "NewEnumerator1" :`NewEnumerator3` "NewEnumerator2" :!type "/Game/Library/CombatSystem/Blueprints/Enums/E_AttackCategory Enum"))
  (bind _attackinfo (`self.AttackInfo`))
  (`/Engine/EditorBlueprintResources/StandardMacros.IsValid` _attackinfo
    (:`Is Valid`
      (`/Game/Library/CombatSystem/Blueprints/Objects/AttackInfo.StoreAttackInfo` _attackinfo "NewEnumerator19" "NewEnumerator1" "NewEnumerator0" false 0.0 0.0 false _returnvalue CombatType AttackIndex))
    (:`Is Not Valid`
      (bind _returnvalue_2 (`|GenericCreateObject` "/Game/Library/CombatSystem/Blueprints/Objects/AttackInfo.AttackInfo_C" (`self.GetOwner`) "NewEnumerator19" "NewEnumerator1" "NewEnumerator0" false 0.0 0.0 false _returnvalue CombatType AttackIndex))
      (set `self.AttackInfo` _returnvalue_2))))

(fn `StoreAttackBufferKey`
  (params (AttackBufferKey :type "/Game/Library/CombatSystem/Blueprints/Enums/CombatEnums/E_AttackTypes Enum" :default "NewEnumerator15"))
  ;[0 1 0.3672] Update stored buffer key (key needs to be updated for every buffered action)
  (set `self.AttackBufferKey` AttackBufferKey)
  (bind _output_get (set `self.StoredBufferKey` "NewEnumerator2"))
  ;[0.1719 0 1] If input buffer is open, save the input. If it is not open perform the action
  (if (`self.bIsBufferOpen`)
    (set `self.bSaveInput` true)
    (else
      (`self.OnInputBufferConsumed` _output_get)
      (`self.ClearStoredBufferKeys`))))

(fn `StoreBufferKey`
  (params (StoredBufferKey :type "/Game/Library/CombatSystem/Blueprints/Enums/E_BufferKey Enum" :default "NewEnumerator0"))
  ;[0 1 0.3672] Update stored buffer key (key needs to be updated for every buffered action)
  (bind _output_get (set `self.StoredBufferKey` StoredBufferKey))
  ;[0.1719 0 1] If input buffer is open, save the input. If it is not open perform the action
  (if (`self.bIsBufferOpen`)
    (set `self.bSaveInput` true)
    (else
      (`self.OnInputBufferConsumed` _output_get)
      (`self.ClearStoredBufferKeys`))))

(fn `StoreHeldBufferKey`
  (params (HeldBufferKey :type "/Game/Library/CombatSystem/Blueprints/Enums/E_BufferKey Enum" :default "NewEnumerator0") (Value :type Boolean) (`Consume?` :type Boolean :default true))
  (if (!= (`self.GetHeldBufferKeyValue` (`local.HeldBufferKey`)) (`local.Value`))
    (if (`local.Value`)
      (`BlueprintMapLibrary.Map_Add` (`self.HeldBufferKeys`) (`local.HeldBufferKey`) (`local.Value`))
      (set `self.LastStoredHeldBufferKey` (`local.HeldBufferKey`))
      (if (and (not (`self.bIsBufferOpen`)) (`local.Consume?`))
        (`self.OnInputBufferConsumed` (`local.HeldBufferKey`))
        (`self.ClearStoredBufferKeys`))
      (else
        (`BlueprintMapLibrary.Map_Remove` (`self.HeldBufferKeys`) (`local.HeldBufferKey`))))))

(fn `StoreQuickSlotBufferKey`
  (params (QuickSlotBufferKey :type "/Game/Library/InventoryandEquipment/Blueprints/Enums/Equipment/E_QuickSlots Enum" :default "NewEnumerator0"))
  ;[0 1 0.3672] Update stored buffer key (key needs to be updated for every buffered action)
  (set `self.QuickSlotBufferKey` QuickSlotBufferKey)
  (bind _output_get (set `self.StoredBufferKey` "NewEnumerator62"))
  ;[0.1719 0 1] If input buffer is open, save the input. If it is not open perform the action
  (if (`self.bIsBufferOpen`)
    (set `self.bSaveInput` true)
    (else
      (`self.OnInputBufferConsumed` _output_get)
      (`self.ClearStoredBufferKeys`))))