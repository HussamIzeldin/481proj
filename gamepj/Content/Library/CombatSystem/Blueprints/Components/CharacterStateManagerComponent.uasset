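; Character component in the combat system that holds the owner's current and previous state, current action, and combat flags like dead, invulnerable, blocking and aiming.
; State, action, blocking, aiming and movement-cancel setters fire events, while queries test the state against fixed sets.
; Movement is disabled by zeroing MaxAcceleration and restored from the value cached at BeginPlay.
; Owner reset fires immediately or on a timer, which SetState attempts to clear.
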(event `self.ReceiveBeginPlay`
  (bind _ascharacter (cast `Character` (`self.GetOwner`)))
  (set `self.GenericOwnerCharacter` _ascharacter)
  (set `self.DefaultMaxAcceleration` (`CharacterMovementComponent.MaxAcceleration` (`self.GetCharacterMovement`))))

(fn `CanMovementCancel?`
  (returns (`bCanMovementCancel?` :type Boolean))
  (return (`self.bCanMovementCancel?`)))

(fn `DisableMovement`
  (params (DisableMovement :type Boolean))
  (bind _output_get (set `self.bMovementDisabled?` DisableMovement))
  (if _output_get
    (set `CharacterMovementComponent.MaxAcceleration` 0.0 (`self.GetCharacterMovement`))
    (else
      (set `CharacterMovementComponent.MaxAcceleration` (`self.DefaultMaxAcceleration`) (`self.GetCharacterMovement`)))))

(fn `Get Current Action`
  (returns (Action :type "/Game/Library/CombatSystem/Blueprints/Enums/CombatEnums/E_CharacterAction Enum"))
  (return (`self.CharacterAction`)))

(fn `Get Current State`
  (returns (State :type "/Game/Library/CombatSystem/Blueprints/Enums/CombatEnums/E_CharacterState Enum"))
  (return (`self.CharacterState`)))

(fn `GetCancelFrames`
  (returns (`CancelFrames?` :type Boolean))
  (return (`self.bCancelFrames?`)))

(fn `GetPrevState`
  (returns (ReturnValue :type "/Game/Library/CombatSystem/Blueprints/Enums/CombatEnums/E_CharacterState Enum"))
  (return (`self.PrevCharacterState`)))

(fn `IsAiming?`
  (returns (Condition :type Boolean))
  (return (`self.bIsAiming?`)))

(fn `IsBlocking?`
  (returns (`bIsBlocking?` :type Boolean))
  (return (`self.bIsBlocking?`)))

(fn `isCombatDisabled?`
  (returns (`Disabled?` :type Boolean))
  (return (`KismetArrayLibrary.Array_Contains` (`|MakeArray` "NewEnumerator24" "NewEnumerator28" "NewEnumerator39" "NewEnumerator42" :!type "/Game/Library/CombatSystem/Blueprints/Enums/CombatEnums/E_CharacterState Enum") (`self.CharacterState`))))

(fn `isDead?`
  (returns (Condition :type Boolean))
  (return (`self.bDead?`)))

(fn `isInvulnerable?`
  (returns (Condition :type Boolean))
  (return (`self.bIsInvulnerable?`)))

(fn `isMovementDisabled?`
  (returns (`MovementDisabled?` :type Boolean))
  (return (`self.bMovementDisabled?`)))

(fn `isReactingToHits?`
  (returns (ReturnValue :type Boolean))
  (return (`KismetArrayLibrary.Array_Contains` (`|MakeArray` "NewEnumerator21" "NewEnumerator30" :!type "/Game/Library/CombatSystem/Blueprints/Enums/CombatEnums/E_CharacterState Enum") (`self.Get Current State`))))

(fn `isStateEqual?`
  (params (StateToCompare :type "/Game/Library/CombatSystem/Blueprints/Enums/CombatEnums/E_CharacterState Enum" :default "NewEnumerator7"))
  (returns (ReturnValue :type Boolean))
  (return (`|EnumEquality` StateToCompare (`self.CharacterState`))))

(fn `isStateNotEqual?`
  (params (StateToCompare :type "/Game/Library/CombatSystem/Blueprints/Enums/CombatEnums/E_CharacterState Enum" :default "NewEnumerator7"))
  (returns (ReturnValue :type Boolean))
  (return (`|EnumInequality` StateToCompare (`self.CharacterState`))))

(fn `OwnerReset(Private)`
  (`self.OnOwnerReset`))

(fn `ResetOwner`
  (params (ResetTime :type "Float (double-precision)"))
  (if (<= ResetTime 0.0)
    (`self.OwnerReset(Private)`)
    (else
      (`KismetSystemLibrary.K2_SetTimerDelegate` (`|CreateDelegate` :!event `OwnerReset(Private)`) ResetTime))))

(fn `ResetState`
  (`self.SetState` "NewEnumerator7")
  (set `self.PrevCharacterState` "NewEnumerator7"))

(fn `Set Invulnerable`
  (params (`Invulnerable?` :type Boolean))
  (set `self.bIsInvulnerable?` `Invulnerable?`))

(fn `SetAction`
  (params (NewAction :type "/Game/Library/CombatSystem/Blueprints/Enums/CombatEnums/E_CharacterAction Enum" :default "NewEnumerator0"))
  (if (`|EnumInequality` NewAction (`self.CharacterAction`))
    (`self.OnActionEnd` (`self.CharacterAction`))
    (bind _output_get (set `self.CharacterAction` (`local.NewAction`)))
    (`self.OnActionBegin` _output_get)))

(fn `SetAimingState`
  (params (NewAimingState :type Boolean))
  (if (!= NewAimingState (`self.IsAiming?`))
    (bind _output_get (set `self.bIsAiming?` (`local.NewAimingState`)))
    (`self.OnAimingStateSet` _output_get)))

(fn `SetBlockingState`
  (params (NewBlockingState :type Boolean))
  (if (!= NewBlockingState (`self.IsBlocking?`))
    (bind _output_get (set `self.bIsBlocking?` (`local.NewBlockingState`)))
    (`self.OnBlockStateSet` _output_get)))

(fn `SetCancelFrames`
  (params (`CancelFrames?` :type Boolean))
  (set `self.bCancelFrames?` `CancelFrames?`))

(fn `SetCanMovementCancel`
  (params (`bCanMovementCancel?` :type Boolean))
  (bind _output_get (set `self.bCanMovementCancel?` `bCanMovementCancel?`))
  (`self.OnMovementCancelSet` _output_get))

(fn `SetDead`
  (params (`Dead?` :type Boolean))
  (set `self.bDead?` `Dead?`))

(fn `SetState`
  (params (NewState :type "/Game/Library/CombatSystem/Blueprints/Enums/CombatEnums/E_CharacterState Enum" :default "NewEnumerator7"))
  (`KismetSystemLibrary.K2_ClearTimer` null "OwnerReset(Private)")
  (if (`|EnumInequality` NewState (`self.CharacterState`))
    (bind _output_get (set `self.PrevCharacterState` (`self.CharacterState`)))
    (`self.OnStateEnd` _output_get)
    (bind _output_get_2 (set `self.CharacterState` (`local.NewState`)))
    (`self.OnStateBegin` _output_get_2)))