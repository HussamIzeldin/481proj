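; Combat stats function library that computes regular and poise damage from base damage, attack type and Punisher Mode.
; Both damage functions apply a Punisher Mode boost and per-type multiplier tables, which differ only for Riposte.
; Regular damage clamps the type multiplier to a minimum of one, while poise damage clamps the final product.
; A separate function scales poise damage by attack power tier, with VeryHeavy yielding zero.
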(fn `AttackPowerMultiplier`
  (params (InPoiseDamage :type "Float (double-precision)") (AttackPower :type "/Game/Library/CombatSystem/Blueprints/Enums/CombatEnums/E_AttackPower Enum" :default "NewEnumerator0"))
  (returns (ReturnValue :type "Float (double-precision)"))
  (return (* InPoiseDamage (select `/Game/Library/CombatSystem/Blueprints/Enums/CombatEnums/E_AttackPower` AttackPower :`NewEnumerator0` 1.0 :`NewEnumerator1` 1.25 :`NewEnumerator2` 1.5 :`NewEnumerator3` 1.75 :!type "Float (single-precision)"))))

(fn `PoiseDamageByAttackType`
  (params (BaseDamage :type "Float (double-precision)") (InAttackType :type "/Game/Library/CombatSystem/Blueprints/Enums/CombatEnums/E_AttackTypes Enum" :default "NewEnumerator15") (`PunisherMode?` :type Boolean))
  (returns (Damage :type "Float (double-precision)"))
  (bind _returnvalue (* (* (`local.BaseDamage`) (select `bool` `PunisherMode?` :`false` 1.0 :`true` 1.8 :!type "Float (single-precision)")) (select `/Game/Library/CombatSystem/Blueprints/Enums/CombatEnums/E_AttackTypes` InAttackType :`NewEnumerator15` 1.0 :`NewEnumerator0` 1.0 :`NewEnumerator1` 1.5 :`NewEnumerator2` 1.7 :`NewEnumerator3` 1.6 :`NewEnumerator4` 1.0 :`NewEnumerator5` 1.7 :`NewEnumerator10` 1.5 :`NewEnumerator11` 1.5 :`NewEnumerator12` 4.0 :`NewEnumerator13` 4.0 :`NewEnumerator14` 1.5 :`NewEnumerator17` 1.2 :`NewEnumerator18` 1.3 :`NewEnumerator19` 1.4 :`NewEnumerator20` 1.0 :`NewEnumerator21` 1.5 :!type "Float (single-precision)")))
  (return (`KismetMathLibrary.FClamp` _returnvalue 1.0 _returnvalue)))

(fn `RegularDamageByAttackType`
  (params (BaseDamage :type "Float (double-precision)") (InAttackType :type "/Game/Library/CombatSystem/Blueprints/Enums/CombatEnums/E_AttackTypes Enum" :default "NewEnumerator15") (`PunisherMode?` :type Boolean))
  (returns (Damage :type "Float (double-precision)"))
  (bind _returnvalue (select `/Game/Library/CombatSystem/Blueprints/Enums/CombatEnums/E_AttackTypes` InAttackType :`NewEnumerator15` 1.0 :`NewEnumerator0` 1.0 :`NewEnumerator1` 1.5 :`NewEnumerator2` 1.7 :`NewEnumerator3` 1.6 :`NewEnumerator4` 1.0 :`NewEnumerator5` 1.7 :`NewEnumerator10` 1.5 :`NewEnumerator11` 1.5 :`NewEnumerator12` 4.0 :`NewEnumerator13` 4.0 :`NewEnumerator14` 1.5 :`NewEnumerator17` 1.2 :`NewEnumerator18` 1.3 :`NewEnumerator19` 1.4 :`NewEnumerator20` 1.0 :`NewEnumerator21` 1.5 :`NewEnumerator22` 2.0 :!type "Float (single-precision)"))
  (return (* (* (`local.BaseDamage`) (select `bool` `PunisherMode?` :`false` 1.0 :`true` 1.8 :!type "Float (single-precision)")) (`KismetMathLibrary.FClamp` _returnvalue 1.0 _returnvalue))))