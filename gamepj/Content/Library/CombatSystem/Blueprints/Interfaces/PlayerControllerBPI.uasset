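; Blueprint interface for the player controller in the CombatSystem library, declaring its UI and menu functions without implementations.
; It covers tracking the open and previous UI and toggling pause, bonfire, controls, inventory and equipment screens, plus message display.
; It also exposes the main HUD, vendor and sell widgets, character name and class, and gamepad input state, so callers avoid casting to a concrete controller.
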(fn `DisableBonfire`)

(fn `DisablePauseMenu`)

(fn `GetCharacterClassType`
  (returns (Class :type Text))
  (return ""))

(fn `GetCharacterName`
  (returns (Name :type Text))
  (return ""))

(fn `GetCurrentVendorInteractionWidget`
  (returns (Widget :type "Widget Object Reference"))
  (return null))

(fn `GetMainHUD`
  (returns (MainHUD :type "UserWidget Object Reference"))
  (return null))

(fn `GetPauseMenuWidget`
  (returns (Menu :type "UserWidget Object Reference"))
  (return null))

(fn `GetPlayerSellWidget`
  (returns (SellWidget :type "Widget Object Reference"))
  (return null))

(fn `GetPrevUserInterface`
  (returns (PrevUserInterface :type "/Game/Library/UI/MainMenu/Blueprints/Enums/E_UserInterface Enum"))
  (return "NewEnumerator0"))

(fn `GetUserInterfaceOpen`
  (returns (OpenedUserInterface :type "/Game/Library/UI/MainMenu/Blueprints/Enums/E_UserInterface Enum"))
  (return "NewEnumerator0"))

(fn `isUsingGamepad?`
  (returns (`UsingGamepad?` :type Boolean))
  (return false))

(fn `OpenControlsMenu`)

(fn `OpenMessageWidget`
  (params (Message :type Text) (`UseOverlay?` :type Boolean)))

(fn `PressedMenuButton`)

(fn `SetUserInterfaceOpen`
  (params (OpenedUserInterface :type "/Game/Library/UI/MainMenu/Blueprints/Enums/E_UserInterface Enum" :default "NewEnumerator0")))

(fn `ToggleBonfireMenu`)

(fn `TogglePauseMenu`
  (params (`Enable?` :type Boolean :default false)))

(fn `TogglePlayerEquipment`
  (params (`Enable?` :type Boolean)))

(fn `TogglePlayerInventory`
  (params (`Enable?` :type Boolean)))

(fn `TogglePlayerSellWidget`
  (params (`Visible?` :type Boolean)))

(fn `ToggleUserInterface`
  (params (UserInterface :type "/Game/Library/UI/MainMenu/Blueprints/Enums/E_UserInterface Enum" :default "NewEnumerator0")))

(fn `UpdateCurrentVendorInteractionWidget`
  (params (Widget :type "Widget Object Reference")))

(fn `UpdateInputMethod`
  (params (`UsingGamepad?` :type Boolean)))