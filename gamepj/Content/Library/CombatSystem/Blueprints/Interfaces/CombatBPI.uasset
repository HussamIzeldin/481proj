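; CombatBPI is a Blueprint Interface that declares the combat system's shared messages between characters, AI and other combat objects.
; It covers executions, countering, attack info, blocking, strong charge attacks, archery, stealth checks, impact effects and input buffering.
; It also declares hooks for boss room music, Punisher mode, and passing AI details for death and respawn.
; Functions are signatures only, with default returns, leaving behavior to implementers.
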(fn `AI Details`
  (params (`AI Type` :type "/Game/Library/CombatSystem/AI/BP/StructuresAndEnums/E_AI_Type Enum" :default "NewEnumerator0") (Location :type "Vector Structure") (Rotation :type "Rotator Structure") (`Patrol Points` :type "Array of Actor Object Reference") (`Combat Type` :type "/Game/Library/CombatSystem/Blueprints/Enums/CombatEnums/E_CombatType Enum" :default "NewEnumerator16") (`AI Class` :type "Character Class Reference")))

(fn `ApplyCriticalDamage`
  (params (CriticalDamageMultiplier :type "Float (double-precision)" :default 1.0)))

(fn `BeginStrongChargeAttack`
  (params (ChargeAnimPlayRate :type "Float (double-precision)" :default 0.2)))

(fn `Boss Room Music End`)

(fn `Boss Room Music Initialization`)

(fn `BufferInput`
  (params (BufferKey :type "/Game/Library/CombatSystem/Blueprints/Enums/E_BufferKey Enum" :default "NewEnumerator0")))

(fn `Camera Aim Rotation`
  (params (`Compared To ` :type "Actor Object Reference"))
  (returns (`Rotation To Actor` :type "Rotator Structure"))
  (return))

(fn `CanDrawString`
  (returns (Condition :type Boolean))
  (return false))

(fn `CheckStealth`
  (params (`Checking With` :type "Actor Object Reference"))
  (returns (`Can Stealth` :type Boolean))
  (return false))

(fn `CombatEnabled?`
  (returns (CombatMode :type Boolean))
  (return false))

(fn `Dead AI Details`
  (params (`AI Type` :type "/Game/Library/CombatSystem/AI/BP/StructuresAndEnums/E_AI_Type Enum" :default "NewEnumerator0") (Location :type "Vector Structure") (Rotation :type "Rotator Structure") (`Patrol Points` :type "Array of Actor Object Reference"))
  (return))

(fn `EndStrongChargeAttack`)

(fn `EnterPunisherMode`)

(fn `ExitPunisherMode`)

(fn `Get Executed Actor`
  (returns (`Executed Actor` :type "Actor Object Reference"))
  (return null))

(fn `Get Mesh Tranform`
  (returns (`Mesh Tranform` :type "Transform Structure"))
  (return))

(fn `GetArrowMesh`
  (returns (Mesh :type "StaticMesh Object Reference"))
  (return null))

(fn `GetBowStringSocketName`
  (returns (Name :type Name))
  (return "None"))

(fn `GetCharacterState`
  (returns (CombatState :type "/Game/Library/CombatSystem/Blueprints/Enums/CombatEnums/E_CharacterState Enum"))
  (return "NewEnumerator7"))

(fn `GetCombatDataTable`
  (returns (DataTable :type "DataTable Object Reference"))
  (return null))

(fn `GetGeneralCombatType`
  (returns (`General Combat Type` :type "/Game/Library/CombatSystem/Blueprints/Enums/CombatEnums/E_GeneralCombatType Enum"))
  (return "NewEnumerator16"))

(fn `GetStrongChargeAmount`
  (returns (StrongChargeAmount :type "Float (double-precision)"))
  (return 0.0))

(fn `Getup(Knockeddown)`)

(fn `PerfectBlockSuccessful?`
  (returns (`PerfectBlock?` :type Boolean))
  (return false))

(fn `PlayImpactEffect`
  (params (ImpactEffect :type "/Game/Library/CombatSystem/Blueprints/ImpactEffects/ImpactEffect_Base Class Reference") (ImpactPoint :type "Vector Structure") (SurfaceType :type "EPhysicalSurface Enum" :default "SurfaceType_Default") (`UseScreenShake?` :type Boolean :default false)))

(fn `ReleaseArcheryProjectile`
  (params (SwingDirection :type "/Game/Library/CombatSystem/Blueprints/Enums/CombatEnums/E_MeleeSwingDirection Enum" :default "NewEnumerator19") (AttackPower :type "/Game/Library/CombatSystem/Blueprints/Enums/CombatEnums/E_AttackPower Enum" :default "NewEnumerator0") (CustomAttackType :type "/Game/Library/CombatSystem/Blueprints/Enums/CombatEnums/E_CustomAttackTypes Enum" :default "NewEnumerator0") (`CauseKnockback?` :type Boolean) (KnockbackTime :type "Float (double-precision)") (KnockbackSpeed :type "Float (double-precision)") (`IsUnblockableAttack?` :type Boolean) (RegularDamageMultiplier :type "Float (double-precision)" :default 1.0) (PoiseDamageMultiplier :type "Float (double-precision)" :default 1.0)))

(fn `Respawn All AIs On The Map`)

(fn `SetExecutionDistance`
  (params (ExecutionDistance :type "Float (double-precision)") (AttackerRotationOffset :type "Float (double-precision)") (TransitionSpeedMultiplier :type "Float (double-precision)" :default 1.0)))

(fn `SetExecutionDistance(Forced)`
  (params (ExecutionDistance :type "Float (double-precision)") (AttackerRotationOffset :type "Float (double-precision)") (TransitionSpeedMultiplier :type "Float (double-precision)") (`Face Actor` :type Boolean)))

(fn `Start Countering TL`
  (params (`Play Rate` :type "Float (double-precision)" :default 1.0) (Direction :type "Map of /Game/Library/CombatSystem/Blueprints/Enums/CombatEnums/E_HitFacingDirection Enum to Float (double-precision)")))

(fn `Start Execution TL`
  (params (ExecutedActor :type "Actor Object Reference") (FacingActor :type Boolean)))

(fn `UpdateAttackInfo`
  (params (SwingDirection :type "/Game/Library/CombatSystem/Blueprints/Enums/CombatEnums/E_MeleeSwingDirection Enum" :default "NewEnumerator21") (AttackPower :type "/Game/Library/CombatSystem/Blueprints/Enums/CombatEnums/E_AttackPower Enum" :default "NewEnumerator0") (CustomAttackType :type "/Game/Library/CombatSystem/Blueprints/Enums/CombatEnums/E_CustomAttackTypes Enum" :default "NewEnumerator0") (`CauseKnockback?` :type Boolean) (KnockbackTime :type "Float (double-precision)") (KnockbackSpeed :type "Float (double-precision)") (`IsUnblockableAttack?` :type Boolean) (AttackCategory :type "/Game/Library/CombatSystem/Blueprints/Enums/E_AttackCategory Enum" :default "NewEnumerator0") (RegularDamageMultiplier :type "Float (double-precision)" :default 1.0) (PoiseDamageMultiplier :type "Float (double-precision)" :default 1.0)))