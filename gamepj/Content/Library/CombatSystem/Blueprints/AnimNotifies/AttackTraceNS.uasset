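; Anim notify state that opens a melee attack trace window during an attack animation.
; On begin, it sends swing, power, knockback, unblockable and damage multiplier data to the owner, then enables collision tracing on the selected target.
; Weapon, off-hand and shield traces use the equipped actor's collision component with radius and trace count modifiers; hands and feet use the owner's CollisionComponent.
; On end, it disables that collision.
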(fn `Received_NotifyBegin`
  (params (MeshComp :type "SkeletalMeshComponent Object Reference") (Animation :type "AnimSequenceBase Object Reference") (TotalDuration :type "Float (double-precision)"))
  (returns (ReturnValue :type Boolean))
  (bind _returnvalue (`ActorComponent.GetOwner` MeshComp))
  (bind _returnvalue_2 (`Actor.GetComponentByClass` _returnvalue "/Game/Library/InventoryandEquipment/Blueprints/Components/EquipmentComponent.EquipmentComponent_C"))
  (bind _returnvalue_3 (`Actor.GetComponentByClass` _returnvalue "/Game/Library/CombatSystem/Blueprints/Components/CollisionComponent.CollisionComponent_C"))
  (bind _shieldweapon (`/Game/Library/InventoryandEquipment/Blueprints/Components/EquipmentComponent.Get Equipped Shield Actor` (`Actor.GetComponentByClass` _returnvalue "/Game/Library/InventoryandEquipment/Blueprints/Components/EquipmentComponent.EquipmentComponent_C")))
  (bind _returnvalue_4 (`/Game/Library/InventoryandEquipment/Blueprints/Components/EquipmentComponent.Get Equipped Off-hand Weapon Actor` _returnvalue_2))
  (bind _returnvalue_5 (`/Game/Library/InventoryandEquipment/Blueprints/Components/EquipmentComponent.Get Equipped Weapon Actor` _returnvalue_2))
  (bind _weaponcollisioncomponent (`/Game/Library/InventoryandEquipment/Blueprints/Actors/WeaponParent_BP.WeaponCollisionComponent` _shieldweapon))
  (bind _secondweaponcollisioncomponent (`/Game/Library/InventoryandEquipment/Blueprints/Actors/WeaponParent_BP.SecondWeaponCollisionComponent` _returnvalue_4))
  (bind _weaponcollisioncomponent_2 (`/Game/Library/InventoryandEquipment/Blueprints/Actors/WeaponParent_BP.WeaponCollisionComponent` _returnvalue_5))
  (message `/Game/Library/CombatSystem/Blueprints/Interfaces/CombatBPI.UpdateAttackInfo` _returnvalue (`self.SwingDirection`) (`self.AttackPower`) (`self.CustomAttackType`) (`self.CauseKnockback?`) (`self.KnockbackTime`) (`self.KnockbackSpeed`) (`self.IsUnblockableAttack?`) (`self.AttackCategory`) (`self.RegularDamageMultiplier`) (`self.PoiseDamageMultiplier`))
  (switch `/Game/Library/CombatSystem/Blueprints/Enums/CombatEnums/E_CollisionTraceTarget` (`self.AttackTraceTarget`)
    (:`NewEnumerator2`
      ;[1 0 0.04857] Melee Weapon Attack Trace
      (`/Engine/EditorBlueprintResources/StandardMacros.IsValid` _returnvalue_2
        (:`Is Valid`
          (`/Engine/EditorBlueprintResources/StandardMacros.IsValid` _returnvalue_5
            (:`Is Valid`
              (set `/Game/Library/CombatSystem/Blueprints/Components/CollisionComponent.TraceRadiusModifier` (`self.TraceRadiusModifier`) _weaponcollisioncomponent_2)
              (set `/Game/Library/CombatSystem/Blueprints/Components/CollisionComponent.MaxTracesModifier` (`self.MaxTracesModifier`) _weaponcollisioncomponent_2)
              (`/Game/Library/CombatSystem/Blueprints/Components/CollisionComponent.EnableCollision` _weaponcollisioncomponent_2 "NewEnumerator2")
              (return true))))))
    (:`NewEnumerator1`
      (`/Engine/EditorBlueprintResources/StandardMacros.IsValid` _returnvalue_2
        (:`Is Valid`
          (`/Engine/EditorBlueprintResources/StandardMacros.IsValid` _returnvalue_4
            (:`Is Valid`
              (set `/Game/Library/CombatSystem/Blueprints/Components/CollisionComponent.TraceRadiusModifier` (`self.TraceRadiusModifier`) _secondweaponcollisioncomponent)
              (set `/Game/Library/CombatSystem/Blueprints/Components/CollisionComponent.MaxTracesModifier` (`self.MaxTracesModifier`) _secondweaponcollisioncomponent)
              (`/Game/Library/CombatSystem/Blueprints/Components/CollisionComponent.EnableCollision` _secondweaponcollisioncomponent "NewEnumerator1")
              (return true))))))
    (:`NewEnumerator10`
      ;[1 0 0.05719] Enable Shield Attack Trace
      (`/Engine/EditorBlueprintResources/StandardMacros.IsValid` _shieldweapon
        (:`Is Valid`
          (set `/Game/Library/CombatSystem/Blueprints/Components/CollisionComponent.TraceRadiusModifier` (`self.TraceRadiusModifier`) _weaponcollisioncomponent)
          (set `/Game/Library/CombatSystem/Blueprints/Components/CollisionComponent.MaxTracesModifier` (`self.MaxTracesModifier`) _weaponcollisioncomponent)
          (`/Game/Library/CombatSystem/Blueprints/Components/CollisionComponent.EnableCollision` _weaponcollisioncomponent "NewEnumerator10")
          (return true))))
    (:`NewEnumerator3`
      _)
    (:`NewEnumerator4`
      _)
    (:`NewEnumerator5`
      _)
    (:`NewEnumerator6`
      _))
  ;[1 0 0.05719] Enable Unarmed Attack Trace
  (`/Engine/EditorBlueprintResources/StandardMacros.IsValid` _returnvalue_3
    (:`Is Valid`
      (`/Game/Library/CombatSystem/Blueprints/Components/CollisionComponent.EnableCollision` _returnvalue_3 (`self.AttackTraceTarget`))
      (return true))))

(fn `Received_NotifyEnd`
  (params (MeshComp :type "SkeletalMeshComponent Object Reference") (Animation :type "AnimSequenceBase Object Reference"))
  (returns (ReturnValue :type Boolean))
  (bind _returnvalue (`ActorComponent.GetOwner` MeshComp))
  (bind _returnvalue_2 (`Actor.GetComponentByClass` _returnvalue "/Game/Library/InventoryandEquipment/Blueprints/Components/EquipmentComponent.EquipmentComponent_C"))
  (bind _returnvalue_3 (`Actor.GetComponentByClass` _returnvalue "/Game/Library/CombatSystem/Blueprints/Components/CollisionComponent.CollisionComponent_C"))
  (bind _shieldweapon (`/Game/Library/InventoryandEquipment/Blueprints/Components/EquipmentComponent.Get Equipped Shield Actor` (`Actor.GetComponentByClass` _returnvalue "/Game/Library/InventoryandEquipment/Blueprints/Components/EquipmentComponent.EquipmentComponent_C")))
  (bind _returnvalue_4 (`/Game/Library/InventoryandEquipment/Blueprints/Components/EquipmentComponent.Get Equipped Off-hand Weapon Actor` _returnvalue_2))
  (bind _returnvalue_5 (`/Game/Library/InventoryandEquipment/Blueprints/Components/EquipmentComponent.Get Equipped Weapon Actor` _returnvalue_2))
  (switch `/Game/Library/CombatSystem/Blueprints/Enums/CombatEnums/E_CollisionTraceTarget` (`self.AttackTraceTarget`)
    (:`NewEnumerator2`
      ;[1 0 0.04857] Disable Melee Weapon Attack Trace
      (`/Engine/EditorBlueprintResources/StandardMacros.IsValid` _returnvalue_2
        (:`Is Valid`
          (`/Engine/EditorBlueprintResources/StandardMacros.IsValid` _returnvalue_5
            (:`Is Valid`
              (`/Game/Library/CombatSystem/Blueprints/Components/CollisionComponent.DisableCollision` (`/Game/Library/InventoryandEquipment/Blueprints/Actors/WeaponParent_BP.WeaponCollisionComponent` _returnvalue_5))
              (return true))
            (:`Is Not Valid`
              _)))
        (:`Is Not Valid`
          _))
      (return false))
    (:`NewEnumerator1`
      (`/Engine/EditorBlueprintResources/StandardMacros.IsValid` _returnvalue_2
        (:`Is Valid`
          (`/Engine/EditorBlueprintResources/StandardMacros.IsValid` _returnvalue_4
            (:`Is Valid`
              (`/Game/Library/CombatSystem/Blueprints/Components/CollisionComponent.DisableCollision` (`/Game/Library/InventoryandEquipment/Blueprints/Actors/WeaponParent_BP.SecondWeaponCollisionComponent` _returnvalue_4))
              (return true))))
        (:`Is Not Valid`
          (return false))))
    (:`NewEnumerator10`
      ;[1 0 0.05719] Disable Shield Attack Trace
      (`/Engine/EditorBlueprintResources/StandardMacros.IsValid` _shieldweapon
        (:`Is Valid`
          (`/Game/Library/CombatSystem/Blueprints/Components/CollisionComponent.DisableCollision` (`/Game/Library/InventoryandEquipment/Blueprints/Actors/WeaponParent_BP.WeaponCollisionComponent` _shieldweapon))
          (return true))
        (:`Is Not Valid`
          (return false))))
    (:`NewEnumerator3`
      _)
    (:`NewEnumerator4`
      _)
    (:`NewEnumerator5`
      _)
    (:`NewEnumerator6`
      _))
  ;[1 0 0.05719] Disable Unarmed Attack Trace
  (`/Engine/EditorBlueprintResources/StandardMacros.IsValid` _returnvalue_3
    (:`Is Valid`
      (`/Game/Library/CombatSystem/Blueprints/Components/CollisionComponent.DisableCollision` _returnvalue_3)
      (return true))
    (:`Is Not Valid`
      (return false))))