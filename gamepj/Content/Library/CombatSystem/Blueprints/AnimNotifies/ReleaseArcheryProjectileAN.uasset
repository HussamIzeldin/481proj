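; Animation notify that signals the owning actor to release an archery projectile at a set point in an animation.
; On notify, it sends a ReleaseArcheryProjectile message to the mesh owner, carrying the notify's attack settings.
; These settings cover swing direction, attack power and type, knockback, unblockability, and regular and poise damage multipliers.
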(fn `Received_Notify`
  (params (MeshComp :type "SkeletalMeshComponent Object Reference") (Animation :type "AnimSequenceBase Object Reference"))
  (returns (ReturnValue :type Boolean))
  (message `/Game/Library/CombatSystem/Blueprints/Interfaces/CombatBPI.ReleaseArcheryProjectile` (`ActorComponent.GetOwner` MeshComp) (`self.SwingDirection`) (`self.AttackPower`) (`self.CustomAttackType`) (`self.CauseKnockback`) (`self.KnockbackTime`) (`self.KnockbackSpeed`) (`self.IsUnblockableAttack?`) (`self.RegularDamageMultiplier`) (`self.PoiseDamageMultiplier`))
  (return true))