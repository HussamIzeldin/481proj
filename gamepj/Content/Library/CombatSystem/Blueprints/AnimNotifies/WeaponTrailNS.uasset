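; Anim notify state that shows a weapon trail over a window of an animation.
; It finds the owner's EquipmentComponent and picks the right-hand or off-hand weapon actor from the WeaponSlotForTrail setting.
; Notify begin calls StartTrail on that weapon with the configured trail and UseNotifyTrail flag, and notify end calls EndTrail, each only when the component and weapon are valid.
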(fn `Received_NotifyBegin`
  (params (MeshComp :type "SkeletalMeshComponent Object Reference") (Animation :type "AnimSequenceBase Object Reference") (TotalDuration :type "Float (double-precision)"))
  (returns (ReturnValue :type Boolean))
  (bind _returnvalue (`Actor.GetComponentByClass` (`ActorComponent.GetOwner` MeshComp) "/Game/Library/InventoryandEquipment/Blueprints/Components/EquipmentComponent.EquipmentComponent_C"))
  (bind _returnvalue_2 (`/Game/Library/InventoryandEquipment/Blueprints/Components/EquipmentComponent.Get Equipped Weapon Actor` _returnvalue "VR_LeftHand"))
  (bind _returnvalue_3 (`/Game/Library/InventoryandEquipment/Blueprints/Components/EquipmentComponent.Get Equipped Weapon Actor` _returnvalue))
  (`/Engine/EditorBlueprintResources/StandardMacros.IsValid` _returnvalue
    (:`Is Valid`
      (switch `/Game/Library/CombatSystem/Blueprints/Enums/CombatEnums/E_CollisionTraceTarget` (`self.WeaponSlotForTrail`)
        (:`NewEnumerator2`
          (`/Engine/EditorBlueprintResources/StandardMacros.IsValid` _returnvalue_3
            (:`Is Valid`
              (`/Game/Library/InventoryandEquipment/Blueprints/Actors/WeaponParent_BP.StartTrail` _returnvalue_3 (`self.WeaponTrail`) (`self.UseNotifyTrail`))
              (return true))))
        (:`NewEnumerator1`
          (`/Engine/EditorBlueprintResources/StandardMacros.IsValid` _returnvalue_2
            (:`Is Valid`
              (`/Game/Library/InventoryandEquipment/Blueprints/Actors/WeaponParent_BP.StartTrail` _returnvalue_2 (`self.WeaponTrail`) (`self.UseNotifyTrail`))
              (return true))))))))

(fn `Received_NotifyEnd`
  (params (MeshComp :type "SkeletalMeshComponent Object Reference") (Animation :type "AnimSequenceBase Object Reference"))
  (returns (ReturnValue :type Boolean))
  (bind _returnvalue (`Actor.GetComponentByClass` (`ActorComponent.GetOwner` MeshComp) "/Game/Library/InventoryandEquipment/Blueprints/Components/EquipmentComponent.EquipmentComponent_C"))
  (bind _returnvalue_2 (`/Game/Library/InventoryandEquipment/Blueprints/Components/EquipmentComponent.Get Equipped Weapon Actor` _returnvalue "VR_LeftHand"))
  (bind _returnvalue_3 (`/Game/Library/InventoryandEquipment/Blueprints/Components/EquipmentComponent.Get Equipped Weapon Actor` _returnvalue))
  (`/Engine/EditorBlueprintResources/StandardMacros.IsValid` _returnvalue
    (:`Is Valid`
      (switch `/Game/Library/CombatSystem/Blueprints/Enums/CombatEnums/E_CollisionTraceTarget` (`self.WeaponSlotForTrail`)
        (:`NewEnumerator2`
          (`/Engine/EditorBlueprintResources/StandardMacros.IsValid` _returnvalue_3
            (:`Is Valid`
              (`/Game/Library/InventoryandEquipment/Blueprints/Actors/WeaponParent_BP.EndTrail` _returnvalue_3)
              (return false))))
        (:`NewEnumerator1`
          (`/Engine/EditorBlueprintResources/StandardMacros.IsValid` _returnvalue_2
            (:`Is Valid`
              (`/Game/Library/InventoryandEquipment/Blueprints/Actors/WeaponParent_BP.EndTrail` _returnvalue_2))))))))