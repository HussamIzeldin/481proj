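; Anim notify state that grants invincibility frames during a section of an animation, such as a dodge, in the combat system.
; On begin it finds the CharacterStateManagerComponent on the mesh owner and sets it invulnerable.
; On end it clears that invulnerability, so the window length follows the notify's placement on the animation timeline.
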(fn `Received_NotifyBegin`
  (params (MeshComp :type "SkeletalMeshComponent Object Reference") (Animation :type "AnimSequenceBase Object Reference") (TotalDuration :type "Float (double-precision)"))
  (returns (ReturnValue :type Boolean))
  (bind _returnvalue (`Actor.GetComponentByClass` (`ActorComponent.GetOwner` MeshComp) "/Game/Library/CombatSystem/Blueprints/Components/CharacterStateManagerComponent.CharacterStateManagerComponent_C"))
  (`/Engine/EditorBlueprintResources/StandardMacros.IsValid` _returnvalue
    (:`Is Valid`
      (`/Game/Library/CombatSystem/Blueprints/Components/CharacterStateManagerComponent.Set Invulnerable` _returnvalue true)
      (return true))))

(fn `Received_NotifyEnd`
  (params (MeshComp :type "SkeletalMeshComponent Object Reference") (Animation :type "AnimSequenceBase Object Reference"))
  (returns (ReturnValue :type Boolean))
  (bind _returnvalue (`Actor.GetComponentByClass` (`ActorComponent.GetOwner` MeshComp) "/Game/Library/CombatSystem/Blueprints/Components/CharacterStateManagerComponent.CharacterStateManagerComponent_C"))
  (`/Engine/EditorBlueprintResources/StandardMacros.IsValid` _returnvalue
    (:`Is Valid`
      (`/Game/Library/CombatSystem/Blueprints/Components/CharacterStateManagerComponent.Set Invulnerable` _returnvalue false)
      (return false))))