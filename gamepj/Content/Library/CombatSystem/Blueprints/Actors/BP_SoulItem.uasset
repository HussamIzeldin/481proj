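; BP_SoulItem is a pickup actor that carries souls to the player and grants them on arrival.
; On BeginPlay it destroys itself if Souls is not positive, otherwise a MoveToPlayer timeline lerps it from its spawn location to the player character's current position.
; When the timeline finishes, it calls GainSouls on the player's StatsManagerComponent and destroys itself.
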(event `self.ReceiveBeginPlay`
  (if (> (`self.Souls`) 0)
    (set `self.InitialActorLocation` (`self.K2_GetActorLocation`))
    (bind (_direction _alpha) (`Timeline|MoveToPlayer`)
      (:`Update`
        (`self.K2_SetActorLocation` (`KismetMathLibrary.VLerp` (`self.InitialActorLocation`) (`self.K2_GetActorLocation` (`GameplayStatics.GetPlayerCharacter` 0)) _alpha)))
      (:`Finished`
        (`self.FinishCollectItem`)))
    (else
      (`self.K2_DestroyActor`))))

(event `FinishCollectItem`
  (`/Game/Library/CombatSystem/Blueprints/Components/StatsManagerComponent.GainSouls` (`self.GetComponentByClass` (`GameplayStatics.GetPlayerCharacter` 0) "/Game/Library/CombatSystem/Blueprints/Components/StatsManagerComponent.StatsManagerComponent_C") (`self.Souls`))
  (`self.K2_DestroyActor`))

(fn `UserConstructionScript`)