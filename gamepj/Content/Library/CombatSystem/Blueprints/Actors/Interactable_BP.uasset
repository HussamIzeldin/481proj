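; Base interactable actor for the combat system, showing a prompt widget and tracking whether an interaction is in progress.
; On BeginPlay it caches its message widget and sets the prompt text after a short delay.
; Toggling the prompt refreshes its gamepad/keyboard style and hides it during interaction.
; Interact and EndInteraction update that state and call empty begin/end hooks, alongside stub getters for loot and spawn transform.
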(event `self.ReceiveBeginPlay`
  (bind _aswb_interactable_message (cast `/Game/Library/UI/MainMenu/Blueprints/WidgetBP/WB_InteractableMessage` (`WidgetComponent.GetUserWidgetObject` (`self.InteractionWidget`))))
  (set `self.InteractionWidgetBP` _aswb_interactable_message)
  (`KismetSystemLibrary.Delay` 0.2)
  (`/Game/Library/UI/MainMenu/Blueprints/WidgetBP/WB_Text.SetText` (`/Game/Library/UI/MainMenu/Blueprints/WidgetBP/WB_MenuPrompt.Text` (`/Game/Library/UI/MainMenu/Blueprints/WidgetBP/WB_InteractableMessage.WB_MenuPrompt` (`self.InteractionWidgetBP`))) (`self.InteractableMessage`)))

(event `/Game/Library/CombatSystem/Blueprints/Interfaces/InteractableBPI.ToggleInteractableMessage`
  (params (`Enabled?` :type Boolean))
  (bind _interactionwidgetbp (`self.InteractionWidgetBP`)
    (:`then`
      (bind _usinggamepad_ (message `/Game/Library/CombatSystem/Blueprints/Interfaces/PlayerControllerBPI.isUsingGamepad?` (`GameplayStatics.GetPlayerController` 0)))
      (`/Game/Library/UI/MainMenu/Blueprints/WidgetBP/WB_MenuPrompt.OnInputMethodChanged` (`/Game/Library/UI/MainMenu/Blueprints/WidgetBP/WB_InteractableMessage.WB_MenuPrompt` (`self.InteractionWidgetBP`)) _usinggamepad_)
      (`Widget.SetVisibility` _interactionwidgetbp (select `bool` (and `Enabled?` (not (`self.bIsInteracting`))) :`false` "Collapsed" :`true` "SelfHitTestInvisible" :!type "ESlateVisibility Enum")))
    (:`else`)))

(event `/Game/Library/CombatSystem/Blueprints/Interfaces/InteractableBPI.Interact`
  (params (Caller :type "Actor Object Reference"))
  (bind _output_get (set `self.Interactor` Caller))
  (`self.SetInteracting` true)
  (`self.OnInteractionBegin` _output_get))

(event `/Game/Library/CombatSystem/Blueprints/Interfaces/InteractableBPI.EndInteraction`
  (`self.SetInteracting` false)
  (`self.OnInteractionEnd`))

(fn `GetInteractableType`
  (returns (InteractableType :type "/Game/Library/CombatSystem/Blueprints/Enums/E_Interactables Enum"))
  (return (`self.Interactable_Type`)))

(fn `GetLootItems`
  (returns (ItemToEquip :type "Array of /Game/Library/InventoryandEquipment/Blueprints/Structs/ItemSlot_Struct Structure"))
  (return))

(fn `GetPlayerSpawnTransform`
  (returns (SpawnTransform :type "Transform Structure"))
  (return))

(fn `isInteracting?`
  (returns (bIsInteracting :type Boolean))
  (return (`self.bIsInteracting`)))

(fn `OnInteractionBegin`
  (params (Caller :type "Actor Object Reference")))

(fn `OnInteractionEnd`)

(fn `SetInteracting`
  (params (isInteracting :type Boolean))
  (set `self.bIsInteracting` isInteracting))

(fn `UserConstructionScript`)