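; Interactable soul pickup in the combat system that grants its stored souls to whoever interacts with it.
; On Interact it passes its Souls value to the caller's StatsManagerComponent, then shows the WB_SoulsRetrieved widget on player 0's viewport.
; The actor destroys itself afterward if DestroyInteractableOnUse is set.
; GetPlayerSpawnTransform and the construction script are empty.
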(event `/Game/Library/CombatSystem/Blueprints/Interfaces/InteractableBPI.Interact`
  (params (Caller :type "Actor Object Reference"))
  (`/Game/Library/CombatSystem/Blueprints/Components/StatsManagerComponent.GainSouls` (`self.GetComponentByClass` Caller "/Game/Library/CombatSystem/Blueprints/Components/StatsManagerComponent.StatsManagerComponent_C") (`self.Souls`))
  (bind _returnvalue (`|CreateWidget` "/Game/Library/UI/CombatUI/Widgets/WB_SoulsRetrieved.WB_SoulsRetrieved_C" (`GameplayStatics.GetPlayerController` 0)))
  (`UserWidget.AddToViewport` _returnvalue 0)
  (if (`self.bDestroyInteractableOnUse?`)
    (`self.K2_DestroyActor`)))

(fn `GetPlayerSpawnTransform`
  (returns (SpawnTransform :type "Transform Structure"))
  (return))

(fn `UserConstructionScript`)