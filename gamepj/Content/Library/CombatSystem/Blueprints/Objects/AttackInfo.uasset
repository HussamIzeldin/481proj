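; AttackInfo is a combat system data object that holds the parameters describing an attack.
; StoreAttackInfo copies swing direction, power, category, combat type, index, custom type, knockback settings and an unblockable flag into member variables.
; GetCustomAttackType looks up an impact decision in the TestCustomAttackType map, independent of the stored CustomAttackType.
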(fn `GetCustomAttackType`
  (params (ImpactDecision :type "/Game/Library/CombatSystem/Blueprints/Enums/E_ImpactDecision Enum" :default "NewEnumerator5"))
  (returns (Value :type "/Game/Library/CombatSystem/Blueprints/Enums/CombatEnums/E_HitReactionType Enum"))
  (return (`BlueprintMapLibrary.Map_Find` (`self.TestCustomAttackType`) ImpactDecision)))

(fn `StoreAttackInfo`
  (params (MeleeSwingDirection :type "/Game/Library/CombatSystem/Blueprints/Enums/CombatEnums/E_MeleeSwingDirection Enum" :default "NewEnumerator21") (AttackPower :type "/Game/Library/CombatSystem/Blueprints/Enums/CombatEnums/E_AttackPower Enum" :default "NewEnumerator0") (CustomAttackType :type "/Game/Library/CombatSystem/Blueprints/Enums/CombatEnums/E_CustomAttackTypes Enum" :default "NewEnumerator0") (`CauseKnockback?` :type Boolean) (KnockbackTime :type "Float (double-precision)") (KnockbackSpeed :type "Float (double-precision)") (`IsUnblockableAttack?` :type Boolean) (AttackCategory :type "/Game/Library/CombatSystem/Blueprints/Enums/E_AttackCategory Enum" :default "NewEnumerator0") (CombatType :type "/Game/Library/CombatSystem/Blueprints/Enums/CombatEnums/E_CombatType Enum" :default "NewEnumerator16") (AttackIndex :type Integer))
  (set `self.MeleeSwingDirection` MeleeSwingDirection)
  (set `self.AttackPower` AttackPower)
  (set `self.CustomAttackType` CustomAttackType)
  (set `self.CauseKnockback?` `CauseKnockback?`)
  (set `self.KnockbackTime` KnockbackTime)
  (set `self.KnockbackSpeed` KnockbackSpeed)
  (set `self.IsUnblockableAttack?` `IsUnblockableAttack?`)
  (set `self.AttackCategory` AttackCategory)
  (set `self.CombatType` CombatType)
  (set `self.AttackIndex` AttackIndex))