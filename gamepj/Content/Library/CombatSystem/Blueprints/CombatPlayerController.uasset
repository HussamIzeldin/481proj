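; Player controller for the combat system that owns and toggles the player's UI widgets.
; InitializeMainHUD builds the HUD, pause, inventory, equipment and vendor sell menus from the passed components, mostly collapsed until toggled.
; Archery, bonfire and message widgets are created on separate events, and getters expose several widgets and state.
; Key and mouse input track gamepad versus mouse use, which sets cursor visibility for the bonfire menu.
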(event `AddArcheryWidget`
  (bind _archerywidget (`self.ArcheryWidget`)
    (:`then`
      (`Widget.RemoveFromParent` _archerywidget))
    (:`else`
      _))
  (bind _returnvalue (`|CreateWidget` "/Game/Library/UI/CombatUI/Widgets/ArcheryHUD_Widget.ArcheryHUD_Widget_C" self 1.0 0.0))
  (bind _output_get (set `self.ArcheryWidget` _returnvalue))
  (`UserWidget.AddToViewport` _output_get 0))

(event `InitializeMainHUD`
  (params (OwnerStatsComponent :type "/Game/Library/CombatSystem/Blueprints/Components/StatsManagerComponent Object Reference") (OwnerEquipmentManager :type "/Game/Library/InventoryandEquipment/Blueprints/Components/EquipmentComponent Object Reference") (PlayerInventoryComponent :type "/Game/Library/InventoryandEquipment/Blueprints/Components/PlayerInventoryComponent Object Reference"))
  (bind _playerequipmentmenu (`self.PlayerEquipmentMenu`))
  (bind _inventorycomponent (`/Game/Library/InventoryandEquipment/Blueprints/Components/EquipmentComponent.InventoryComponent` OwnerEquipmentManager))
  (`|ExecutionSequence`
    (:`then_0`
      (bind _mainhudwidget (`self.MainHUDWidget`)
        (:`then`
          (`Widget.RemoveFromParent` _mainhudwidget))
        (:`else`
          _))
      (bind _returnvalue (`|CreateWidget` "/Game/Library/UI/CombatUI/Widgets/MainHUD.MainHUD_C" self))
      (bind _output_get (set `self.MainHUDWidget` _returnvalue))
      (`/Game/Library/UI/CombatUI/Widgets/MainHUD.InitializeStatBars` _output_get OwnerStatsComponent)
      (`/Game/Library/UI/CombatUI/Widgets/MainHUD.InitializeQuickSlots` _output_get OwnerEquipmentManager)
      (`UserWidget.AddToViewport` _output_get 0))
    (:`then_1`
      (bind _returnvalue_2 (`|CreateWidget` "/Game/Library/UI/MainMenu/Blueprints/WidgetBP/WB_PauseMenu.WB_PauseMenu_C" self))
      (set `self.PauseMenu` _returnvalue_2)
      (`Widget.SetVisibility` (`self.PauseMenu`) "Collapsed")
      (`UserWidget.AddToViewport` (`self.PauseMenu`) 0))
    (:`then_2`
      (bind _playerinventorywidget (`self.PlayerInventoryWidget`)
        (:`then`
          (`Widget.RemoveFromParent` _playerinventorywidget))
        (:`else`
          _))
      (bind _returnvalue_3 (`|CreateWidget` "/Game/Library/UI/InventoryEquipmentUI/Blueprints/WB_PlayerInventoryMenu.WB_PlayerInventoryMenu_C" self))
      (bind _output_get_2 (set `self.PlayerInventoryWidget` _returnvalue_3))
      (`Widget.SetVisibility` _output_get_2 "Collapsed")
      (`UserWidget.AddToViewport` (`self.PlayerInventoryWidget`) 0))
    (:`then_3`
      (`KismetSystemLibrary.Delay` 0.2)
      (bind _returnvalue_4 (`|CreateWidget` "/Game/Library/UI/InventoryEquipmentUI/Blueprints/WB_VendorInventory.WB_VendorInventory_C" self "NewEnumerator2"))
      (bind _output_get_3 (set `self.WB_PlayerSellInventory` _returnvalue_4))
      (`Widget.SetVisibility` _output_get_3 "Collapsed")
      (`UserWidget.AddToViewport` _output_get_3 0)
      (`/Game/Library/UI/InventoryEquipmentUI/Blueprints/WB_CoreInventory.Initialize` (`/Game/Library/UI/InventoryEquipmentUI/Blueprints/WB_VendorInventory.WB_CoreInventory` (`self.WB_PlayerSellInventory`)) (`/Game/Library/InventoryandEquipment/Blueprints/Components/InventoryComponent.SlotsPerRow` _inventorycomponent) _inventorycomponent))
    (:`then_4`
      (bind _returnvalue_5 (`|CreateWidget` "/Game/Library/UI/InventoryEquipmentUI/Blueprints/WB_EquipmentWindow.WB_EquipmentWindow_C" self))
      (bind _output_get_4 (set `self.PlayerEquipmentMenu` _returnvalue_5))
      (`/Game/Library/UI/InventoryEquipmentUI/Blueprints/WB_EquipmentWindow.InitializeEquipmentWindow` _output_get_4 PlayerInventoryComponent OwnerEquipmentManager)
      (`Widget.SetVisibility` _playerequipmentmenu "Collapsed")
      (`UserWidget.AddToViewport` _playerequipmentmenu 0))))

(event `/Game/Library/CombatSystem/Blueprints/Interfaces/PlayerControllerBPI.OpenMessageWidget`
  (params (Message :type Text) (`UseOverlay?` :type Boolean))
  (bind _messagewidget (`self.MessageWidget`))
  (bind _messagewidget_2 (`self.MessageWidget`))
  (bind _messagewidget_3 (`self.MessageWidget`))
  (`/Engine/EditorBlueprintResources/StandardMacros.IsValid` _messagewidget_3
    (:`Is Valid`
      (`/Game/Library/UI/InventoryEquipmentUI/Blueprints/Subwidgets/WB_ErrorMessage.Update` _messagewidget_3 Message `UseOverlay?`)
      (`Widget.SetKeyboardFocus` _messagewidget)
      (`Widget.SetVisibility` _messagewidget "Visible"))
    (:`Is Not Valid`
      (bind _returnvalue (`|CreateWidget` "/Game/Library/UI/InventoryEquipmentUI/Blueprints/Subwidgets/WB_ErrorMessage.WB_ErrorMessage_C" self Message `UseOverlay?`))
      (set `self.MessageWidget` _returnvalue)
      (`UserWidget.AddToViewport` _messagewidget_2 0)
      (`Widget.SetKeyboardFocus` _messagewidget_2))))

(event `/Game/Library/CombatSystem/Blueprints/Interfaces/PlayerControllerBPI.ToggleBonfireMenu`
  ;[0.8516 0 1] Add bonfire menu to the players viewport
  (bind _returnvalue (`|CreateWidget` "/Game/Library/UI/MainMenu/Blueprints/WidgetBP/WB_BonfireSelection.WB_BonfireSelection_C" (`GameplayStatics.GetPlayerController` 0)))
  (bind _output_get (set `self.BonfireMenu` _returnvalue))
  (`UserWidget.AddToViewport` _output_get 0)
  (if (`self.bUsingGamepad?`)
    (set `self.bShowMouseCursor` false)
    (else
      (set `self.bShowMouseCursor` true))))

(event `/Game/Library/CombatSystem/Blueprints/Interfaces/PlayerControllerBPI.TogglePauseMenu`
  (params (`Enable?` :type Boolean))
  (bind _pausemenu (`self.PauseMenu`))
  ;[0 1 0.08594] Toggle the player menu's on and off
  (`|ExecutionSequence`
    (:`then_0`
      (bind _playerequipmentmenu (`self.PlayerEquipmentMenu`)
        (:`then`
          (`/Game/Library/UI/InventoryEquipmentUI/Blueprints/WB_EquipmentWindow.CloseMenu` _playerequipmentmenu))
        (:`else`
          _))
      (bind _playerinventorywidget (`self.PlayerInventoryWidget`)
        (:`then`
          (`/Game/Library/UI/InventoryEquipmentUI/Blueprints/WB_PlayerInventoryMenu.Close Menu` _playerinventorywidget))
        (:`else`)))
    (:`then_1`
      (`/Engine/EditorBlueprintResources/StandardMacros.IsValid` (`self.PlayerInventoryWidget`)
        (:`Is Valid`
          (if (`/Game/Library/UI/MainMenu/Blueprints/WidgetBP/WB_PauseMenu.bIsMenuOpen?` (`self.PauseMenu`))
            (`/Game/Library/UI/MainMenu/Blueprints/WidgetBP/WB_PauseMenu.Resume` _pausemenu)
            (else
              (`/Game/Library/UI/MainMenu/Blueprints/WidgetBP/WB_PauseMenu.Open Menu` _pausemenu))))))))

(event `/Game/Library/CombatSystem/Blueprints/Interfaces/PlayerControllerBPI.TogglePlayerInventory`
  (params (`Enable?` :type Boolean))
  (bind _playerinventorywidget (`self.PlayerInventoryWidget`))
  ;[0 1 0.08594] Toggle the player menu's on and off
  (`|ExecutionSequence`
    (:`then_0`
      (bind _playerequipmentmenu (`self.PlayerEquipmentMenu`)
        (:`then`
          (`/Game/Library/UI/InventoryEquipmentUI/Blueprints/WB_EquipmentWindow.CloseMenu` _playerequipmentmenu))
        (:`else`)))
    (:`then_1`
      (`/Engine/EditorBlueprintResources/StandardMacros.IsValid` (`self.PlayerInventoryWidget`)
        (:`Is Valid`
          (if (`/Game/Library/UI/InventoryEquipmentUI/Blueprints/WB_PlayerInventoryMenu.bIsMenuOpen?` (`self.PlayerInventoryWidget`))
            (`/Game/Library/UI/InventoryEquipmentUI/Blueprints/WB_PlayerInventoryMenu.Resume` _playerinventorywidget)
            (else
              (`/Game/Library/UI/InventoryEquipmentUI/Blueprints/WB_PlayerInventoryMenu.OpenMenu` _playerinventorywidget))))))))

(event `/Game/Library/CombatSystem/Blueprints/Interfaces/PlayerControllerBPI.TogglePlayerEquipment`
  (params (`Enable?` :type Boolean))
  (bind _playerequipmentmenu (`self.PlayerEquipmentMenu`))
  (bind _playerequipmentmenu_2 (`self.PlayerEquipmentMenu`))
  ;[0 1 0.08594] Toggle the player menu's on and off
  (`|ExecutionSequence`
    (:`then_0`
      (bind _playerinventorywidget (`self.PlayerInventoryWidget`)
        (:`then`
          (`/Game/Library/UI/InventoryEquipmentUI/Blueprints/WB_PlayerInventoryMenu.Close Menu` _playerinventorywidget))
        (:`else`)))
    (:`then_1`
      (`/Engine/EditorBlueprintResources/StandardMacros.IsValid` _playerequipmentmenu_2
        (:`Is Valid`
          (if (`/Game/Library/UI/InventoryEquipmentUI/Blueprints/WB_EquipmentWindow.bIsMenuOpen?` _playerequipmentmenu_2)
            (`/Game/Library/UI/InventoryEquipmentUI/Blueprints/WB_EquipmentWindow.Resume` _playerequipmentmenu)
            (else
              (`/Game/Library/UI/InventoryEquipmentUI/Blueprints/WB_EquipmentWindow.OpenMenu` _playerequipmentmenu))))))))

(event `Key|AnyKey` :consume false
  (params (Key :type "Key Structure"))
  (:`Pressed`
    (`self.SetUsingGamepad` (`KismetInputLibrary.Key_IsGamepadKey` Key))))

(event `/Game/Library/CombatSystem/Blueprints/Interfaces/PlayerControllerBPI.UpdateInputMethod`
  (params (`UsingGamepad?` :type Boolean))
  (`self.SetUsingGamepad` `UsingGamepad?`))

(event `/Game/Library/CombatSystem/Blueprints/Interfaces/PlayerControllerBPI.DisablePauseMenu`
  (`/Game/Library/UI/InventoryEquipmentUI/Blueprints/WB_PlayerInventoryMenu.Resume` (`self.PlayerInventoryWidget`)))

(event `/Game/Library/CombatSystem/Blueprints/Interfaces/PlayerControllerBPI.UpdateCurrentVendorInteractionWidget`
  (params (Widget :type "Widget Object Reference"))
  (set `self.VendorInteractionWidget` Widget))

(event `SetUsingGamepad`
  (params (`bUsingGamepad?` :type Boolean))
  (if (!= `bUsingGamepad?` (`self.bUsingGamepad?`))
    (bind _output_get (set `self.bUsingGamepad?` `bUsingGamepad?`))
    (`self.OnInputMethodChanged` _output_get)))

(event `/Game/Library/CombatSystem/Blueprints/Interfaces/PlayerControllerBPI.TogglePlayerSellWidget`
  (params (`Visible?` :type Boolean))
  (`Widget.SetVisibility` (`self.WB_PlayerSellInventory`) (select `bool` `Visible?` :`false` "Collapsed" :`true` "SelfHitTestInvisible" :!type "ESlateVisibility Enum"))
  (if `Visible?`
    _))

(event `InputAxisKey|MouseX` :consume false :overrideparent false
  (params (AxisValue :type "Float (single-precision)"))
  (if (or (!= AxisValue 0.0) (!= (stale `InputAxisKey|MouseY` AxisValue) 0.0)) :!label _label
    (`self.SetUsingGamepad` false)))

(event `InputAxisKey|MouseY` :consume false :overrideparent false
  (params (AxisValue :type "Float (single-precision)"))
  (goto _label))

(event `OnInputMethodChanged`
  (params (`IsUsingGamepad?` :type Boolean))
  (if `IsUsingGamepad?`
    (`self.SetMouseLocation` 0)))

(event `/Game/Library/CombatSystem/Blueprints/Interfaces/PlayerControllerBPI.ToggleUserInterface`
  (params (UserInterface :type "/Game/Library/UI/MainMenu/Blueprints/Enums/E_UserInterface Enum" :default "NewEnumerator0"))
  (switch `/Game/Library/UI/MainMenu/Blueprints/Enums/E_UserInterface` UserInterface
    (:`NewEnumerator3`
      (bind _bonfiremenu (`self.BonfireMenu`)
        (:`then`
          (if (`/Game/Library/UI/MainMenu/Blueprints/WidgetBP/WB_BonfireSelection.BonfireMenuOpen` _bonfiremenu)
            (`/Game/Library/UI/MainMenu/Blueprints/WidgetBP/WB_BonfireSelection.SetBonfireActive` _bonfiremenu false)
            (else
              (`/Game/Library/UI/MainMenu/Blueprints/WidgetBP/WB_BonfireSelection.SetBonfireActive` _bonfiremenu true)
              (if (`self.bUsingGamepad?`) :!label _label_2
                (set `self.bShowMouseCursor` false)
                (else
                  (set `self.bShowMouseCursor` true)))
              (`WidgetBlueprintLibrary.SetInputMode_UIOnlyEx` self (`self.BonfireMenu`)))))
        (:`else`
          (bind _returnvalue (`|CreateWidget` "/Game/Library/UI/MainMenu/Blueprints/WidgetBP/WB_BonfireSelection.WB_BonfireSelection_C" self))
          (bind _output_get (set `self.BonfireMenu` _returnvalue))
          (`UserWidget.AddToViewport` _output_get 0)
          (goto _label_2))))))

(fn `GetCharacterClassType`
  (returns (Class :type Text))
  (return "Character Class"))

(fn `GetCharacterName`
  (returns (Name :type Text))
  (return (`self.CharacterName`)))

(fn `GetCurrentVendorInteractionWidget`
  (returns (Widget :type "Widget Object Reference"))
  (return (`self.VendorInteractionWidget`)))

(fn `GetMainHUD`
  (returns (MainHUD :type "UserWidget Object Reference"))
  (return (`self.MainHUDWidget`)))

(fn `GetPauseMenuWidget`
  (returns (Menu :type "UserWidget Object Reference"))
  (return (`self.PlayerInventoryWidget`)))

(fn `GetPlayerHUD`
  (returns (MainHUDWidget :type "/Game/Library/UI/CombatUI/Widgets/MainHUD Object Reference"))
  (bind _mainhudwidget (`self.MainHUDWidget`)
    (:`then`
      (return _mainhudwidget))
    (:`else`)))

(fn `GetPlayerSellWidget`
  (returns (SellWidget :type "Widget Object Reference"))
  (return (`self.WB_PlayerSellInventory`)))

(fn `GetPrevUserInterface`
  (returns (PrevUserInterface :type "/Game/Library/UI/MainMenu/Blueprints/Enums/E_UserInterface Enum"))
  (return (`self.PrevUserInterfaceOpened`)))

(fn `GetUserInterfaceOpen`
  (returns (OpenedUserInterface :type "/Game/Library/UI/MainMenu/Blueprints/Enums/E_UserInterface Enum"))
  (return (`self.UserInterfaceOpened`)))

(fn `isUsingGamepad?`
  (returns (`UsingGamepad?` :type Boolean))
  (return (`self.bUsingGamepad?`)))

(fn `UserConstructionScript`)