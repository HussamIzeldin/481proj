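; Base arrow projectile for AI bow attacks that launches on spawn and either sticks or bounces on impact.
; A state machine toggles socket-traced collision and a runtime-added movement component, with speed scaled by bow charge and delayed gravity.
; Pawn hits apply regular, poise and additional damage, feeding the victim's HitReactionComponent.
; Block outcome or surface type decides between attaching and physics bounce, with cleanup via lifespan.
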(event `self.ReceiveBeginPlay`
  ;[0 1 0.2266 0.5] Event Begin Play
  (`parent.ReceiveBeginPlay`)
  (bind _ascharacter (cast `Character` (`self.GetOwner`)))
  (set `self.Owner Character` _ascharacter)
  (`/Game/Library/CombatSystem/Blueprints/Components/CollisionComponent.InitializeComponent` (`self.ProjectileCollisionComponent`) (`self.GetOwner`))
  (`StaticMeshComponent.SetStaticMesh` (`self.Arrow Mesh`) (`self.AI Arrow Mesh`))
  (`PrimitiveComponent.SetCollisionProfileName` (`self.Arrow Mesh`) "NoCollision" true)
  (`self.Set Weapon Projectile State` "NewEnumerator3"))

(event `self.ProjectileCollisionComponent.OnCollisionEnabled`
  (params (TraceTarget :type "/Game/Library/CombatSystem/Blueprints/Enums/CombatEnums/E_CollisionTraceTarget Enum" :default "NewEnumerator0"))
  (bind _arrow_mesh (`self.Arrow Mesh`))
  (`/Game/Library/CombatSystem/Blueprints/Components/CollisionComponent.SetCollisionMesh` (`self.ProjectileCollisionComponent`) _arrow_mesh (`SceneComponent.GetAllSocketNames` _arrow_mesh)))

(event `SetProjectileVelocity`
  (bind _projectilecomponent (`self.ProjectileComponent`))
  (bind _returnvalue (* (`self.GetActorForwardVector`) (`KismetMathLibrary.Lerp` 100.0 8000.0 (`self.BowChargeAmount`))))
  ;[0 0.2314 1 1 39] Shoot Projectile
  (`GameplayStatics.PlaySoundAtLocation` (`self.ShootProjectileSound`) (`self.K2_GetActorLocation`) (struct) 1.0 1.0 0.0 null null null)
  (bind _returnvalue_2 (`AddComponent|NODE_AddProjectileMovementComponent-1`))
  (bind _output_get (set `self.ProjectileComponent` _returnvalue_2))
  (set `ProjectileMovementComponent.InitialSpeed` (`KismetMathLibrary.VSize` _returnvalue) _output_get)
  (set `ProjectileMovementComponent.bRotationFollowsVelocity` true _output_get)
  (set `MovementComponent.Velocity` _returnvalue _output_get)
  (`|ExecutionSequence`
    (:`then_0`
      (`KismetSystemLibrary.Delay` 0.3)
      (`/Engine/EditorBlueprintResources/StandardMacros.IsValid` _projectilecomponent
        (:`Is Valid`
          (set `ProjectileMovementComponent.ProjectileGravityScale` 0.3 _projectilecomponent))))
    (:`then_1`
      (`ActorComponent.Activate` (`self.Particletrail`) false))))

(event `self.ProjectileCollisionComponent.OnHit`
  (params (HitResult :type "HitResult Structure") (HitCollisionChannel :type "ECollisionChannel Enum" :default "ECC_WorldStatic"))
  (bind _hitcharacter (`self.HitCharacter`))
  (bind _lasthit (`self.LastHit`))
  (bind _arrow_mesh (`self.Arrow Mesh`))
  (bind _returnvalue (- (`.ImpactPoint` (`GameplayStatics.BreakHitResult` (`self.LastHit`))) (* (`self.GetActorForwardVector`) 50.0)))
  ;[1 0 0.008357 1 37] Projectile Hit Event
  (if (`|EnumEquality` HitCollisionChannel "ECC_Pawn")
    (set `self.LastHit` HitResult)
    (bind _success_ (`self.TryToApplyDamage` (`.HitActor` (`GameplayStatics.BreakHitResult` (`self.LastHit`)))))
    (if _success_
      (`self.Set Weapon Projectile State` "NewEnumerator1")
      (`/Engine/EditorBlueprintResources/StandardMacros.IsValid` _hitcharacter
        (:`Is Valid`
          (if (select `/Game/Library/CombatSystem/Blueprints/Enums/E_ImpactDecision` (`.ImpactDecision_39_7AC92D644C6F631EC7CB2C84C1C36CB4` (break `/Game/Library/CombatSystem/Blueprints/Structs/CombatHitData_Struct` (`self.LastCombatHitData`))) :`NewEnumerator0` true :`NewEnumerator4` true)
            (bind (_sweephitresult _returnvalue_2) (`self.K2_SetActorLocation` _returnvalue false true))
            (if _returnvalue_2
              (`self.K2_AttachToComponent` (`Character.Mesh` _hitcharacter) (`.HitBoneName` (`GameplayStatics.BreakHitResult` (`self.LastHit`))) "KeepWorld" "KeepWorld" "KeepWorld")
              (`self.Set Weapon Projectile State` "NewEnumerator5"))
            (else
              (`PrimitiveComponent.SetSimulatePhysics` _arrow_mesh true :!label _label)
              (`PrimitiveComponent.SetCollisionProfileName` _arrow_mesh "ragdoll" true)
              (`PrimitiveComponent.SetCollisionProfileName` (`self.Arrow Mesh`) "ragdoll" true)
              (`PrimitiveComponent.SetAllPhysicsLinearVelocity` _arrow_mesh (* (`self.GetActorForwardVector`) (`KismetMathLibrary.Lerp` -100.0 -400.0 (`self.BowChargeAmount`))) true))))
        (:`Is Not Valid`
          (if (`KismetArrayLibrary.Array_Contains` (`self.SurfaceTypesToAttach`) (`GameplayStatics.GetSurfaceType` (`self.LastHit`))) :!label _label_2
            (bind (_sweephitresult_2 _returnvalue_3) (`self.K2_SetActorLocation` _returnvalue false true))
            (if _returnvalue_3
              (`self.K2_AttachToActor` (`.HitActor` (`GameplayStatics.BreakHitResult` (`self.LastHit`))) "None" "KeepWorld" "KeepWorld" "KeepWorld")
              (`self.Set Weapon Projectile State` "NewEnumerator5"))
            (else
              (goto _label))))))
    (else
      (message `/Game/Library/CombatSystem/Blueprints/Interfaces/CombatBPI.PlayImpactEffect` (`self.GetOwner`) (`self.AttackImpactFX`) (`.ImpactPoint` (`GameplayStatics.BreakHitResult` _lasthit)) (`GameplayStatics.GetSurfaceType` _lasthit) false)
      (`self.Set Weapon Projectile State` "NewEnumerator1")
      (goto _label_2))))

(event `MaterialImpactEffect`
  (params (InputPin :type "EPhysicalSurface Enum" :default "SurfaceType_Default"))
  ;[1 0.1406 0] Material  Impact effect
  (`/Engine/EditorBlueprintResources/StandardMacros.DoOnce` false :!label _label_3
    (:`Completed`
      (set `self.SurfaceType` InputPin)
      (set `self.ImpactPoint` (`.ImpactPoint` (`GameplayStatics.BreakHitResult` (`self.LastHit`))))
      (`/Engine/EditorBlueprintResources/StandardMacros.IsValid` null
        (:`Is Valid`
          (switch `EPhysicalSurface` (`self.SurfaceType`)))))))

(event `ResetMaterialReaction`
  ;[1 0.1406 0] Material  Impact effect
  (goto _label_3 :!via `Reset`))

(fn `Get Direction`
  (returns (ReturnValue :type "Rotator Structure"))
  (locals (`Local Direction` :type "Vector Structure" :default (0.0 0.0 0.0)))
  (bind (_worldposition _worlddirection) (`GameplayStatics.DeprojectScreenToWorld` (`GameplayStatics.GetPlayerController` 0) (/ (`WidgetLayoutLibrary.GetViewportSize`) 2.0)))
  (set `local.Local Direction` _worlddirection)
  (bind (_outhit _returnvalue) (`KismetSystemLibrary.LineTraceSingleForObjects` _worldposition (+ _worldposition (* (`local.Local Direction`) 3000.0)) (`|MakeArray` "ObjectTypeQuery3" "ObjectTypeQuery1" :!type "EObjectTypeQuery Enum") false (`|MakeArray` self (`self.GetOwner`) :!type "Actor Object Reference")))
  (if _returnvalue
    (bind (_bblockinghit _binitialoverlap _time _distance _location _impactpoint _normal _impactnormal _physmat _hitactor _hitcomponent _hitbonename _hititem _faceindex _tracestart _traceend) (`GameplayStatics.BreakHitResult` _outhit))
    (bind _ascharacter (cast `Character` _hitactor)
      (:`then`
        (set `self.Hit Location` (+ _location (* (`local.Local Direction`) (`CapsuleComponent.CapsuleRadius` (`Character.CapsuleComponent` _ascharacter)))))
        (for _index (range 1 11) :!label _label
          (bind (_outhits _returnvalue_2) (`KismetSystemLibrary.SphereTraceMultiForObjects` _location (+ _location (* (`local.Local Direction`) (* _index 5.0))) 2.0 (`|MakeArray` "ObjectTypeQuery3" :!type "EObjectTypeQuery Enum")))
          (if _returnvalue_2
            (for _array_element _outhits
              (bind (_bblockinghit_2 _binitialoverlap_2 _time_2 _distance_2 _location_2 _impactpoint_2 _normal_2 _impactnormal_2 _physmat_2 _hitactor_2 _hitcomponent_2) (`GameplayStatics.BreakHitResult` _array_element))
              (if (!= (`PrimitiveComponent.GetCollisionProfileName` _hitcomponent_2) "Pawn")
                (set `self.Hit Location` _location_2)
                (goto _label :!via `Break`))))))
      (:`CastFailed`
        (set `self.Hit Location` _location)))
    (else
      (set `self.Hit Location` _traceend)))
  (return (`KismetMathLibrary.Conv_VectorToRotator` (`KismetMathLibrary.GetDirectionUnitVector` (`self.K2_GetActorLocation`) (`self.Hit Location`)))))

(fn `GetArrowState`
  (returns (ArrowState :type "/Game/Library/CombatSystem/Blueprints/Enums/Archery/E_WeaponProjectileState Enum"))
  (return (`self.ArrowState`)))

(fn `GetProjectileState`
  (returns (ProjectileState :type "/Game/Library/CombatSystem/Blueprints/Enums/Archery/E_WeaponProjectileState Enum"))
  (return "NewEnumerator0"))

(fn `OnStateBegin`
  (params (ArrowState :type "/Game/Library/CombatSystem/Blueprints/Enums/Archery/E_WeaponProjectileState Enum" :default "NewEnumerator0"))
  (bind _arrow_mesh (`self.Arrow Mesh`))
  (switch `/Game/Library/CombatSystem/Blueprints/Enums/Archery/E_WeaponProjectileState` ArrowState
    (:`NewEnumerator1`
      (`PrimitiveComponent.SetCollisionProfileName` _arrow_mesh "OverlapAllDynamic" true))
    (:`NewEnumerator2`
      (`PrimitiveComponent.SetCollisionProfileName` _arrow_mesh "NoCollision" true))
    (:`NewEnumerator3`
      (`/Game/Library/CombatSystem/Blueprints/Components/CollisionComponent.EnableCollision` (`self.ProjectileCollisionComponent`) "NewEnumerator0")
      (`self.SetProjectileVelocity`))))

(fn `OnStateEnd`
  (params (ArrowState :type "/Game/Library/CombatSystem/Blueprints/Enums/Archery/E_WeaponProjectileState Enum" :default "NewEnumerator0"))
  (bind _projectilecomponent (`self.ProjectileComponent`))
  (switch `/Game/Library/CombatSystem/Blueprints/Enums/Archery/E_WeaponProjectileState` ArrowState
    (:`NewEnumerator3`
      (`/Engine/EditorBlueprintResources/StandardMacros.IsValid` _projectilecomponent
        (:`Is Valid`
          (`ActorComponent.K2_DestroyComponent` _projectilecomponent))
        (:`Is Not Valid`
          _))
      (`/Game/Library/CombatSystem/Blueprints/Components/CollisionComponent.DisableCollision` (`self.ProjectileCollisionComponent`))
      (`ParticleSystemComponent.EndTrails` (`self.Particletrail`))
      (`self.SetLifeSpan` 15.0))))

(fn `Set Weapon Projectile State`
  (params (New_ArrowState :type "/Game/Library/CombatSystem/Blueprints/Enums/Archery/E_WeaponProjectileState Enum" :default "NewEnumerator0"))
  (if (`|EnumInequality` New_ArrowState (`self.ArrowState`))
    (`self.OnStateEnd` (`self.ArrowState`))
    (bind _output_get (set `self.ArrowState` (`local.New_ArrowState`)))
    (`self.OnStateBegin` _output_get)))

(fn `TryToApplyDamage`
  (params (HitActor :type "Actor Object Reference"))
  (returns (`Success?` :type Boolean))
  (locals (L_EnemyHitReactionComponent :type "/Game/Library/CombatSystem/Blueprints/Components/HitReactionComponent Object Reference"))
  (bind _attackimpactfx (`self.AttackImpactFX`))
  (bind _lasthit (`self.LastHit`))
  (bind _l_enemyhitreactioncomponent (`local.L_EnemyHitReactionComponent`))
  (bind _ascharacter (cast `Character` HitActor)
    (:`then`
      (bind _output_get (set `self.HitCharacter` _ascharacter))
      (`/Engine/EditorBlueprintResources/StandardMacros.IsValid` (`self.AttackInfo`)
        (:`Is Valid`
          (set `self.HitBoneName` (`.HitBoneName` (`GameplayStatics.BreakHitResult` (`self.LastHit`))))
          (`PlayerController.ClientStartCameraShake` :`self` (`GameplayStatics.GetPlayerController` 0) :`Shake` "/Game/Library/CombatSystem/Blueprints/Camera/Shakes/RegularAttackCameraShake.RegularAttackCameraShake_C")
          (bind _combathitdata (message `/Game/Library/CombatSystem/Blueprints/Interfaces/DamageBPI.GetCombatHitData` (`self.GetOwner`) (`self.LastHit`)))
          (set `self.LastCombatHitData` _combathitdata)
          (set `local.L_EnemyHitReactionComponent` (`self.GetComponentByClass` _output_get "/Game/Library/CombatSystem/Blueprints/Components/HitReactionComponent.HitReactionComponent_C"))
          (`/Game/Library/CombatSystem/Blueprints/Components/HitReactionComponent.StoreCombatHitData` (`local.L_EnemyHitReactionComponent`) (`self.LastCombatHitData`))
          (`GameplayStatics.ApplyDamage` _output_get (`self.RegularDamage`) (`self.GetInstigatorController` (`self.GetOwner`)) self "/Game/Library/CombatSystem/Blueprints/DamageTypes/Instances/ProjectileDamage.ProjectileDamage_C")
          (`GameplayStatics.ApplyDamage` _output_get (`self.PoiseDamage`) (`self.GetInstigatorController` (`self.GetOwner`)) self "/Game/Library/CombatSystem/Blueprints/DamageTypes/Instances/PoiseDamage.PoiseDamage_C")
          (`GameplayStatics.ApplyDamage` _output_get (`self.AdditionalDamageTypeAmount`) (`self.GetInstigatorController` (`self.GetOwner`)) self (`self.AdditionalDamageType`))
          (`/Engine/EditorBlueprintResources/StandardMacros.IsValid` _l_enemyhitreactioncomponent
            (:`Is Valid`
              (`/Game/Library/CombatSystem/Blueprints/Components/HitReactionComponent.Store Enemy Attack Info` _l_enemyhitreactioncomponent (`self.AttackInfo`))
              (`/Game/Library/CombatSystem/Blueprints/Components/HitReactionComponent.ApplyImpactEffect` _l_enemyhitreactioncomponent _attackimpactfx (`GameplayStatics.GetSurfaceType` _lasthit) (`.ImpactPoint` (`GameplayStatics.BreakHitResult` _lasthit)))
              (`/Game/Library/CombatSystem/Blueprints/Components/HitReactionComponent.ApplyHitEffect` _l_enemyhitreactioncomponent)
              (`/Game/Library/CombatSystem/Blueprints/Components/HitReactionComponent.ApplyCameraShake` (`local.L_EnemyHitReactionComponent`) _attackimpactfx)
              (return true))))))
    (:`CastFailed`
      (return false))))

(fn `UserConstructionScript`)