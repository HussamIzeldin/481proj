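; BP_BaseCameraMode is the base object for camera modes in the camera system, exposing initialize, start, tick and end events.
; Initialize and start are empty hooks, while tick only stores the incoming TickValue.
; Ending the mode tells CameraSystemComponent to exit it and optionally resets TimePassed.
; A getter and a change-checked setter manage the mode's status.
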(event `Initialize Camera Mode`)

(event `Start Camera Mode`)

(event `Tick Camera Mode`
  (params (`Tick Value` :type "Float (double-precision)"))
  (set `self.Tick Value` `Tick Value`))

(event `End Camera Mode`
  (`/Game/Library/CameraSystem/CameraSystemComponent.Exit Current Camera Mode` (`self.CameraSystemComponent`) self)
  (if (`self.Reset Time On End`)
    (set `self.Time Passed` 0.0)))

(fn `Get Camera Mode Status`
  (returns (`Camera Mode Status` :type "/Game/Library/CameraSystem/EnumsStructs/E_CameraModeState Enum"))
  (return (`self.Camera Mode Status`)))

(fn `Set Camera Mode Status`
  (params (`Camera Mode Status` :type "/Game/Library/CameraSystem/EnumsStructs/E_CameraModeState Enum" :default "NewEnumerator0"))
  (if (`|EnumInequality` `Camera Mode Status` (`self.Camera Mode Status`))
    (set `self.Camera Mode Status` `Camera Mode Status`)))