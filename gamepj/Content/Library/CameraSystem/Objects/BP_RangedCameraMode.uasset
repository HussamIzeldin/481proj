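; BP_RangedCameraMode is a camera mode object that transitions the spring arm to a ranged camera setup.
; On start it snapshots the current arm length, socket offset and camera lag speed, then enters the Looping status.
; Each tick accumulates time and lerps those values toward RequiredCameraProperties, using a float curve as alpha.
; When the curve's end time is reached, it resets the timer and sets the status to Nothing.
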(event `self.Start Camera Mode`
  (bind _spring_arm_component (`/Game/Library/CameraSystem/CameraSystemComponent.Spring Arm Component` (`self.CameraSystemComponent`)))
  (set `self.Current Target Arm Length` (`SpringArmComponent.TargetArmLength` _spring_arm_component))
  (set `self.Current Socket Offset` (`SpringArmComponent.SocketOffset` _spring_arm_component))
  (set `self.Current Camera Lag Speed` (`SpringArmComponent.CameraLagSpeed` _spring_arm_component))
  (`self.Set Camera Mode Status` "NewEnumerator2"))

(event `self.Tick Camera Mode`
  (params (`Tick Value` :type "Float (single-precision)"))
  (bind (_targetarmlength _socketoffset _targetoffset _cameralag _cameralagspeed) (break `/Game/Library/CameraSystem/EnumsStructs/S_CameraProperties` (`self.Required Camera Properties`)))
  (bind _returnvalue (`CurveFloat.GetFloatValue` (`self.Float Curve To Use`) (`self.Time Passed`)))
  (bind (_mintime _maxtime) (`CurveBase.GetTimeRange` (`self.Float Curve To Use`)))
  (`parent.Tick Camera Mode` `Tick Value`)
  (switch `/Game/Library/CameraSystem/EnumsStructs/E_CameraModeState` (`self.Get Camera Mode Status`)
    (:`NewEnumerator2`
      (set `self.Time Passed` (select `bool` (>= (`self.Time Passed`) _maxtime) :`false` (+ (`self.Tick Value`) (`self.Time Passed`)) :`true` _maxtime))
      (set `SpringArmComponent.TargetArmLength` (`KismetMathLibrary.Lerp` (`self.Current Target Arm Length`) _targetarmlength (`CurveFloat.GetFloatValue` (`self.Float Curve To Use`) (`self.Time Passed`))) (`/Game/Library/CameraSystem/CameraSystemComponent.Spring Arm Component` (`self.CameraSystemComponent`)))
      (set `SpringArmComponent.SocketOffset` (`KismetMathLibrary.VLerp` (`self.Current Socket Offset`) _socketoffset _returnvalue) (`/Game/Library/CameraSystem/CameraSystemComponent.Spring Arm Component` (`self.CameraSystemComponent`)))
      (set `SpringArmComponent.CameraLagSpeed` (`KismetMathLibrary.Lerp` (`self.Current Camera Lag Speed`) _cameralagspeed _returnvalue) (`/Game/Library/CameraSystem/CameraSystemComponent.Spring Arm Component` (`self.CameraSystemComponent`)))
      (if (>= (`self.Time Passed`) (`.MaxTime` (`CurveBase.GetTimeRange` (`self.Float Curve To Use`))))
        (set `self.Time Passed` 0.0)
        (`self.Set Camera Mode Status` "NewEnumerator0")))))